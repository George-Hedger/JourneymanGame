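; BP_CogworkMoth is an AI-controlled mechanical moth enemy that spots the player inside its PatrolZone box.
; Each tick it tests the player's location against the box and updates the "hasSeenPlayer?" Blackboard key, only setting it true while "Waiting" is false.
; Activation changes write the "Waiting" key.
; Damage reduces health and briefly flashes the mesh red, while death notifies the ActiveArea and destroys the actor.
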(event `self.ReceiveAnyDamage`
  (params (Damage :type "Float (single-precision)") (DamageType :type "DamageType Object Reference") (InstigatedBy :type "Controller Object Reference") (DamageCauser :type "Actor Object Reference"))
  (bind _mesh (`self.Mesh`))
  (`self.SetHealth` Damage true)
  (`/Engine/EditorBlueprintResources/StandardMacros.IsValid` _mesh
    (:`Is Valid`
      (`PrimitiveComponent.SetMaterial` _mesh 0 "/Game/JourneyManContent/Assets/Materials/Placeholder/M_Red.M_Red")
      (`KismetSystemLibrary.Delay` 0.2)
      (`PrimitiveComponent.SetMaterial` _mesh 0 (`self.Material`)))))

(event `self.ReceiveBeginPlay`
  (set `self.Material` (`PrimitiveComponent.GetMaterial` (`self.Mesh`) 0))
  (`self.SetHealth` (`self.MaxHealth`)))

(event `self.ReceiveTick`
  (params (DeltaSeconds :type "Float (single-precision)"))
  (bind _returnvalue (`GameplayStatics.GetPlayerCharacter` 0))
  (bind _box (`/Game/JourneyManContent/Blueprints/Characters/Enemies/Mechanical_Moth/BP_FlyerPatrolZone.Box` (`self.Patrol Zone`)))
  (bind _returnvalue_2 (`AIBlueprintHelperLibrary.GetBlackboard` (`AIBlueprintHelperLibrary.GetAIController` self)))
  (`/Engine/EditorBlueprintResources/StandardMacros.IsValid` _returnvalue
    (:`Is Valid`
      (bind _output_get (set `self.Player Seen` (`KismetMathLibrary.IsPointInBoxWithTransform` (`self.K2_GetActorLocation` _returnvalue) (`SceneComponent.K2_GetComponentToWorld` _box) (`BoxComponent.GetUnscaledBoxExtent` _box))))
      (if _output_get
        (if (not (`BlackboardComponent.GetValueAsBool` _returnvalue_2 "Waiting"))
          (`BlackboardComponent.SetValueAsBool` _returnvalue_2 "hasSeenPlayer?" true))
        (else
          (`BlackboardComponent.SetValueAsBool` _returnvalue_2 "hasSeenPlayer?" false))))))

(event `Get Active Area`
  (params (`Activation Area` :type "/Game/JourneyManContent/Blueprints/Characters/Enemies/BP_EnemyStart Object Reference"))
  (set `self.Active Area` `Activation Area`))

(event `CustomEvent`
  (bind _active_area (`self.Active Area`))
  (`/Engine/EditorBlueprintResources/StandardMacros.IsValid` _active_area
    (:`Is Valid`
      (`/Game/JourneyManContent/Blueprints/Characters/Enemies/BP_EnemyStart.EnemyDeath` _active_area))
    (:`Is Not Valid`
      _))
  (`self.K2_DestroyActor`))

(event `self.OnDeath`
  (bind _active_area (`self.Active Area`))
  (`/Engine/EditorBlueprintResources/StandardMacros.IsValid` _active_area
    (:`Is Valid`
      (`/Game/JourneyManContent/Blueprints/Characters/Enemies/BP_EnemyStart.EnemyDeath` _active_area))
    (:`Is Not Valid`
      _))
  (`self.K2_DestroyActor`))

(event `/Game/JourneyManContent/Blueprints/Interfaces/BPI_Activate.OnActivationChanged`
  (params (IsActive :type Boolean))
  (`BlackboardComponent.SetValueAsBool` (`AIBlueprintHelperLibrary.GetBlackboard` (`AIBlueprintHelperLibrary.GetAIController` self)) "Waiting" IsActive))

(fn `UserConstructionScript`
  (`parent.UserConstructionScript`))