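; BP_EnemyStart is an encounter trigger that signals a group of enemies and responds when they are defeated.
; The first player overlap with its Box sends an activation message with false to listed spiders and cogwork moths, also passing itself to spiders as their active area.
; It tallies the listed enemies on BeginPlay, and EnemyDeath calls decrement that count until zero, when responding actors implementing BPI_Activate receive true.
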(event `self.ReceiveBeginPlay`
  (for _ (`self.Effected Enemies`)
    (set `self.Enemy Tally` (+ (`self.Enemy Tally`) 1))))

(event `self.Box.OnComponentBeginOverlap`
  (params (OverlappedComponent :type "PrimitiveComponent Object Reference") (OtherActor :type "Actor Object Reference") (OtherComp :type "PrimitiveComponent Object Reference") (OtherBodyIndex :type Integer) (bFromSweep :type Boolean) (SweepResult :type "HitResult Structure (by ref)"))
  (cast `/Game/JourneyManContent/Blueprints/Characters/Player/BP_ThirdPersonCharacter` OtherActor)
  (`/Engine/EditorBlueprintResources/StandardMacros.DoOnce` false
    (:`Completed`
      (for _array_element (`self.Effected Enemies`)
        (`/Engine/EditorBlueprintResources/StandardMacros.IsValid` _array_element
          (:`Is Valid`
            (bind _asbp_spider (cast `/Game/JourneyManContent/Blueprints/Characters/Enemies/Spider/BP_Spider` _array_element)
              (:`then`
                (message `/Game/JourneyManContent/Blueprints/Interfaces/BPI_Activate.OnActivationChanged` _asbp_spider false)
                (`/Game/JourneyManContent/Blueprints/Characters/Enemies/Spider/BP_Spider.Get Active Area` _asbp_spider self))
              (:`CastFailed`
                (bind _asbp_cogwork_moth (cast `/Game/JourneyManContent/Blueprints/Characters/Enemies/Mechanical_Moth/BP_CogworkMoth` _array_element))
                (message `/Game/JourneyManContent/Blueprints/Interfaces/BPI_Activate.OnActivationChanged` _asbp_cogwork_moth false)))))))))

(event `EnemyDeath`
  (set `self.Enemy Tally` (- (`self.Enemy Tally`) 1))
  (if (<= (`self.Enemy Tally`) 0)
    (for _array_element (`self.Responding Actors`)
      (`/Engine/EditorBlueprintResources/StandardMacros.IsValid` _array_element
        (:`Is Valid`
          (if (`KismetSystemLibrary.DoesImplementInterface` _array_element "/Game/JourneyManContent/Blueprints/Interfaces/BPI_Activate.BPI_Activate_C")
            (message `/Game/JourneyManContent/Blueprints/Interfaces/BPI_Activate.OnActivationChanged` _array_element true)))))))

(fn `UserConstructionScript`)