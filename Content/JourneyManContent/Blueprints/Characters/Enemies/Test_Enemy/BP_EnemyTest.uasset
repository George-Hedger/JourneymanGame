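; BP_EnemyTest is a test enemy that flags when it has seen the player.
; When PawnSensing sees a pawn, it runs a synchronous navigation path query from itself to that pawn.
; If the path object is valid and the pawn is a BP_ThirdPersonCharacter, it sets the hasSeenPlayer? Blackboard bool on its AI controller.
; An invalid path object only prints an out-of-range message, and nothing here clears the flag.
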(event `self.PawnSensing.OnSeePawn`
  (params (Pawn :type "Pawn Object Reference"))
  (bind _returnvalue (`NavigationSystemV1.FindPathToLocationSynchronously` (`self.K2_GetActorLocation` self) (`self.K2_GetActorLocation` Pawn) Pawn null))
  (`/Engine/EditorBlueprintResources/StandardMacros.IsValid` _returnvalue
    (:`Is Valid`
      (cast `/Game/JourneyManContent/Blueprints/Characters/Player/BP_ThirdPersonCharacter` Pawn)
      (`BlackboardComponent.SetValueAsBool` (`AIBlueprintHelperLibrary.GetBlackboard` (`AIBlueprintHelperLibrary.GetAIController` self)) "hasSeenPlayer?" true))
    (:`Is Not Valid`
      (`KismetSystemLibrary.PrintString` "Player out of range"))))

(fn `UserConstructionScript`
  (`parent.UserConstructionScript`))