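; BP_BossCrate is a crate in the boss encounter that drops into place and is destroyed by the boss's hand.
; On BeginPlay a DropIn timeline lerps it from its placed location down by FloorHeightDifference, without sweeping.
; When its Cube component begins overlapping a BP_BossHand actor, the crate destroys itself.
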(event `self.ReceiveBeginPlay`
  (bind _output_get (set `self.Start Location` (`self.K2_GetActorLocation`)))
  (set `self.Target Location` (`KismetMathLibrary.MakeVector` (.x _output_get) (.y _output_get) (- (.z _output_get) (`self.Floor height Difference`))))
  (bind (_direction _movement) (`Timeline|Drop In`)
    (:`Update`
      (`self.K2_SetActorLocation` (`KismetMathLibrary.VLerp` (`self.Start Location`) (`self.Target Location`) _movement)))))

(event `self.Cube.OnComponentBeginOverlap`
  (params (OverlappedComponent :type "PrimitiveComponent Object Reference") (OtherActor :type "Actor Object Reference") (OtherComp :type "PrimitiveComponent Object Reference") (OtherBodyIndex :type Integer) (bFromSweep :type Boolean) (SweepResult :type "HitResult Structure (by ref)"))
  (cast `/Game/JourneyManContent/Blueprints/Characters/Enemies/Boss/BP_BossHand` OtherActor)
  (`self.K2_DestroyActor`))

(fn `UserConstructionScript`)