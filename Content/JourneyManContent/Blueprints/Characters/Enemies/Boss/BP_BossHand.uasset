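; BP_BossHand is a boss hand that spins continuously, damaging the player on contact and dealing massive damage to cobwebs it touches.
; A looping Delay in BeginPlay adds yaw every tick of the loop, using a Speed value.
; OnActivationChanged counts active cogs, raising Speed on any change below the required count, including deactivations.
; Reaching that count triggers Victory, which teleports the player to a hard-coded location.
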(event `Speed up`
  (set `self.Speed` (+ (`self.Speed`) 0.4)))

(event `self.ReceiveBeginPlay`
  (`|ExecutionSequence`
    (:`then_1`
      (`SceneComponent.K2_AddWorldRotation` (`self.DefaultSceneRoot`) (`KismetMathLibrary.MakeRotator` 0.0 0.0 (+ (`self.Delta Rotation Z (Yaw)`) (`self.Speed`))) false false :!label _label)
      (`KismetSystemLibrary.Delay` 0.01)
      (goto _label))))

(event `/Game/JourneyManContent/Blueprints/Interfaces/BPI_Activate.OnActivationChanged`
  (params (IsActive :type Boolean))
  (bind _output_get (set `self.NumberActivations` (`KismetMathLibrary.Max` (+ (`self.NumberActivations`) (`KismetMathLibrary.SelectInt` 1 -1 IsActive)))))
  (if (>= _output_get (`self.NumberOfCogActivationsForActive`))
    (`self.Victory`)
    (else
      (`self.Speed up`))))

(event `self.Box.OnComponentBeginOverlap`
  (params (OverlappedComponent :type "PrimitiveComponent Object Reference") (OtherActor :type "Actor Object Reference") (OtherComp :type "PrimitiveComponent Object Reference") (OtherBodyIndex :type Integer) (bFromSweep :type Boolean) (SweepResult :type "HitResult Structure (by ref)"))
  (bind _asbp_third_person_character (cast `/Game/JourneyManContent/Blueprints/Characters/Player/BP_ThirdPersonCharacter` OtherActor)
    (:`then`
      (`GameplayStatics.ApplyDamage` _asbp_third_person_character 20.0))
    (:`CastFailed`
      (bind _asbp_cobweb (cast `/Game/JourneyManContent/Blueprints/LevelObjects/Hazards/BP_Cobweb` OtherActor))
      (`GameplayStatics.ApplyDamage` _asbp_cobweb 10000.0))))

(event `Victory`
  (bind _asbp_third_person_character (cast `/Game/JourneyManContent/Blueprints/Characters/Player/BP_ThirdPersonCharacter` (`GameplayStatics.GetPlayerCharacter` 0)))
  (`self.K2_SetActorLocation` _asbp_third_person_character (-14990.0 7560.0 862.0) false false))

(fn `UserConstructionScript`)