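; BP_ActiveCamera is a trigger volume that plays a one-time cutscene and then activates linked objects.
; When the third-person character overlaps the box and HasPlayed is true, a DoN gate starts the Camera's cutscene and the player's cutscene state.
; After a delay based on blend and pause times, Update sends BPI_Activate messages to each Active entry or its implementing components, printing errors for non-implementers.
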(event `self.Box.OnComponentBeginOverlap`
  (params (OverlappedComponent :type "PrimitiveComponent Object Reference") (OtherActor :type "Actor Object Reference") (OtherComp :type "PrimitiveComponent Object Reference") (OtherBodyIndex :type Integer) (bFromSweep :type Boolean) (SweepResult :type "HitResult Structure (by ref)"))
  (cast `/Game/JourneyManContent/Blueprints/Characters/Player/BP_ThirdPersonCharacter` OtherActor)
  (if (`self.Has played`)
    (`/Engine/EditorBlueprintResources/StandardMacros.Do N` 1
      (:`Exit`
        (bind _camera (`self.Camera`)
          (:`then`
            (`/Game/JourneyManContent/Blueprints/LevelObjects/CoreMechanics/BP_CutsceneCamera.Play Cutscene` _camera)
            (bind _asbp_third_person_character (cast `/Game/JourneyManContent/Blueprints/Characters/Player/BP_ThirdPersonCharacter` (`GameplayStatics.GetPlayerPawn` 0))
              (:`then`
                (`/Game/JourneyManContent/Blueprints/Characters/Player/BP_ThirdPersonCharacter.StartCutscene` _asbp_third_person_character))
              (:`CastFailed`
                _))
            (`KismetSystemLibrary.Delay` (+ (`/Game/JourneyManContent/Blueprints/LevelObjects/CoreMechanics/BP_CutsceneCamera.Camera Blend Time` _camera) (* (`/Game/JourneyManContent/Blueprints/LevelObjects/CoreMechanics/BP_CutsceneCamera.Pause At Target Time` _camera) 0.3)))
            (`self.Update` true))
          (:`else`))))))

(fn `Update`
  (params (IsActive :type Boolean))
  (for (_array_element _array_index) (`self.Active`)
    (if (`KismetSystemLibrary.DoesImplementInterface` _array_element "/Game/JourneyManContent/Blueprints/Interfaces/BPI_Activate.BPI_Activate_C")
      (message `/Game/JourneyManContent/Blueprints/Interfaces/BPI_Activate.OnActivationChanged` _array_element IsActive)
      (else
        (bind _returnvalue (`self.GetComponentsByInterface` _array_element "/Game/JourneyManContent/Blueprints/Interfaces/BPI_Activate.BPI_Activate_C"))
        (if (> (`KismetArrayLibrary.Array_Length` _returnvalue) 0)
          (for _array_element_2 _returnvalue
            (message `/Game/JourneyManContent/Blueprints/Interfaces/BPI_Activate.OnActivationChanged` _array_element_2 IsActive))
          (else
            (`KismetSystemLibrary.PrintString` (`KismetStringLibrary.Concat_StrStr` "Object at index: " (`KismetStringLibrary.Conv_IntToString` _array_index) " does not implement BPI_Activate and cannot be activated") true true (struct :`R` 1.0 :`A` 1.0) 100.0)))))))

(fn `UserConstructionScript`)