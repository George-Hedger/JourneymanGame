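; Cogwork Soldier enemy that stays idle until an activation event switches it on, and is destroyed by any damage.
; Once active, Tick starts a one-time patrol that cycles through a waypoint array with AI MoveTo.
; A player entering its Box interrupts patrol with a single move to their current position, with Y locked to zero.
; The player leaving the Box resumes patrol.
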(event `self.ReceiveBeginPlay`
  ;[0.003416 0.15 0.00705 0.5] Begin play
  (`parent.ReceiveBeginPlay`)
  (set `self.IsActivated?` false)
  (set `self.IsChasing?` false))

(event `self.ReceiveAnyDamage`
  (params (Damage :type "Float (single-precision)") (DamageType :type "DamageType Object Reference") (InstigatedBy :type "Controller Object Reference") (DamageCauser :type "Actor Object Reference"))
  ;[0.15 0 0.01339 0.5] Death
  (`self.K2_DestroyActor`))

(event `self.ReceiveTick`
  (params (DeltaSeconds :type "Float (single-precision)"))
  (if (`self.IsActivated?`)
    (`/Engine/EditorBlueprintResources/StandardMacros.DoOnce` false
      (:`Completed`
        (`self.Patrol`)))))

(event `/Game/JourneyManContent/Blueprints/Interfaces/BPI_Activate.OnActivationChanged`
  (params (IsActive :type Boolean))
  ;[0.02593 0.15 0.02818 0.5] activate event
  (set `self.IsActivated?` IsActive))

(event `Patrol`
  (bind _current_waypoint (`self.Current Waypoint`))
  ; Patrol
  (if (`self.IsActivated?`)
    (if (not (`self.IsChasing?`))
      (`|AIMoveTo` self (0.0 0.0 0.0) (`|GetArrayItem` (`self.Waypoint`) (`self.Current Waypoint`))
        (:`OnSuccess`
          (bind _result (`/Engine/EditorBlueprintResources/StandardMacros.IncrementInt` _current_waypoint)
            (:`  `
              (`KismetSystemLibrary.PrintString` (`KismetStringLibrary.Conv_IntToString` _result))
              (if (>= _current_waypoint (`KismetArrayLibrary.Array_Length` (`self.Waypoint`)))
                (set `self.Current Waypoint` 0))
              (`self.Patrol`))))
        (:`OnFail`
          (`KismetSystemLibrary.PrintString` "Cant find Waypoint"))))))

(event `self.Box.OnComponentBeginOverlap`
  (params (OverlappedComponent :type "PrimitiveComponent Object Reference") (OtherActor :type "Actor Object Reference") (OtherComp :type "PrimitiveComponent Object Reference") (OtherBodyIndex :type Integer) (bFromSweep :type Boolean) (SweepResult :type "HitResult Structure (by ref)"))
  ; Chase
  (if (`self.IsActivated?`)
    (bind _asbp_third_person_character (cast `/Game/JourneyManContent/Blueprints/Characters/Player/BP_ThirdPersonCharacter` OtherActor))
    (set `self.IsChasing?` true)
    (bind (_returnvalue_x _returnvalue_y _returnvalue_z) (`KismetMathLibrary.BreakVector` (`self.K2_GetActorLocation` _asbp_third_person_character)))
    (`|AIMoveTo` self (`KismetMathLibrary.MakeVector` _returnvalue_x 0.0 _returnvalue_z) null)))

(event `self.Box.OnComponentEndOverlap`
  (params (OverlappedComponent :type "PrimitiveComponent Object Reference") (OtherActor :type "Actor Object Reference") (OtherComp :type "PrimitiveComponent Object Reference") (OtherBodyIndex :type Integer))
  ; Stop Chase Resume Patrol
  (if (`self.IsActivated?`)
    (cast `/Game/JourneyManContent/Blueprints/Characters/Player/BP_ThirdPersonCharacter` OtherActor)
    (set `self.IsChasing?` false)
    (`self.Patrol`)))

(fn `UserConstructionScript`
  (`parent.UserConstructionScript`))