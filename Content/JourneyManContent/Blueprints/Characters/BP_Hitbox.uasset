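; BP_Hitbox is a damage volume that hurts overlapping actors, skipping BP_Base_Character instances on TeamToIgnore.
; In one-shot mode, it damages each actor once on overlap, tracked through HitActors.
; In damage-per-second mode, Tick applies frame-scaled damage to everything inside the Box.
; A positive Lifetime makes the hitbox destroy itself when time runs out, while zero or less keeps it active indefinitely.
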(event `self.ReceiveActorBeginOverlap`
  (params (OtherActor :type "Actor Object Reference"))
  (if (`self.IsDamagePerSecond`)
    _
    (elif (not (`KismetArrayLibrary.Array_Contains` (`self.HitActors`) OtherActor))
      (`KismetArrayLibrary.Array_Add` (`self.HitActors`) OtherActor)
      (if (not (`self.ShouldIgnore` OtherActor))
        (`GameplayStatics.ApplyDamage` OtherActor (`self.Damage`) null (`self.DamageCausingActor`))))))

(event `self.ReceiveTick`
  (params (DeltaSeconds :type "Float (single-precision)"))
  (if (<= (`self.Lifetime`) 0.0)
    (if (`self.IsDamagePerSecond`) :!label _label
      (for _array_element (`PrimitiveComponent.GetOverlappingActors` (`self.Box`) null)
        (if (not (`self.ShouldIgnore` _array_element))
          (`GameplayStatics.ApplyDamage` _array_element (* DeltaSeconds (`self.Damage`)) null (`self.DamageCausingActor`)))))
    (else
      (bind _output_get (set `self.CurrentLifetime` (+ DeltaSeconds (`self.CurrentLifetime`))))
      (if (>= _output_get (`self.Lifetime`))
        (`self.K2_DestroyActor`)
        (else
          (goto _label))))))

(fn `ShouldIgnore`
  (params (Object :type "Object Object Reference"))
  (returns (ShouldIgnore :type Boolean))
  (locals (Ignore :type Boolean))
  (bind _asbp_base_character (cast `/Game/JourneyManContent/Blueprints/Characters/BP_Base_Character` Object)
    (:`then`
      (set `local.Ignore` (`|EnumEquality` (`self.TeamToIgnore`) (`/Game/JourneyManContent/Blueprints/Characters/BP_Base_Character.Team` _asbp_base_character))))
    (:`CastFailed`
      _))
  (return (`local.Ignore`)))

(fn `UserConstructionScript`)