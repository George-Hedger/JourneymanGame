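; BP_Base_Friend is a friend character base that plays a cutscene when the player touches it, then shrinks away.
; Overlap of its Box by BP_ThirdPersonCharacter calls PlayCutscene on CutsceneCam and, after a fixed delay, opens a Gate.
; Tick feeds that Gate, so each frame reduces the scale by delta time, clamped at zero, and destroys the actor once it is nearly invisible.
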(event `self.Box.OnComponentBeginOverlap`
  (params (OverlappedComponent :type "PrimitiveComponent Object Reference") (OtherActor :type "Actor Object Reference") (OtherComp :type "PrimitiveComponent Object Reference") (OtherBodyIndex :type Integer) (bFromSweep :type Boolean) (SweepResult :type "HitResult Structure (by ref)"))
  (cast `/Game/JourneyManContent/Blueprints/Characters/Player/BP_ThirdPersonCharacter` OtherActor)
  (`/Game/JourneyManContent/Blueprints/LevelObjects/CoreMechanics/BP_CutsceneCamera.Play Cutscene` (`self.CutsceneCam`))
  (`KismetSystemLibrary.Delay` 4.0)
  (goto _label :!via `Open`))

(event `self.ReceiveTick`
  (params (DeltaSeconds :type "Float (single-precision)"))
  (bind (_returnvalue_x _returnvalue_y _returnvalue_z) (`KismetMathLibrary.BreakVector` (- (`self.GetActorScale3D`) (* (1.0 1.0 1.0) DeltaSeconds))))
  (`/Engine/EditorBlueprintResources/StandardMacros.Gate` true :!label _label
    (:`Exit`
      (`self.SetActorScale3D` (`KismetMathLibrary.MakeVector` (`KismetMathLibrary.FClamp` _returnvalue_x) (`KismetMathLibrary.FClamp` _returnvalue_y) (`KismetMathLibrary.FClamp` _returnvalue_z)))
      (if (<= (`KismetMathLibrary.VSizeSquared` (`self.GetActorScale3D`)) 0.01)
        (`self.K2_DestroyActor`)))))

(fn `UserConstructionScript`)