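; BP_Base_Character is a base character Blueprint that provides health and death handling.
; It sets Health to MaxHealth on BeginPlay, and AnyDamage subtracts incoming damage, capping the result at MaxHealth.
; When Health reaches zero or below it calls OnDeath, which destroys the actor.
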(event `self.ReceiveBeginPlay`
  (set `self.Health` (`self.MaxHealth`)))

(event `self.ReceiveAnyDamage`
  (params (Damage :type "Float (single-precision)") (DamageType :type "DamageType Object Reference") (InstigatedBy :type "Controller Object Reference") (DamageCauser :type "Actor Object Reference"))
  (bind _output_get (set `self.Health` (`KismetMathLibrary.FMin` (- (`self.Health`) Damage) (`self.MaxHealth`))))
  (if (<= _output_get 0.0)
    (`self.OnDeath`)))

(fn `OnDeath`
  (`self.K2_DestroyActor`))

(fn `UserConstructionScript`)