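; Component that projects a drop shadow decal beneath the player character.
; On BeginPlay it adds a decal with M_DropShadow to player 0's BP_ThirdPersonCharacter, regardless of owner, and stops the capsule receiving decals.
; Each tick it line traces from the capsule along its negative up vector on the Visibility channel and, on a hit, moves the decal slightly above the impact point.
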(event `self.ReceiveBeginPlay`
  (bind _asbp_third_person_character (cast `/Game/JourneyManContent/Blueprints/Characters/Player/BP_ThirdPersonCharacter` (`GameplayStatics.GetPlayerCharacter` 0)))
  (bind _returnvalue (`|AddComponentByClass` :`self` _asbp_third_person_character :`Class` "/Script/Engine.DecalComponent"))
  (`PrimitiveComponent.SetReceivesDecals` (`Character.CapsuleComponent` _asbp_third_person_character) false)
  (`DecalComponent.SetDecalMaterial` _returnvalue "/Game/JourneyManContent/Assets/Materials/Placeholder/M_DropShadow.M_DropShadow"))

(event `self.ReceiveTick`
  (params (DeltaSeconds :type "Float (single-precision)"))
  (bind _capsulecomponent (`Character.CapsuleComponent` (stale `self.ReceiveBeginPlay` _asbp_third_person_character)))
  (bind _returnvalue (`SceneComponent.K2_GetComponentLocation` _capsulecomponent))
  (bind (_outhit _returnvalue_2) (`KismetSystemLibrary.LineTraceSingle` _returnvalue (- _returnvalue (* (`SceneComponent.GetUpVector` _capsulecomponent) 5000)) "TraceTypeQuery1"))
  (if _returnvalue_2
    (bind (_bblockinghit _binitialoverlap _time _distance _location _impactpoint) (`GameplayStatics.BreakHitResult` _outhit))
    (`SceneComponent.K2_SetWorldLocation` (stale `self.ReceiveBeginPlay` _returnvalue) (`KismetMathLibrary.MakeVector` (.x _impactpoint) (.y _impactpoint) (+ (.z _impactpoint) 16.0)) false false)))