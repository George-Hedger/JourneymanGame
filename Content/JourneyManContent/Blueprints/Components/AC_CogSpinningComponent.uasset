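; Actor component that continuously spins its owner, likely a cog, by adding local rotation to the root component each tick while enabled.
; An activation-change event toggles the spinning on and off.
; On BeginPlay it looks for an AC_Timeslow component on the owner and, if found, scales rotation speed by its timeslow multiplier, so spinning respects time-slow effects.
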(event `self.ReceiveTick`
  (params (DeltaSeconds :type "Float (single-precision)"))
  (if (`self.Enabled`)
    (`SceneComponent.K2_AddLocalRotation` (`Actor.RootComponent` (`self.GetOwner`)) (* (`self.RotationAmount`) (* DeltaSeconds (`self.GetMultiplier`))) false false)))

(event `/Game/JourneyManContent/Blueprints/Interfaces/BPI_Activate.OnActivationChanged`
  (params (IsActive :type Boolean))
  (set `self.Enabled` IsActive))

(event `self.ReceiveBeginPlay`
  (bind _returnvalue (`Actor.GetComponentByClass` (`self.GetOwner`) "/Game/JourneyManContent/Blueprints/Components/AC_Timeslow.AC_Timeslow_C"))
  (`/Engine/EditorBlueprintResources/StandardMacros.IsValid` _returnvalue
    (:`Is Valid`
      (set `self.Timeslow exists?` true)
      (set `self.Timeslow` _returnvalue))
    (:`Is Not Valid`
      (set `self.Timeslow exists?` false))))

(fn `GetMultiplier`
  (returns (`TimeSlow Mult` :type "Float (double-precision)"))
  (if (`self.Timeslow exists?`)
    (return (`/Game/JourneyManContent/Blueprints/Components/AC_Timeslow.Timeslow Multiplier` (`self.Timeslow`)))
    (else
      (return 1.0))))