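; A static level-object platform on stilts, assembled in the construction script with no active runtime logic.
; The Size setting selects the deck mesh and the stilt offset from the centre.
; Large and Medium platforms get four corner stilts, while Small gets a single centred one.
; StiltLengthScale is negated as the stilts' Z scale, flipping the mesh vertically and setting its length.
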(fn `UserConstructionScript`
  (bind _offset (`self.offset`))
  (bind _offset_2 (`self.offset`))
  (bind _offset_3 (`self.offset`))
  (bind _offset_4 (`self.offset`))
  (`|ExecutionSequence`
    (:`then_0`
      (bind _returnvalue (`AddComponent|NODE_AddStaticMeshComponent-4`))
      (switch `/Game/JourneyManContent/Blueprints/LevelObjects/Static/E_PlatformSize` (`self.Size`)
        (:`NewEnumerator0`
          (`StaticMeshComponent.SetStaticMesh` _returnvalue "/Game/JourneyManContent/Assets/StaticMeshes/Static/Platforms/SM_Platform_Large.SM_Platform_Large"))
        (:`NewEnumerator1`
          (`StaticMeshComponent.SetStaticMesh` _returnvalue "/Game/JourneyManContent/Assets/StaticMeshes/Static/Platforms/SM_Platform_Medium.SM_Platform_Medium"))
        (:`NewEnumerator2`
          (`StaticMeshComponent.SetStaticMesh` _returnvalue "/Game/JourneyManContent/Assets/StaticMeshes/Static/Platforms/SM_Platform_Small.SM_Platform_Small"))))
    (:`then_1`
      (switch `/Game/JourneyManContent/Blueprints/LevelObjects/Static/E_PlatformSize` (`self.Size`)
        (:`NewEnumerator0`
          (set `self.offset` 300.0))
        (:`NewEnumerator1`
          (set `self.offset` 225.0))
        (:`NewEnumerator2`
          (set `self.small` true)
          (set `self.offset` 0.0))))
    (:`then_2`
      (bind _returnvalue_2 (`AddComponent|NODE_AddStaticMeshComponent-0` :`RelativeTransform` (`KismetMathLibrary.MakeTransform` (`KismetMathLibrary.MakeVector` _offset_2 _offset_2) (struct) (`KismetMathLibrary.MakeVector` 1.0 1.0 (* (`self.StiltLengthScale`) -1.0)))))
      (`StaticMeshComponent.SetStaticMesh` _returnvalue_2 "/Game/JourneyManContent/Assets/StaticMeshes/Static/Platforms/SM_Platform_Stilt.SM_Platform_Stilt"))
    (:`then_3`
      (if (not (`self.small`))
        (`|ExecutionSequence`
          (:`then_0`
            (bind _returnvalue_3 (`AddComponent|NODE_AddStaticMeshComponent-1` :`RelativeTransform` (`KismetMathLibrary.MakeTransform` (`KismetMathLibrary.MakeVector` _offset_3 (* _offset_3 -1.0)) (struct) (`KismetMathLibrary.MakeVector` 1.0 1.0 (* (`self.StiltLengthScale`) -1.0)))))
            (`StaticMeshComponent.SetStaticMesh` _returnvalue_3 "/Game/JourneyManContent/Assets/StaticMeshes/Static/Platforms/SM_Platform_Stilt.SM_Platform_Stilt"))
          (:`then_1`
            (bind _returnvalue_4 (`AddComponent|NODE_AddStaticMeshComponent-2` :`RelativeTransform` (`KismetMathLibrary.MakeTransform` (`KismetMathLibrary.MakeVector` (* _offset_4 -1.0) _offset_4) (struct) (`KismetMathLibrary.MakeVector` 1.0 1.0 (* (`self.StiltLengthScale`) -1.0)))))
            (`StaticMeshComponent.SetStaticMesh` _returnvalue_4 "/Game/JourneyManContent/Assets/StaticMeshes/Static/Platforms/SM_Platform_Stilt.SM_Platform_Stilt"))
          (:`then_2`
            (bind _returnvalue_5 (`AddComponent|NODE_AddStaticMeshComponent-3` :`RelativeTransform` (`KismetMathLibrary.MakeTransform` (`KismetMathLibrary.MakeVector` (* _offset -1.0) (* _offset -1.0)) (struct) (`KismetMathLibrary.MakeVector` 1.0 1.0 (* (`self.StiltLengthScale`) -1.0)))))
            (`StaticMeshComponent.SetStaticMesh` _returnvalue_5 "/Game/JourneyManContent/Assets/StaticMeshes/Static/Platforms/SM_Platform_Stilt.SM_Platform_Stilt")))))))