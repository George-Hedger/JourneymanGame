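; BP_WoodenWallPlacer is a level-building actor that generates a wooden wall as a grid of static meshes sized by Horizontal and Vertical.
; Its construction script loops over rows and columns, adding SM_WoodWall_No_Ends components at fixed spacing along X and Z.
; Each cell gets a second copy, rotated 180 degrees and offset to sit back-to-back with the first.
; The event graph contains no active logic.
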(fn `UserConstructionScript`
  (for _index (range (`self.Vertical`))
    (for _index_2 (range (`self.Horizontal`))
      (`|ExecutionSequence`
        (:`then_0`
          (bind _returnvalue (`AddComponent|NODE_AddStaticMeshComponent-0` :`RelativeTransform` (`KismetMathLibrary.MakeTransform` (`KismetMathLibrary.MakeVector` (`KismetMathLibrary.Conv_IntToDouble` (* _index_2 298)) 0.0 (`KismetMathLibrary.Conv_IntToDouble` (* _index 273))))))
          (`StaticMeshComponent.SetStaticMesh` _returnvalue "/Game/JourneyManContent/Assets/StaticMeshes/Static/Walls/SM_WoodWall_No_Ends.SM_WoodWall_No_Ends"))
        (:`then_1`
          (bind _returnvalue_2 (`AddComponent|NODE_AddStaticMeshComponent-1` :`RelativeTransform` (`KismetMathLibrary.MakeTransform` (`KismetMathLibrary.MakeVector` (`KismetMathLibrary.Conv_IntToDouble` (* (+ _index_2 1) 298)) -18.0 (`KismetMathLibrary.Conv_IntToDouble` (* _index 273))) (struct :`Yaw` 180.0))))
          (`StaticMeshComponent.SetStaticMesh` _returnvalue_2 "/Game/JourneyManContent/Assets/StaticMeshes/Static/Walls/SM_WoodWall_No_Ends.SM_WoodWall_No_Ends"))))))