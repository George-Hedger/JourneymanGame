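; BP_GrapplePoint is a grabbable level object that pulls the player toward it while grabbed.
; WhilstGrabbed calls the player's GrappleTowards with the point's location and ends the grab when the result is Arrived or Blocked.
; OnGrabEnd sets the player's velocity to GrappleSpeed along the direction from the movement component's last update location to the current position, carrying momentum out of the grapple.
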(fn `OnGrabEnd`
  (params (Player :type "/Game/JourneyManContent/Blueprints/Characters/Player/BP_ThirdPersonCharacter Object Reference"))
  (bind _charactermovement (`Character.CharacterMovement` Player))
  (`parent.OnGrabEnd` null)
  (set `MovementComponent.Velocity` (* (`KismetMathLibrary.Normal` (- (`self.K2_GetActorLocation` Player) (`CharacterMovementComponent.GetLastUpdateLocation` _charactermovement))) (`/Game/JourneyManContent/Blueprints/Characters/Player/BP_ThirdPersonCharacter.GrappleSpeed` Player)) _charactermovement))

(fn `UserConstructionScript`
  (`parent.UserConstructionScript`))

(fn `WhilstGrabbed`
  (params (Player :type "/Game/JourneyManContent/Blueprints/Characters/Player/BP_ThirdPersonCharacter Object Reference"))
  (`parent.WhilstGrabbed` Player)
  (bind _result (`/Game/JourneyManContent/Blueprints/Characters/Player/BP_ThirdPersonCharacter.GrappleTowards` Player (`self.K2_GetActorLocation`)))
  (switch `/Game/JourneyManContent/Blueprints/Characters/Player/E_GrappleResult` _result
    (:`NewEnumerator1`
      _)
    (:`NewEnumerator2`
      _))
  (`/Game/JourneyManContent/Blueprints/Characters/Player/BP_ThirdPersonCharacter.EndGrab` Player))