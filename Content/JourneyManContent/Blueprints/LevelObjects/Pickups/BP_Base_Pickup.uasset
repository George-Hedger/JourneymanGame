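; Base pickup actor for level objects that highlights on player hover and can be reset to where it started.
; Hover applies an outline overlay material to the mesh and drives a camera-facing child-actor widget, which is hidden on BeginPlay and hover end.
; BeginPlay caches transform, collision mode and physics state.
; ResetActor teleports back and zeroes velocities, while Disable/EnableCollision switch off and restore collision and physics.
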(event `/Game/JourneyManContent/Blueprints/Interfaces/BPI_Interactable.OnPlayerHoverBegin`
  (`SceneComponent.SetVisibility` (`self.Widget Component`) true false) ; keep disabled just in case we revert later
  (`MeshComponent.SetOverlayMaterial` (`self.StaticMesh`) "/Game/JourneyManContent/Assets/Materials/Outline/MI_InteractOutline.MI_InteractOutline"))

(event `self.ReceiveBeginPlay`
  (set `self.StartingTransform` (`self.GetTransform`))
  (set `self.CollisionMode` (`PrimitiveComponent.GetCollisionEnabled` (`self.StaticMesh`)))
  (set `self.IsSimulatingPhysics` (`SceneComponent.IsSimulatingPhysics` (`self.StaticMesh`) "None"))
  (set `self.Widget Component` (`self.GetComponentByClass` (`ChildActorComponent.ChildActor` (`self.BP_CameraFacingUI`)) "/Script/UMG.WidgetComponent"))
  (`SceneComponent.SetVisibility` (`self.Widget Component`) false false :!label _label)
  (`MeshComponent.SetOverlayMaterial` (`self.StaticMesh`) null))

(event `/Game/JourneyManContent/Blueprints/Interfaces/BPI_Interactable.OnPlayerHoverEnd`
  (goto _label))

(event `/Game/JourneyManContent/Blueprints/Interfaces/BPI_Reset.ResetActor`
  (`self.K2_SetActorTransform` (`self.StartingTransform`) false true)
  (`PrimitiveComponent.SetAllPhysicsLinearVelocity` (`self.StaticMesh`) (0.0 0.0 0.0) false)
  (`PrimitiveComponent.SetAllPhysicsAngularVelocityInDegrees` (`self.StaticMesh`) (`KismetMathLibrary.MakeVector` 0.0) false))

(fn `DisableCollision`
  (`PrimitiveComponent.SetSimulatePhysics` (`self.StaticMesh`) false)
  (`PrimitiveComponent.SetCollisionEnabled` (`self.StaticMesh`) "NoCollision"))

(fn `EnableCollision`
  (`PrimitiveComponent.SetSimulatePhysics` (`self.StaticMesh`) (`self.IsSimulatingPhysics`))
  (`PrimitiveComponent.SetCollisionEnabled` (`self.StaticMesh`) (`self.CollisionMode`)))

(fn `UserConstructionScript`)