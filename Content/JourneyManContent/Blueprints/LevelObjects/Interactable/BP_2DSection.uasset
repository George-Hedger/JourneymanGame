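; A level section volume that turns the player camera side-on to a guide spline, giving a 2D-style view.
; While the player overlaps it, camera yaw input is halved and a periodic timer compares camera yaw to the spline's perpendicular, optionally inverted.
; Misalignment starts a frame-rate timer that eases yaw through interpolated controller input deltas until aligned.
; Exiting restores input; the construction script previews the camera direction at the spline's start.
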(event `self.ReceiveBeginPlay`
  ; for accessing controller and variables in character bp
  (`|ExecutionSequence`
    (:`then_0`
      (bind _asbp_third_person_character (cast `/Game/JourneyManContent/Blueprints/Characters/Player/BP_ThirdPersonCharacter` (`GameplayStatics.GetPlayerCharacter` 0)))
      (set `self.As BP Third Person Character` _asbp_third_person_character))
    (:`then_1`
      ; check if the playercharacter starts inside the section
      (if (`KismetArrayLibrary.Array_Contains` (`self.GetOverlappingActors` "/Game/JourneyManContent/Blueprints/Characters/Player/BP_ThirdPersonCharacter.BP_ThirdPersonCharacter_C") (`self.As BP Third Person Character`))
        ; player input would be reduced
        (set `/Game/JourneyManContent/Blueprints/Characters/Player/BP_ThirdPersonCharacter.CameraYawModifier` 0.5 (`self.As BP Third Person Character`) :!label _label)
        ; setting up a timer for rough check if the rotators are aligned
        (bind _returnvalue (`KismetSystemLibrary.K2_SetTimerDelegate` (delegate `RoughCheck`) (/ 1.0 (`KismetMathLibrary.Conv_IntToDouble` (`self.CheckFrequency`))) true))))))

(event `self.ReceiveActorEndOverlap`
  (params (OtherActor :type "Actor Object Reference"))
  (bind _as_bp_third_person_character (`self.As BP Third Person Character`))
  ; check if it is the player character who left
  (if (== OtherActor _as_bp_third_person_character)
    ; restore the player input, probably need a different logic if there are other things that can change the modifier. currently its like how it is
    (set `/Game/JourneyManContent/Blueprints/Characters/Player/BP_ThirdPersonCharacter.CameraYawModifier` 1.0 _as_bp_third_person_character)
    ; clear the rough checking handle
    (if (`KismetSystemLibrary.K2_IsValidTimerHandle` (stale `self.ReceiveBeginPlay` _returnvalue))
      (`KismetSystemLibrary.K2_ClearAndInvalidateTimerHandle` (stale `self.ReceiveBeginPlay` _returnvalue))
      ; preventing it to clear a timer handle thats not set(if the player somehow get the angle right)
      (if (`KismetSystemLibrary.K2_IsValidTimerHandle` (stale `RoughCheck` _returnvalue)) :!label _label_2
        ; clear yaw control handle
        (`KismetSystemLibrary.K2_ClearAndInvalidateTimerHandle` (stale `RoughCheck` _returnvalue))
        (goto _label_3 :!via `Reset`)))))

(event `self.ReceiveActorBeginOverlap`
  (params (OtherActor :type "Actor Object Reference"))
  ; check if the overlapping actor is the player character
  (if (== OtherActor (`self.As BP Third Person Character`))
    (goto _label)))

(event `RoughCheck`
  ; get the new desired yaw then compare it with the current one
  (`self.UpdateDesiredYaw`)
  (bind _missed (`self.CompareRotatorYaw` (`self.DesiredCameraYaw`) (`SceneComponent.K2_GetComponentRotation` (`/Game/JourneyManContent/Blueprints/Characters/Player/BP_ThirdPersonCharacter.FollowCamera` (`self.As BP Third Person Character`)))))
  (if _missed
    ; if the rotators are not aligned, try correct it, at tick rate
    (`/Engine/EditorBlueprintResources/StandardMacros.DoOnce` false :!label _label_3
      (:`Completed`
        (bind _returnvalue (`KismetSystemLibrary.K2_SetTimer` null "YawControl" (`GameplayStatics.GetWorldDeltaSeconds`) true))
        (goto _label_4 :!via `Reset`)))
    (else
      ; preventing it to clear a timer handle thats not set(if the player somehow get the angle right)
      (`/Engine/EditorBlueprintResources/StandardMacros.DoOnce` true :!label _label_4
        (:`Completed`
          (goto _label_2))))))

(fn `CompareRotatorYaw`
  (params (Rotator1 :type "Rotator Structure") (Rotator2 :type "Rotator Structure"))
  (returns (Missed :type Boolean))
  (bind (_returnvalue_roll _returnvalue_pitch _returnvalue_yaw) (`KismetMathLibrary.BreakRotator` (`KismetMathLibrary.NormalizedDeltaRotator` Rotator1 Rotator2)))
  (return (< 0.2 (`KismetMathLibrary.Abs` _returnvalue_yaw))))

(fn `UpdateDesiredYaw`
  (bind _guiderail (`self.GuideRail`))
  (bind _returnvalue (`KismetMathLibrary.GetRightVector` (`SplineComponent.GetRotationAtDistanceAlongSpline` _guiderail (`SplineComponent.GetDistanceAlongSplineAtLocation` _guiderail (`self.K2_GetActorLocation` (`GameplayStatics.GetPlayerCharacter` 0)) "World") "World")))
  (if (`self.InvertCameraLocation`)
    (set `self.DesiredCameraYaw` (`KismetMathLibrary.MakeRotFromX` (* _returnvalue -1)))
    (else
      (set `self.DesiredCameraYaw` (`KismetMathLibrary.MakeRotFromX` _returnvalue)))))

(fn `UserConstructionScript`
  (bind _cameralookingdirection (`self.CameraLookingDirection`))
  (bind _returnvalue (`KismetMathLibrary.GetRightVector` (`SplineComponent.GetRotationAtSplinePoint` (`self.GuideRail`) 0 "World")))
  ; same logic as the desire yaw function. just a preview where the camera would be look at
  (if (`self.InvertCameraLocation`)
    (`SceneComponent.K2_SetWorldRotation` _cameralookingdirection (`KismetMathLibrary.MakeRotFromX` (* _returnvalue -1.0)) false false)
    (else
      (`SceneComponent.K2_SetWorldRotation` _cameralookingdirection (`KismetMathLibrary.MakeRotFromX` _returnvalue) false false))))

(fn `YawControl`
  (bind _returnvalue (`SceneComponent.K2_GetComponentRotation` (`/Game/JourneyManContent/Blueprints/Characters/Player/BP_ThirdPersonCharacter.FollowCamera` (`self.As BP Third Person Character`))))
  (bind (_returnvalue_roll _returnvalue_pitch _returnvalue_yaw) (`KismetMathLibrary.BreakRotator` (`KismetMathLibrary.NormalizedDeltaRotator` (`KismetMathLibrary.RInterpTo` _returnvalue (`self.DesiredCameraYaw`) (`GameplayStatics.GetWorldDeltaSeconds`) (`self.SmoothFactor`)) _returnvalue)))
  ; This function should be ran at tick rate to work
  (`Pawn.AddControllerYawInput` (`self.As BP Third Person Character`) _returnvalue_yaw))