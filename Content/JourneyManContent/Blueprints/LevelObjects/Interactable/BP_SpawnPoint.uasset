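; BP_SpawnPoint is a level object that respawns the player character at its own transform when that character is destroyed.
; On BeginPlay it caches the player's class and its own transform, then binds to the character's OnDestroyed event.
; On destruction it spawns and possesses a replacement, then calls WhenCheckpointed, which repeats that setup on the new character.
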(event `self.ReceiveBeginPlay`
  (bind _returnvalue (`GameplayStatics.GetPlayerCharacter` 0))
  ; respawns and possesses player character
  (set `self.PlayerClass` (`GameplayStatics.GetObjectClass` _returnvalue) :!label _label)
  (add `self.OnDestroyed` _returnvalue (delegate `OnDestroyed_Event`))
  (set `self.Spawn Transform` (`self.GetTransform`)))

(event `WhenCheckpointed`
  (goto _label))

(event `OnDestroyed_Event`
  (params (DestroyedActor :type "Actor Object Reference"))
  ; respawns and possesses player character
  (bind _returnvalue (`|SpawnActorFromClass` (`self.PlayerClass`) (`self.Spawn Transform`) "Undefined" "MultiplyWithRoot" null null))
  (`Controller.Possess` (`GameplayStatics.GetPlayerController` 0) _returnvalue)
  (`self.WhenCheckpointed`))

(fn `UserConstructionScript`)