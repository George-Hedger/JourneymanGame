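; Base interactable slot that takes the player's held pickup or hands it back, switching linked objects on or off.
; Activation reaches ObjectsToActivate through BPI_Activate on the actor, or else its components.
; The first placement can play a target camera cutscene, delaying activation until partway through.
; Afterward, Tick spins any slotted pickup and two counter-rotating component groups; hovering while carrying an item outlines the mesh.
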(event `self.ReceiveBeginPlay`
  (`self.UpdateAllObjects` false))

(event `/Game/JourneyManContent/Blueprints/Interfaces/BPI_Interactable.OnInteract`
  (bind (_returnvalue_location _returnvalue_rotation _returnvalue_scale) (`KismetMathLibrary.BreakTransform` (`self.GetTransform`)))
  (bind _asbp_third_person_character (cast `/Game/JourneyManContent/Blueprints/Characters/Player/BP_ThirdPersonCharacter` (`GameplayStatics.GetPlayerPawn` 0)))
  (`/Engine/EditorBlueprintResources/StandardMacros.IsValid` (`self.PickupInSlot`)
    (:`Is Valid`
      (`/Game/JourneyManContent/Blueprints/Characters/Player/BP_ThirdPersonCharacter.PickupItem` _asbp_third_person_character (`self.PickupInSlot`))
      (set `self.PickupInSlot` null)
      (`self.UpdateAllObjects` false))
    (:`Is Not Valid`
      (bind _helditemref (`/Game/JourneyManContent/Blueprints/Characters/Player/BP_ThirdPersonCharacter.DropPickup` _asbp_third_person_character))
      (`/Engine/EditorBlueprintResources/StandardMacros.IsValid` _helditemref
        (:`Is Valid`
          (`/Game/JourneyManContent/Blueprints/LevelObjects/Pickups/BP_Base_Pickup.DisableCollision` _helditemref)
          (bind _output_get (set `self.PickupInSlot` _helditemref))
          (`self.K2_SetActorTransform` _output_get (`KismetMathLibrary.MakeTransform` (+ _returnvalue_location (`self.PickupTransform`)) _returnvalue_rotation _returnvalue_scale) false true)
          (if (`self.HasPlayedCutscene`)
            (`self.UpdateAllObjects` true :!label _label)
            (else
              (bind _targetcutscenecamera (`self.TargetCutsceneCamera`)
                (:`then`
                  (`/Game/JourneyManContent/Blueprints/LevelObjects/CoreMechanics/BP_CutsceneCamera.Play Cutscene` _targetcutscenecamera)
                  (bind _asbp_third_person_character_2 (cast `/Game/JourneyManContent/Blueprints/Characters/Player/BP_ThirdPersonCharacter` (`GameplayStatics.GetPlayerPawn` 0))
                    (:`then`
                      (`/Game/JourneyManContent/Blueprints/Characters/Player/BP_ThirdPersonCharacter.StartCutscene` _asbp_third_person_character_2))
                    (:`CastFailed`
                      _))
                  (`KismetSystemLibrary.Delay` (+ (`/Game/JourneyManContent/Blueprints/LevelObjects/CoreMechanics/BP_CutsceneCamera.Camera Blend Time` _targetcutscenecamera) (* (`/Game/JourneyManContent/Blueprints/LevelObjects/CoreMechanics/BP_CutsceneCamera.Pause At Target Time` _targetcutscenecamera) 0.3)))
                  (`self.UpdateAllObjects` true)
                  (set `self.HasPlayedCutscene` true))
                (:`else`
                  (set `self.HasPlayedCutscene` true)
                  (goto _label))))))))))

(event `self.ReceiveTick`
  (params (DeltaSeconds :type "Float (single-precision)"))
  (bind _returnvalue (* (`KismetMathLibrary.MakeRotator` 0.0 (`self.SlotActorRotationSpeed`)) DeltaSeconds))
  (if (`self.HasPlayedCutscene`)
    (`/Engine/EditorBlueprintResources/StandardMacros.IsValid` (`self.PickupInSlot`)
      (:`Is Valid`
        (`self.K2_AddActorLocalRotation` (`self.PickupInSlot`) _returnvalue false false)
        (`|ExecutionSequence`
          (:`then_0`
            (`self.RotateChildren` _returnvalue (`self.Rotate`)))
          (:`then_1`
            (`self.RotateChildren` (`KismetMathLibrary.NegateRotator` _returnvalue) (`self.RotateOpposite`))))))))

(event `/Game/JourneyManContent/Blueprints/Interfaces/BPI_Interactable.OnPlayerHoverBegin`
  (bind _asbp_third_person_character (cast `/Game/JourneyManContent/Blueprints/Characters/Player/BP_ThirdPersonCharacter` (`GameplayStatics.GetPlayerPawn` 0)))
  (`/Game/JourneyManContent/Blueprints/Characters/Player/BP_ThirdPersonCharacter.HeldPickupableActor` _asbp_third_person_character
    (:`then`
      (`MeshComponent.SetOverlayMaterial` (`self.Mesh`) "/Game/JourneyManContent/Assets/Materials/Outline/MI_InteractOutline.MI_InteractOutline"))
    (:`else`)))

(event `/Game/JourneyManContent/Blueprints/Interfaces/BPI_Interactable.OnPlayerHoverEnd`
  (`MeshComponent.SetOverlayMaterial` (`self.Mesh`) null))

(fn `UpdateAllObjects`
  (params (IsActive :type Boolean))
  (for (_array_element _array_index) (`self.ObjectsToActivate`)
    (if (`KismetSystemLibrary.DoesImplementInterface` _array_element "/Game/JourneyManContent/Blueprints/Interfaces/BPI_Activate.BPI_Activate_C")
      (message `/Game/JourneyManContent/Blueprints/Interfaces/BPI_Activate.OnActivationChanged` _array_element IsActive)
      (else
        (bind _returnvalue (`self.GetComponentsByInterface` _array_element "/Game/JourneyManContent/Blueprints/Interfaces/BPI_Activate.BPI_Activate_C"))
        (if (> (`KismetArrayLibrary.Array_Length` _returnvalue) 0)
          (for _array_element_2 _returnvalue
            (message `/Game/JourneyManContent/Blueprints/Interfaces/BPI_Activate.OnActivationChanged` _array_element_2 IsActive))
          (else
            (`KismetSystemLibrary.PrintString` (`KismetStringLibrary.Concat_StrStr` "Object at index: " (`KismetStringLibrary.Conv_IntToString` _array_index) " does not implement BPI_Activate and cannot be activated") true true (struct :`R` 1.0 :`A` 1.0) 100.0)))))))

(fn `UserConstructionScript`)