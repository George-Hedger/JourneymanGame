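; BP_TestInteractable is a test interactable level object that gives debug feedback for hovering and interaction.
; Player hover begin and end events set a hovered flag and apply or clear an outline overlay material on its sphere.
; Tick prints an interact prompt while the flag is set, and the interact event prints a confirmation message.
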(event `/Game/JourneyManContent/Blueprints/Interfaces/BPI_Interactable.OnInteract`
  (`KismetSystemLibrary.PrintString` "Interacted!" true false))

(event `/Game/JourneyManContent/Blueprints/Interfaces/BPI_Interactable.OnPlayerHoverBegin`
  (set `self.IsHovered` true)
  (`MeshComponent.SetOverlayMaterial` (`self.Sphere`) "/Game/JourneyManContent/Assets/Materials/Outline/MI_InteractOutline.MI_InteractOutline"))

(event `/Game/JourneyManContent/Blueprints/Interfaces/BPI_Interactable.OnPlayerHoverEnd`
  (set `self.IsHovered` false)
  (`MeshComponent.SetOverlayMaterial` (`self.Sphere`) null))

(event `self.ReceiveTick`
  (params (DeltaSeconds :type "Float (single-precision)"))
  (if (`self.IsHovered`)
    (`KismetSystemLibrary.PrintString` "Press [Interact]" true false (struct :`G` 1.0 :`B` 0.40022 :`A` 1.0) 0.0)))

(fn `UserConstructionScript`)