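; BP_Cobweb is a level hazard that hampers the player character's movement while inside its Box trigger.
; On BeginPlay it caches player 0's max speed, jump velocity and horizontal dive speed, and optionally enables physics on its Wall component.
; Box overlap divides those cached values by separate slowdown and dampening factors, and end overlap restores them.
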(event `self.ReceiveBeginPlay`
  (`|ExecutionSequence`
    (:`then_0`
      (bind _asbp_third_person_character (cast `/Game/JourneyManContent/Blueprints/Characters/Player/BP_ThirdPersonCharacter` (`GameplayStatics.GetPlayerCharacter` 0)))
      (bind _charactermovement (`Character.CharacterMovement` _asbp_third_person_character))
      (set `self.Max speed` (`MovementComponent.GetMaxSpeed` _charactermovement))
      (set `self.Max jump` (`CharacterMovementComponent.JumpZVelocity` _charactermovement))
      (set `self.Max dive speed` (`/Game/JourneyManContent/Blueprints/Characters/Player/BP_ThirdPersonCharacter.DiveHorizontalSpeed` _asbp_third_person_character)))
    (:`then_1`
      (if (`self.Spawn with physics?`)
        (`PrimitiveComponent.SetSimulatePhysics` (`self.Wall`) true)))))

(event `self.Box.OnComponentBeginOverlap`
  (params (OverlappedComponent :type "PrimitiveComponent Object Reference") (OtherActor :type "Actor Object Reference") (OtherComp :type "PrimitiveComponent Object Reference") (OtherBodyIndex :type Integer) (bFromSweep :type Boolean) (SweepResult :type "HitResult Structure (by ref)"))
  (bind _asbp_third_person_character (cast `/Game/JourneyManContent/Blueprints/Characters/Player/BP_ThirdPersonCharacter` OtherActor))
  (bind _charactermovement (`Character.CharacterMovement` _asbp_third_person_character))
  (set `CharacterMovementComponent.MaxWalkSpeed` (/ (`self.Max speed`) (`self.Slowdown amount`)) _charactermovement)
  (set `CharacterMovementComponent.JumpZVelocity` (/ (`self.Max jump`) (`self.Jump dampen`)) _charactermovement)
  (set `/Game/JourneyManContent/Blueprints/Characters/Player/BP_ThirdPersonCharacter.DiveHorizontalSpeed` (/ (`self.Max dive speed`) (`self.Dive dampen`)) _asbp_third_person_character))

(event `self.Box.OnComponentEndOverlap`
  (params (OverlappedComponent :type "PrimitiveComponent Object Reference") (OtherActor :type "Actor Object Reference") (OtherComp :type "PrimitiveComponent Object Reference") (OtherBodyIndex :type Integer))
  (bind _asbp_third_person_character (cast `/Game/JourneyManContent/Blueprints/Characters/Player/BP_ThirdPersonCharacter` OtherActor))
  (bind _charactermovement (`Character.CharacterMovement` _asbp_third_person_character))
  (set `CharacterMovementComponent.MaxWalkSpeed` (`self.Max speed`) _charactermovement)
  (set `CharacterMovementComponent.JumpZVelocity` (`self.Max jump`) _charactermovement)
  (set `/Game/JourneyManContent/Blueprints/Characters/Player/BP_ThirdPersonCharacter.DiveHorizontalSpeed` (`self.Max dive speed`) _asbp_third_person_character))

(fn `UserConstructionScript`)