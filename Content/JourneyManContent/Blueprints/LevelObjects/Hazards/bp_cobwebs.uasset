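; Cobweb hazard that slows the player character and weakens its jump while the character overlaps it.
; On BeginPlay it caches the third-person player character along with its current max speed and jump Z velocity.
; Overlapping the Cobweb component divides those values by SlowdownAmount and JumpDampen, and ending the overlap restores the cached values.
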(event `self.ReceiveBeginPlay`
  (bind _asbp_third_person_character (cast `/Game/JourneyManContent/Blueprints/Characters/Player/BP_ThirdPersonCharacter` (`GameplayStatics.GetPlayerCharacter` 0)))
  (set `self.As BP Third Person Character` _asbp_third_person_character)
  (bind _charactermovement (`Character.CharacterMovement` _asbp_third_person_character))
  (set `self.Max speed` (`MovementComponent.GetMaxSpeed` _charactermovement))
  (set `self.Max jump` (`CharacterMovementComponent.JumpZVelocity` _charactermovement)))

(event `self.cobweb.OnComponentBeginOverlap`
  (params (OverlappedComponent :type "PrimitiveComponent Object Reference") (OtherActor :type "Actor Object Reference") (OtherComp :type "PrimitiveComponent Object Reference") (OtherBodyIndex :type Integer) (bFromSweep :type Boolean) (SweepResult :type "HitResult Structure (by ref)"))
  (bind _as_bp_third_person_character (`self.As BP Third Person Character`))
  (bind _charactermovement (`Character.CharacterMovement` _as_bp_third_person_character))
  (if (== OtherActor _as_bp_third_person_character)
    (set `CharacterMovementComponent.MaxWalkSpeed` (/ (`self.Max speed`) (`self.Slowdown amount`)) _charactermovement)
    (set `CharacterMovementComponent.JumpZVelocity` (/ (`self.Max jump`) (`self.Jump dampen`)) _charactermovement)))

(event `self.cobweb.OnComponentEndOverlap`
  (params (OverlappedComponent :type "PrimitiveComponent Object Reference") (OtherActor :type "Actor Object Reference") (OtherComp :type "PrimitiveComponent Object Reference") (OtherBodyIndex :type Integer))
  (bind _charactermovement (`Character.CharacterMovement` (`self.As BP Third Person Character`)))
  (if (== OtherActor (`self.As BP Third Person Character`))
    (set `CharacterMovementComponent.MaxWalkSpeed` (`self.Max speed`) _charactermovement)
    (set `CharacterMovementComponent.JumpZVelocity` (`self.Max jump`) _charactermovement)))

(fn `UserConstructionScript`)