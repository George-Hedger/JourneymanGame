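; Component that continuously spins its owning actor vertically, apparently for moving platforms among the level's core mechanics.
; Each tick it adds a local pitch rotation to the owner's root component, scaled by Speed and delta time.
; StopPlatform caches Speed in LastSpeed and zeroes it, and StartPlatform restores the cached value.
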(event `self.ReceiveTick`
  (params (DeltaSeconds :type "Float (single-precision)"))
  (`SceneComponent.K2_AddLocalRotation` (`Actor.RootComponent` (`self.GetOwner`)) (* (`KismetMathLibrary.MakeRotator` 0.0 (`self.Speed`)) DeltaSeconds) false false))

(event `Stop Platform`
  (set `self.Last Speed` (`self.Speed`))
  (set `self.Speed` 0.0))

(event `Start Platform`
  (set `self.Speed` (`self.Last Speed`)))