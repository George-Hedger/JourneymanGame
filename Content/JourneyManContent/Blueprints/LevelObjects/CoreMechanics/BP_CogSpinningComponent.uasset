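; BP_CogSpinningComponent is a component that continuously spins its owning actor, likely for cog-style level objects.
; Each Tick, while Enabled, it adds a local rotation of RotationAmount scaled by delta time to the owner's root component.
; StartPlatform and StopPlatform events toggle the Enabled flag to start or halt the spin.
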(event `self.ReceiveTick`
  (params (DeltaSeconds :type "Float (single-precision)"))
  (if (`self.Enabled`)
    (`SceneComponent.K2_AddLocalRotation` (`Actor.RootComponent` (`self.GetOwner`)) (* (`self.RotationAmount`) DeltaSeconds) false false)))

(event `Stop Platform`
  (set `self.Enabled` false))

(event `Start Platform`
  (set `self.Enabled` true))