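; A 2D gameplay section volume that switches the third-person character into 2D mode and blends the view to its own camera.
; While the player is inside, Tick moves the camera to the spline point closest to the pawn.
; Leaving the larger EndCollision box restores the character and its view, with paired DoOnce gates preventing repeat triggers.
; The construction script sizes both boxes and a preview cube that is hidden at BeginPlay.
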(event `self.ReceiveTick`
  (params (DeltaSeconds :type "Float (single-precision)"))
  (if (`self.Overlapped?`)
    (`SceneComponent.K2_SetWorldLocation` (`self.Camera`) (`SplineComponent.FindLocationClosestToWorldLocation` (`self.Spline`) (`self.K2_GetActorLocation` (`GameplayStatics.GetPlayerPawn` 0)) "World") false false)))

(event `self.ReceiveBeginPlay`
  (`SceneComponent.SetVisibility` (`self.Cube`) false false))

(event `self.Collision.OnComponentBeginOverlap`
  (params (OverlappedComponent :type "PrimitiveComponent Object Reference") (OtherActor :type "Actor Object Reference") (OtherComp :type "PrimitiveComponent Object Reference") (OtherBodyIndex :type Integer) (bFromSweep :type Boolean) (SweepResult :type "HitResult Structure (by ref)"))
  (bind _asbp_third_person_character (cast `/Game/JourneyManContent/Blueprints/Characters/Player/BP_ThirdPersonCharacter` OtherActor))
  (set `self.Overlapped?` true)
  (`/Engine/EditorBlueprintResources/StandardMacros.DoOnce` false :!label _label
    (:`Completed`
      (`|ExecutionSequence`
        (:`then_0`
          (`PlayerController.SetViewTargetWithBlend` (`GameplayStatics.GetPlayerController` 0) self 0.25 "VTBlend_Linear" 0.0 false)
          (`/Game/JourneyManContent/Blueprints/Characters/Player/BP_ThirdPersonCharacter.2DStart` _asbp_third_person_character self))
        (:`then_1`
          (goto _label_2 :!via `Reset`))))))

(event `self.EndCollision.OnComponentEndOverlap`
  (params (OverlappedComponent :type "PrimitiveComponent Object Reference") (OtherActor :type "Actor Object Reference") (OtherComp :type "PrimitiveComponent Object Reference") (OtherBodyIndex :type Integer))
  (bind _asbp_third_person_character (cast `/Game/JourneyManContent/Blueprints/Characters/Player/BP_ThirdPersonCharacter` OtherActor))
  (set `self.Overlapped?` false)
  (`/Engine/EditorBlueprintResources/StandardMacros.DoOnce` true :!label _label_2
    (:`Completed`
      (`|ExecutionSequence`
        (:`then_0`
          (`/Game/JourneyManContent/Blueprints/Characters/Player/BP_ThirdPersonCharacter.2DEnd` _asbp_third_person_character)
          (`PlayerController.SetViewTargetWithBlend` (`GameplayStatics.GetPlayerController` 0) _asbp_third_person_character 0.25 "VTBlend_Linear" 0.0 false))
        (:`then_1`
          (goto _label :!via `Reset`))))))

(fn `UserConstructionScript`
  (`SceneComponent.K2_SetRelativeLocation` (`self.Collision`) (* (`self.Size`) (`self.OffsetMultipliers`)) false false)
  (`BoxComponent.SetBoxExtent` (`self.Collision`) (`self.Size`) true)
  (`BoxComponent.SetBoxExtent` (`self.EndCollision`) (+ (`self.Size`) (`self.EndCollisionExtent`)) true)
  (`SceneComponent.SetWorldScale3D` (`self.Cube`) (/ (`BoxComponent.BoxExtent` (`self.Collision`)) 50)))