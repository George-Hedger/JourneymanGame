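; Actor component that gives its owning level object a timeslow multiplier, easing it down when slowed and back to normal when released.
; Start and stop events set the target and open a Tick-driven gate, which closes once the multiplier reaches that target.
; While open, the gate broadcasts a multiplier-changed dispatcher and interpolates the value at constant speed each frame.
; Player hover begin and end events are empty.
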(event `Timeslow Player Hover Begin`)

(event `Timeslow Player Hover End`)

(event `Timeslow Start`
  (set `self.Timeslow Target` 0.1)
  (goto _label :!via `Open`))

(event `Timeslow Stop`
  (set `self.Timeslow Target` 1.0)
  (goto _label :!via `Open`))

(event `self.ReceiveTick`
  (params (DeltaSeconds :type "Float (single-precision)"))
  (`/Engine/EditorBlueprintResources/StandardMacros.Gate` true :!label _label
    (:`Exit`
      (`self.OnMultiplierChanged`)
      (bind _output_get (set `self.Timeslow Multiplier` (`KismetMathLibrary.FInterpTo_Constant` (`self.Timeslow Multiplier`) (`self.Timeslow Target`) DeltaSeconds (`self.Interp Speed`))))
      (if (== _output_get (`self.Timeslow Target`))
        (goto _label :!via `Close`)))))