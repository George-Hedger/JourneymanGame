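; AC_CogSpinningComponent is an actor component that spins its owning actor, intended for cogs in level objects.
; Each tick while enabled, it adds a local rotation to the owner's root component, scaled by delta time.
; If the owner has an AC_Timeslow component, found on BeginPlay, its multiplier also scales the spin.
; An activation-change event switches the spinning on or off.
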(event `self.ReceiveTick`
  (params (DeltaSeconds :type "Float (single-precision)"))
  (if (`self.Enabled`)
    (`SceneComponent.K2_AddLocalRotation` (`Actor.RootComponent` (`self.GetOwner`)) (* (`self.RotationAmount`) (* DeltaSeconds (`KismetMathLibrary.SelectFloat` (`/Game/JourneyManContent/Blueprints/LevelObjects/CoreMechanics/AC_Timeslow.Timeslow Multiplier` (`self.Timeslow`)) 1.0 (`self.Timeslow exists?`)))) false false)))

(event `/Game/JourneyManContent/Blueprints/Interfaces/BPI_Activate.OnActivationChanged`
  (params (IsActive :type Boolean))
  (set `self.Enabled` IsActive))

(event `self.ReceiveBeginPlay`
  (bind _returnvalue (`Actor.GetComponentByClass` (`self.GetOwner`) "/Game/JourneyManContent/Blueprints/LevelObjects/CoreMechanics/AC_Timeslow.AC_Timeslow_C"))
  (`/Engine/EditorBlueprintResources/StandardMacros.IsValid` _returnvalue
    (:`Is Valid`
      (set `self.Timeslow exists?` true)
      (set `self.Timeslow` _returnvalue))
    (:`Is Not Valid`
      (set `self.Timeslow exists?` false))))