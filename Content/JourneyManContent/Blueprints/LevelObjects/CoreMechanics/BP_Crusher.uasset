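; BP_Crusher is a level hazard that moves back and forth along a spline and kills the player on contact.
; A timeline starts on BeginPlay, maps its track to distance along the spline to position the Crusher without sweeping, and flips direction each time it finishes.
; A Box overlap with the player character calls OnDeath on BP_Base_Character.
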(event `self.ReceiveBeginPlay`
  (bind (_direction _newtrack_0) (`Timeline|Timeline` :!label _label)
    (:`Update`
      (`SceneComponent.K2_SetWorldLocation` (`self.Crusher`) (`SplineComponent.GetLocationAtDistanceAlongSpline` (`self.Spline`) (`KismetMathLibrary.Lerp` 0.0 (`SplineComponent.GetSplineLength` (`self.Spline`)) _newtrack_0) "World") false false))
    (:`Finished`
      (switch `ETimelineDirection` _direction
        (:`Forward`
          (goto _label :!via `Reverse`))
        (:`Backward`
          (goto _label))))))

(event `self.Box.OnComponentBeginOverlap`
  (params (OverlappedComponent :type "PrimitiveComponent Object Reference") (OtherActor :type "Actor Object Reference") (OtherComp :type "PrimitiveComponent Object Reference") (OtherBodyIndex :type Integer) (bFromSweep :type Boolean) (SweepResult :type "HitResult Structure (by ref)"))
  (bind _returnvalue (`GameplayStatics.GetPlayerCharacter` 0))
  (if (== OtherActor _returnvalue)
    (bind _asbp_base_character (cast `/Game/JourneyManContent/Blueprints/Characters/BP_Base_Character` _returnvalue))
    (`/Game/JourneyManContent/Blueprints/Characters/BP_Base_Character.OnDeath` _asbp_base_character)))

(fn `UserConstructionScript`)