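; Level-building Blueprint that assembles a conveyor platform of configurable length and speed in its construction script.
; It adds static mesh components at a fixed spacing, capping the Sections middle pieces with an end mesh on each side.
; A hidden BP_Conveyor child actor is scaled and centered along the run and receives Speed.
; An arrow is centered above the belt and flips when Speed is negative.
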(event `self.ReceiveBeginPlay`)

(fn `UserConstructionScript`
  (bind _childactor (`self.ChildActor`))
  (bind _childactor_2 (`self.ChildActor`))
  (`|ExecutionSequence`
    (:`then_0`
      (`SceneComponent.K2_SetRelativeLocation` _childactor_2 (`KismetMathLibrary.MakeVector` (* (`KismetMathLibrary.Conv_IntToDouble` (`self.Sections`)) 499.5 0.5) 0.0 45.0) false false)
      (`SceneComponent.SetRelativeScale3D` _childactor_2 (`KismetMathLibrary.MakeVector` (* (+ (* (`KismetMathLibrary.Conv_IntToDouble` (`self.Sections`)) 499.5) 200.0) 0.01) 3.84 1.0))
      (`ChildActorComponent.SetChildActorClass` _childactor "/Game/JourneyManContent/Blueprints/LevelObjects/Platforms/BP_Conveyor.BP_Conveyor_C")
      (bind _asbp_conveyor (cast `/Game/JourneyManContent/Blueprints/LevelObjects/Platforms/BP_Conveyor` (`ChildActorComponent.ChildActor` _childactor)))
      (set `/Game/JourneyManContent/Blueprints/LevelObjects/Platforms/BP_Conveyor.Conveyor Speed` (`self.Speed`) _asbp_conveyor))
    (:`then_1`
      (for _index (range (+ (+ (`self.Sections`) 1) 1))
        (if (or (== (+ (`self.Sections`) 1) _index) (== 0 _index))
          (if (== _index 0)
            (bind _returnvalue (`AddComponent|NODE_AddStaticMeshComponent-1` :`RelativeTransform` (`KismetMathLibrary.MakeTransform` (0.0 0.0 0.0) (struct :`Yaw` 180.0))))
            (`StaticMeshComponent.SetStaticMesh` _returnvalue "/Game/JourneyManContent/Assets/NewMeshes/Platforms/SM_ConveyorEnd.SM_ConveyorEnd")
            (else
              (bind _returnvalue_2 (`AddComponent|NODE_AddStaticMeshComponent-2` :`RelativeTransform` (`KismetMathLibrary.MakeTransform` (`KismetMathLibrary.MakeVector` (* (`KismetMathLibrary.Conv_IntToDouble` (- _index 1)) 499.5)))))
              (`StaticMeshComponent.SetStaticMesh` _returnvalue_2 "/Game/JourneyManContent/Assets/NewMeshes/Platforms/SM_ConveyorEnd.SM_ConveyorEnd")))
          (else
            (bind _returnvalue_3 (`AddComponent|NODE_AddStaticMeshComponent-0` :`RelativeTransform` (`KismetMathLibrary.MakeTransform` (`KismetMathLibrary.MakeVector` (* (`KismetMathLibrary.Conv_IntToDouble` (- _index 1)) 499.5)))))
            (`StaticMeshComponent.SetStaticMesh` _returnvalue_3 "/Game/JourneyManContent/Assets/NewMeshes/Platforms/SM_ConveyorMiddle.SM_ConveyorMiddle")))))
    (:`then_2`
      (`SceneComponent.SetVisibility` (`self.ChildActor`) false false))
    (:`then_3`
      (`SceneComponent.K2_SetRelativeLocation` (`self.Arrow`) (`KismetMathLibrary.MakeVector` (* (`KismetMathLibrary.Conv_IntToDouble` (`self.Sections`)) 499.5 0.5) 0.0 60.0) false false)
      (if (< (`self.Speed`) 0.0)
        (`SceneComponent.K2_SetRelativeRotation` (`self.Arrow`) (struct :`Yaw` 180.0) false false)))))