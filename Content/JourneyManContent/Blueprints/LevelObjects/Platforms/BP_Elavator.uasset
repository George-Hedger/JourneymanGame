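; Elevator platform that rises while the player character stands in its trigger box and lowers when they leave.
; A timeline paced by SecondsToExtend moves Cube up to the Arrow's relative height and stretches Cube1 vertically to match.
; An Elavate event also toggles the motion through a FlipFlop.
; When the timeline finishes, in either direction, it opens LevelWhichOpenOnExtend if one is set.
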(event `self.ReceiveBeginPlay`
  (bind _asbp_third_person_character (cast `/Game/JourneyManContent/Blueprints/Characters/Player/BP_ThirdPersonCharacter` (`GameplayStatics.GetPlayerCharacter` 0)))
  (set `self.As BP Third Person Character` _asbp_third_person_character)
  (`TimelineComponent.SetPlayRate` (`self.Timeline`) (/ 1.0 (`self.Seconds to extend`))))

(event `Elavate`
  (bind _cube1 (`self.Cube1`))
  (bind (_relativelocation_x _relativelocation_y _relativelocation_z) (`KismetMathLibrary.BreakVector` (`SceneComponent.RelativeLocation` (`self.Arrow`))))
  (bind (_relativescale3d_x _relativescale3d_y) (`KismetMathLibrary.BreakVector` (`SceneComponent.RelativeScale3D` _cube1)))
  (`/Engine/EditorBlueprintResources/StandardMacros.FlipFlop`
    (:`A`
      (bind (_direction _newtrack_0) (`Timeline|Timeline` :!label _label)
        (:`Update`
          (bind _returnvalue (* _newtrack_0 _relativelocation_z))
          (`SceneComponent.K2_SetRelativeLocation` (`self.Cube`) (`KismetMathLibrary.MakeVector` 0.0 0.0 _returnvalue) false false)
          (`SceneComponent.SetRelativeScale3D` _cube1 (`KismetMathLibrary.MakeVector` _relativescale3d_x _relativescale3d_y (/ _returnvalue 100.0))))
        (:`Finished`
          (bind _level_which_open_on_extend (`self.Level which open on extend`)
            (:`then`
              (`GameplayStatics.OpenLevelBySoftObjectPtr` _level_which_open_on_extend))
            (:`else`)))))
    (:`B`
      (goto _label :!via `Reverse`))))

(event `self.Box.OnComponentBeginOverlap`
  (params (OverlappedComponent :type "PrimitiveComponent Object Reference") (OtherActor :type "Actor Object Reference") (OtherComp :type "PrimitiveComponent Object Reference") (OtherBodyIndex :type Integer) (bFromSweep :type Boolean) (SweepResult :type "HitResult Structure (by ref)"))
  (if (== OtherActor (`self.As BP Third Person Character`))
    (goto _label)))

(event `self.Box.OnComponentEndOverlap`
  (params (OverlappedComponent :type "PrimitiveComponent Object Reference") (OtherActor :type "Actor Object Reference") (OtherComp :type "PrimitiveComponent Object Reference") (OtherBodyIndex :type Integer))
  (if (== (`self.As BP Third Person Character`) OtherActor)
    (goto _label :!via `Reverse`)))

(fn `UserConstructionScript`)