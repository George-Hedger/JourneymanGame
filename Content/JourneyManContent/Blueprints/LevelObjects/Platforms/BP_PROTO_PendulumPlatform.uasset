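; Prototype moving platform that travels back and forth along a spline, toggled by StartPlatform and StopPlatform events.
; A timeline alpha maps to distance along the spline and sets the platform's world location each update without sweeping.
; BeginPlay scales the timeline play rate by Speed over spline length, so travel speed accounts for path length.
; When the timeline finishes, it flips direction for a continuous ping-pong swing.
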(event `self.ReceiveBeginPlay`
  (`TimelineComponent.SetPlayRate` (`self.Timeline`) (* (/ 1.0 (`SplineComponent.GetSplineLength` (`self.Spline`))) (`self.Speed`))))

(event `StartPlatform`
  (bind _spline (`self.Spline`))
  (bind (_direction _alpha) (`Timeline|Timeline` :!label _label)
    (:`Update`
      (`SceneComponent.K2_SetWorldLocation` (`self.Temp_platform`) (`SplineComponent.GetLocationAtDistanceAlongSpline` _spline (`KismetMathLibrary.Lerp` 0.0 (`SplineComponent.GetSplineLength` _spline) _alpha) "World") false false))
    (:`Finished`
      (switch `ETimelineDirection` _direction
        (:`Forward`
          (goto _label :!via `Reverse`))
        (:`Backward`
          (goto _label))))))

(event `StopPlatform`
  (goto _label :!via `Stop`))

(fn `UserConstructionScript`)