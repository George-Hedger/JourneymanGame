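; Elevator platform that unlocks once enough cog activations are counted, then carries the player up and optionally opens another level.
; Entering its box switches the view to the elevator and closes the door, which triggers the lift.
; Timelines scale the door and raise the platform to the Arrow's height while stretching a cube beneath, updating only while enabled.
; At the top it opens the level or door, descending when the player leaves.
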(event `/Game/JourneyManContent/Blueprints/Interfaces/BPI_Activate.OnActivationChanged`
  (params (IsActive :type Boolean))
  (bind _output_get (set `self.NumberActivations` (`KismetMathLibrary.Max` (+ (`self.NumberActivations`) (`KismetMathLibrary.SelectInt` 1 -1 IsActive)))))
  (if (>= _output_get (`self.NumberOfCogActivationsForActive`))
    (`TimelineComponent.ReverseFromEnd` (`self.Door timeline`))))

(event `self.ReceiveBeginPlay`
  (`TimelineComponent.SetPlayRate` (`self.Elevate Timeline`) (/ 1.0 (`self.Seconds to extend`)))
  (if (`self.IsActive`)
    (set `self.NumberActivations` (`self.NumberOfCogActivationsForActive`))))

(event `Elevate`
  (bind _cube1 (`self.Cube1`))
  (bind (_relativescale3d_x _relativescale3d_y) (`KismetMathLibrary.BreakVector` (`SceneComponent.RelativeScale3D` _cube1)))
  (bind (_relativelocation_x _relativelocation_y _relativelocation_z) (`KismetMathLibrary.BreakVector` (`SceneComponent.RelativeLocation` (`self.Arrow`))))
  (`/Engine/EditorBlueprintResources/StandardMacros.FlipFlop`
    (:`A`
      (bind (_direction _newtrack_0) (`Timeline|Elevate Timeline` :!label _label)
        (:`Update`
          (if (`self.IsEnablesd`)
            (bind _returnvalue (* _newtrack_0 _relativelocation_z))
            (`SceneComponent.K2_SetRelativeLocation` (`self.Platform`) (`KismetMathLibrary.MakeVector` 0.0 0.0 _returnvalue) false false)
            (`SceneComponent.SetRelativeScale3D` _cube1 (`KismetMathLibrary.MakeVector` _relativescale3d_x _relativescale3d_y (/ _returnvalue 100.0)))))
        (:`Finished`
          (if (`self.Up?`)
            (`self.As BP Third Person Character`
              (:`then`
                (bind _level_which_open_on_extend (`self.Level which open on extend`)
                  (:`then`
                    (`GameplayStatics.OpenLevelBySoftObjectPtr` _level_which_open_on_extend))
                  (:`else`
                    (`self.Open doors`))))
              (:`else`
                (`self.Go down`)))
            (elif (`self.Doors closed?`)
              (`self.Open doors`))))))
    (:`B`
      (goto _label :!via `Reverse`))))

(event `go Up`
  (set `self.Up?` true)
  (goto _label))

(event `Go down`
  (set `self.Up?` false)
  (goto _label :!via `Reverse`))

(event `self.Box.OnComponentBeginOverlap`
  (params (OverlappedComponent :type "PrimitiveComponent Object Reference") (OtherActor :type "Actor Object Reference") (OtherComp :type "PrimitiveComponent Object Reference") (OtherBodyIndex :type Integer) (bFromSweep :type Boolean) (SweepResult :type "HitResult Structure (by ref)"))
  (bind _asbp_third_person_character (cast `/Game/JourneyManContent/Blueprints/Characters/Player/BP_ThirdPersonCharacter` OtherActor))
  (set `self.As BP Third Person Character` _asbp_third_person_character)
  (`PlayerController.SetViewTargetWithBlend` (`GameplayStatics.GetPlayerController` 0) self 0.0 "VTBlend_Linear" 0.0 false)
  (`self.Close doors`))

(event `self.Box.OnComponentEndOverlap`
  (params (OverlappedComponent :type "PrimitiveComponent Object Reference") (OtherActor :type "Actor Object Reference") (OtherComp :type "PrimitiveComponent Object Reference") (OtherBodyIndex :type Integer))
  (cast `/Game/JourneyManContent/Blueprints/Characters/Player/BP_ThirdPersonCharacter` OtherActor)
  (set `self.As BP Third Person Character` null)
  (`PlayerController.SetViewTargetWithBlend` (`GameplayStatics.GetPlayerController` 0) (`GameplayStatics.GetPlayerPawn` 0) 0.0 "VTBlend_Linear" 0.0 false)
  (if (`self.Up?`)
    (`self.Go down`)
    (else
      (`self.Open doors`))))

(event `Close doors`
  (bind _door (`self.Door`))
  (bind (_relativescale3d_x _relativescale3d_y _relativescale3d_z) (`KismetMathLibrary.BreakVector` (`SceneComponent.RelativeScale3D` _door)))
  (set `self.Doors closed?` true)
  (bind (_direction _newtrack_0) (`Timeline|Door timeline` :!label _label_2)
    (:`Update`
      (if (`self.IsEnablesd`)
        (`SceneComponent.SetRelativeScale3D` _door (`KismetMathLibrary.MakeVector` (* _newtrack_0 0.7) _relativescale3d_y _relativescale3d_z))))
    (:`Finished`
      (if (`self.Doors closed?`)
        (`self.As BP Third Person Character`
          (:`then`
            (`self.go Up`))
          (:`else`
            (`self.Open doors`)))))))

(event `Open doors`
  (set `self.Doors closed?` false)
  (goto _label_2 :!via `Reverse`))

(fn `IsEnablesd`
  (returns (Enabled :type Boolean))
  (return (>= (`self.NumberActivations`) (`self.NumberOfCogActivationsForActive`))))

(fn `UserConstructionScript`
  (bind _door (`self.Door`))
  (bind (_relativescale3d_x _relativescale3d_y _relativescale3d_z) (`KismetMathLibrary.BreakVector` (`SceneComponent.RelativeScale3D` _door)))
  (if (not (`self.IsActive`))
    (`SceneComponent.SetRelativeScale3D` _door (`KismetMathLibrary.MakeVector` 0.7 _relativescale3d_y _relativescale3d_z))))