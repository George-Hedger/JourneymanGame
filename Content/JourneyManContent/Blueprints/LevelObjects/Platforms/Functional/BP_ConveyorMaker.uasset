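; Modular conveyor platform that pushes the third-person player along its length while active.
; Construction script assembles end and middle meshes from Sections, fits the trigger box and centers the arrow, flipping it for negative Speed.
; Tick moves the overlapping player along the arrow with a swept offset, scaled by speed and the timeslow multiplier.
; Activation changes toggle movement, with setup and working sounds played on first activation.
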(event `self.Box.OnComponentBeginOverlap`
  (params (OverlappedComponent :type "PrimitiveComponent Object Reference") (OtherActor :type "Actor Object Reference") (OtherComp :type "PrimitiveComponent Object Reference") (OtherBodyIndex :type Integer) (bFromSweep :type Boolean) (SweepResult :type "HitResult Structure (by ref)"))
  (bind _asbp_third_person_character (cast `/Game/JourneyManContent/Blueprints/Characters/Player/BP_ThirdPersonCharacter` OtherActor))
  (set `self.Player Ref` _asbp_third_person_character))

(event `self.Box.OnComponentEndOverlap`
  (params (OverlappedComponent :type "PrimitiveComponent Object Reference") (OtherActor :type "Actor Object Reference") (OtherComp :type "PrimitiveComponent Object Reference") (OtherBodyIndex :type Integer))
  (cast `/Game/JourneyManContent/Blueprints/Characters/Player/BP_ThirdPersonCharacter` OtherActor)
  (set `self.Player Ref` null))

(event `self.ReceiveTick`
  (params (DeltaSeconds :type "Float (single-precision)"))
  (`/Engine/EditorBlueprintResources/StandardMacros.IsValid` (`self.Player Ref`)
    (:`Is Valid`
      (if (`self.IsActive`)
        (`self.K2_AddActorWorldOffset` (`self.Player Ref`) (* (`SceneComponent.GetForwardVector` (`self.Arrow`)) (`KismetMathLibrary.Abs` (`self.Conveyor Speed`)) DeltaSeconds (`/Game/JourneyManContent/Blueprints/Components/AC_Timeslow.Timeslow Multiplier` (`self.AC_Timeslow`))) true false)))))

(event `/Game/JourneyManContent/Blueprints/Interfaces/BPI_Activate.OnActivationChanged`
  (params (IsActive :type Boolean))
  (bind _returnvalue (`SceneComponent.K2_GetComponentLocation` (`self.DefaultSceneRoot`)))
  (bind _output_get (set `self.IsActive` IsActive))
  (if _output_get
    (`/Engine/EditorBlueprintResources/StandardMacros.DoOnce` false
      (:`Completed`
        (`GameplayStatics.PlaySoundAtLocation` "/Game/JourneyManContent/Assets/SFX/Level/Conveyor/SQ_Conveyor_Setup1.SQ_Conveyor_Setup1" _returnvalue (struct) 1.0 1.0 0.0 "/Game/JourneyManContent/Assets/SFX/SoundAttenuation/SA_General.SA_General" null null null)
        (`GameplayStatics.PlaySoundAtLocation` "/Game/JourneyManContent/Assets/SFX/Level/Conveyor/SQ_Conveyor_Working4.SQ_Conveyor_Working4" _returnvalue (struct) 4.0 1.0 0.0 "/Game/JourneyManContent/Assets/SFX/SoundAttenuation/SA_General.SA_General" null null null)))))

(event `self.ReceiveBeginPlay`
  (if (`self.IsActive`)
    (`GameplayStatics.PlaySoundAtLocation` "/Game/JourneyManContent/Assets/SFX/Level/Conveyor/SQ_Conveyor_Working4.SQ_Conveyor_Working4" (`SceneComponent.K2_GetComponentLocation` (`self.DefaultSceneRoot`)) (struct) 1.0 1.0 0.0 "/Game/JourneyManContent/Assets/SFX/SoundAttenuation/SA_General.SA_General" null null null)))

(fn `UserConstructionScript`
  (bind _box (`self.Box`))
  (`|ExecutionSequence`
    (:`then_0`
      (`SceneComponent.K2_SetRelativeLocation` _box (`KismetMathLibrary.MakeVector` (* (`KismetMathLibrary.Conv_IntToDouble` (`self.Sections`)) 499.5 0.5) 0.0 45.0) false false)
      (`SceneComponent.SetRelativeScale3D` _box (`KismetMathLibrary.MakeVector` (* (+ (* (`KismetMathLibrary.Conv_IntToDouble` (`self.Sections`)) 499.5) 200.0) 0.015) 6.0 1.0))
      (set `self.Conveyor Speed` (`self.Speed`)))
    (:`then_1`
      (for _index (range (+ (+ (`self.Sections`) 1) 1))
        (if (or (== (+ (`self.Sections`) 1) _index) (== 0 _index))
          (if (== _index 0)
            (bind _returnvalue (`AddComponent|NODE_AddStaticMeshComponent-1` :`RelativeTransform` (`KismetMathLibrary.MakeTransform` (0.0 0.0 0.0) (struct :`Yaw` 180.0))))
            (`StaticMeshComponent.SetStaticMesh` _returnvalue "/Game/JourneyManContent/Assets/StaticMeshes/Interactive/MovementObjects/SM_ConveyorEnd.SM_ConveyorEnd")
            (else
              (bind _returnvalue_2 (`AddComponent|NODE_AddStaticMeshComponent-2` :`RelativeTransform` (`KismetMathLibrary.MakeTransform` (`KismetMathLibrary.MakeVector` (* (`KismetMathLibrary.Conv_IntToDouble` (- _index 1)) 499.5)))))
              (`StaticMeshComponent.SetStaticMesh` _returnvalue_2 "/Game/JourneyManContent/Assets/StaticMeshes/Interactive/MovementObjects/SM_ConveyorEnd.SM_ConveyorEnd")))
          (else
            (bind _returnvalue_3 (`AddComponent|NODE_AddStaticMeshComponent-0` :`RelativeTransform` (`KismetMathLibrary.MakeTransform` (`KismetMathLibrary.MakeVector` (* (`KismetMathLibrary.Conv_IntToDouble` (- _index 1)) 499.5)))))
            (`StaticMeshComponent.SetStaticMesh` _returnvalue_3 "/Game/JourneyManContent/Assets/StaticMeshes/Interactive/MovementObjects/SM_ConveyorMiddle.SM_ConveyorMiddle")))))
    (:`then_2`
      (`SceneComponent.SetVisibility` (`self.ChildActor`) false false))
    (:`then_3`
      (`SceneComponent.K2_SetRelativeLocation` (`self.Arrow`) (`KismetMathLibrary.MakeVector` (* (`KismetMathLibrary.Conv_IntToDouble` (`self.Sections`)) 499.5 0.5) 0.0 60.0) false false)
      (if (< (`self.Speed`) 0.0)
        (`SceneComponent.K2_SetRelativeRotation` (`self.Arrow`) (struct :`Yaw` 180.0) false false)))))