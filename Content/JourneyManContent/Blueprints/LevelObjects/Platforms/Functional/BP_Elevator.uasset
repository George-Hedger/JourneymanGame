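; Cog-gated level elevator that carries the player to the Arrow's position and can then open another level.
; Enough cog activations enable the door; entering the box switches to the elevator camera and closes it.
; The ride is faked: gears spin during a delay with a results widget added, then platform and player teleport and doors reopen.
; Instanced chain meshes are built from the Arrow distance and cleared on arrival.
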(event `self.ReceiveBeginPlay`
  (if (`self.IsActive`)
    (set `self.NumberActivations` (`self.NumberOfCogActivationsForActive`)))
  (`self.UpdateChain`))

(event `/Game/JourneyManContent/Blueprints/Interfaces/BPI_Activate.OnActivationChanged`
  (params (IsActive :type Boolean))
  (bind _output_get (set `self.NumberActivations` (`KismetMathLibrary.Max` (+ (`self.NumberActivations`) (`KismetMathLibrary.SelectInt` 1 -1 IsActive)))))
  (if (>= _output_get (`self.NumberOfCogActivationsForActive`))
    (`TimelineComponent.ReverseFromEnd` (`self.Door timeline`))))

(event `self.Box.OnComponentBeginOverlap`
  (params (OverlappedComponent :type "PrimitiveComponent Object Reference") (OtherActor :type "Actor Object Reference") (OtherComp :type "PrimitiveComponent Object Reference") (OtherBodyIndex :type Integer) (bFromSweep :type Boolean) (SweepResult :type "HitResult Structure (by ref)"))
  (bind _asbp_third_person_character (cast `/Game/JourneyManContent/Blueprints/Characters/Player/BP_ThirdPersonCharacter` OtherActor))
  (set `self.As BP Third Person Character` _asbp_third_person_character)
  (`PlayerController.SetViewTargetWithBlend` (`GameplayStatics.GetPlayerController` 0) self 0.0 "VTBlend_Linear" 0.0 false)
  (`/Game/JourneyManContent/Blueprints/Characters/Player/BP_ThirdPersonCharacter.SetCanMoveCamera` (`self.As BP Third Person Character`) false)
  (`SceneComponent.K2_SetRelativeRotation` (`/Game/JourneyManContent/Blueprints/Characters/Player/BP_ThirdPersonCharacter.CameraBoom` (`self.As BP Third Person Character`)) (`KismetMathLibrary.ComposeRotators` (`SceneComponent.K2_GetComponentRotation` (`self.Camera`)) (`KismetMathLibrary.NegateRotator` (`self.K2_GetActorRotation` (`self.As BP Third Person Character`)))) false false)
  (if (not (`self.Has moved?`))
    (`self.Close doors`)))

(event `self.Box.OnComponentEndOverlap`
  (params (OverlappedComponent :type "PrimitiveComponent Object Reference") (OtherActor :type "Actor Object Reference") (OtherComp :type "PrimitiveComponent Object Reference") (OtherBodyIndex :type Integer))
  (bind _results_ref (`self.Results ref`))
  (cast `/Game/JourneyManContent/Blueprints/Characters/Player/BP_ThirdPersonCharacter` OtherActor)
  (`PlayerController.SetViewTargetWithBlend` (`GameplayStatics.GetPlayerController` 0) (`GameplayStatics.GetPlayerPawn` 0) 0.0 "VTBlend_Linear" 0.0 false)
  (`/Game/JourneyManContent/Blueprints/Characters/Player/BP_ThirdPersonCharacter.SetCanMoveCamera` (`self.As BP Third Person Character`) true)
  (set `self.As BP Third Person Character` null)
  (`/Engine/EditorBlueprintResources/StandardMacros.IsValid` _results_ref
    (:`Is Valid`
      (`Widget.RemoveFromParent` _results_ref)
      (set `self.Results ref` null))))

(event `Close doors`
  (bind _door (`self.Door`))
  (bind (_relativescale3d_x _relativescale3d_y _relativescale3d_z) (`KismetMathLibrary.BreakVector` (`SceneComponent.RelativeScale3D` _door)))
  ; Comment
  (bind (_direction _newtrack_0) (`Timeline|Door timeline` :!label _label)
    (:`Update`
      (if (`self.IsEnablesd`)
        (`SceneComponent.SetRelativeScale3D` _door (`KismetMathLibrary.MakeVector` (* _newtrack_0 0.5) _relativescale3d_y _relativescale3d_z))))
    (:`Finished`
      (`self.As BP Third Person Character`
        (:`then`
          (switch `ETimelineDirection` _direction
            (:`Forward`
              (`self.Move elevator`)
              (bind _returnvalue (`|CreateWidget` "/Game/JourneyManContent/Blueprints/Widgets/Results/WBP_Results.WBP_Results_C"))
              (bind _output_get (set `self.Results ref` _returnvalue))
              (`UserWidget.AddToViewport` _output_get 0))))
        (:`else`
          (`self.Open doors`))))))

(event `Open doors`
  ; Comment
  (goto _label :!via `Reverse`))

(event `Move elevator`
  (bind _returnvalue (`GameplayStatics.GetPlayerPawn` 0))
  ; Comment
  (set `self.Has moved?` true)
  (set `self.Gear Rotate` true)
  (`KismetSystemLibrary.Delay` (`self.Time until doors open`))
  (bind _asbp_third_person_character (cast `/Game/JourneyManContent/Blueprints/Characters/Player/BP_ThirdPersonCharacter` _returnvalue)
    (:`then`
      (`/Game/JourneyManContent/Blueprints/Characters/Player/BP_ThirdPersonCharacter.EnableBarrier` _asbp_third_person_character))
    (:`CastFailed`
      _))
  (set `self.PlayerOffset` (- (`self.K2_GetActorLocation` _returnvalue) (`self.K2_GetActorLocation`)))
  (`SceneComponent.K2_SetRelativeLocation` (`self.Platform`) (`SceneComponent.RelativeLocation` (`self.Arrow`)) false true)
  (`self.K2_SetActorLocation` (`GameplayStatics.GetPlayerPawn` 0) (+ (`self.PlayerOffset`) (`self.K2_GetActorLocation`)) false true)
  (`InstancedStaticMeshComponent.ClearInstances` (`self.Chain`))
  (`self.Open doors`)
  (set `self.Gear Rotate` false)
  (bind _level_which_open_on_extend (`self.Level which open on extend`)
    (:`then`
      (`GameplayStatics.OpenLevelBySoftObjectPtr` _level_which_open_on_extend))
    (:`else`)))

(event `self.ReceiveTick`
  (params (DeltaSeconds :type "Float (single-precision)"))
  ; Cog spinning
  (if (`self.Gear Rotate`)
    (`SceneComponent.K2_AddWorldRotation` (`self.Gear`) (`KismetMathLibrary.MakeRotator` 0.0 -1.0) false false)
    (`SceneComponent.K2_AddWorldRotation` (`self.Gear2`) (`KismetMathLibrary.MakeRotator` 0.0 -1.0) false false)))

(fn `IsEnablesd`
  (returns (Enabled :type Boolean))
  (return (>= (`self.NumberActivations`) (`self.NumberOfCogActivationsForActive`))))

(fn `UpdateChain`
  (bind (_returnvalue_x _returnvalue_y _returnvalue_z) (`KismetMathLibrary.BreakVector` (`SceneComponent.K2_GetComponentLocation` (`self.ChainStart`))))
  (`InstancedStaticMeshComponent.ClearInstances` (`self.Chain`))
  (for _index (range (+ (`KismetMathLibrary.FCeil` (/ (`KismetMathLibrary.VSize` (- (`SceneComponent.RelativeLocation` (`self.Arrow`)) (`SceneComponent.RelativeLocation` (`self.ChainStart`)))) 155.0)) 1))
    (`InstancedStaticMeshComponent.AddInstance` (`self.Chain`) (`KismetMathLibrary.MakeTransform` (`KismetMathLibrary.MakeVector` _returnvalue_x _returnvalue_y (+ _returnvalue_z (* _index 155.0))) (struct :`Pitch` 90.0)) true)))

(fn `UserConstructionScript`
  (bind _door (`self.Door`))
  (bind (_relativescale3d_x _relativescale3d_y _relativescale3d_z) (`KismetMathLibrary.BreakVector` (`SceneComponent.RelativeScale3D` _door)))
  (`self.UpdateChain`)
  (if (not (`self.IsActive`))
    (`SceneComponent.SetRelativeScale3D` _door (`KismetMathLibrary.MakeVector` 0.5 _relativescale3d_y _relativescale3d_z))))