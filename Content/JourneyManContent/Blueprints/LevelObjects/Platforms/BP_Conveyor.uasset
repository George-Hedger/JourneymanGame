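; BP_Conveyor is a conveyor platform that carries the third-person player character along while they stand on it.
; A Box trigger stores the overlapping BP_ThirdPersonCharacter as PlayerRef and clears it on exit.
; Each Tick, that character gets a swept world offset along the Arrow's forward vector, scaled by ConveyorSpeed and delta time.
; The construction script stretches the Cube mesh and trigger to ConveyorSize in X and Y, with fixed heights.
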(event `self.Box.OnComponentBeginOverlap`
  (params (OverlappedComponent :type "PrimitiveComponent Object Reference") (OtherActor :type "Actor Object Reference") (OtherComp :type "PrimitiveComponent Object Reference") (OtherBodyIndex :type Integer) (bFromSweep :type Boolean) (SweepResult :type "HitResult Structure (by ref)"))
  (bind _asbp_third_person_character (cast `/Game/JourneyManContent/Blueprints/Characters/Player/BP_ThirdPersonCharacter` OtherActor))
  (set `self.Player Ref` _asbp_third_person_character))

(event `self.Box.OnComponentEndOverlap`
  (params (OverlappedComponent :type "PrimitiveComponent Object Reference") (OtherActor :type "Actor Object Reference") (OtherComp :type "PrimitiveComponent Object Reference") (OtherBodyIndex :type Integer))
  (cast `/Game/JourneyManContent/Blueprints/Characters/Player/BP_ThirdPersonCharacter` OtherActor)
  (set `self.Player Ref` null))

(event `self.ReceiveTick`
  (params (DeltaSeconds :type "Float (single-precision)"))
  (`/Engine/EditorBlueprintResources/StandardMacros.IsValid` (`self.Player Ref`)
    (:`Is Valid`
      (`self.K2_AddActorWorldOffset` (`self.Player Ref`) (* (`SceneComponent.GetForwardVector` (`self.Arrow`)) (`self.Conveyor Speed`) DeltaSeconds) true false))))

(fn `UserConstructionScript`
  (bind (_conveyor_size_x _conveyor_size_y) (`KismetMathLibrary.BreakVector2D` (`self.Conveyor Size`)))
  (bind (_conveyor_size_x_2 _conveyor_size_y_2) (`KismetMathLibrary.BreakVector2D` (`self.Conveyor Size`)))
  (`SceneComponent.SetRelativeScale3D` (`self.Cube`) (`KismetMathLibrary.MakeVector` _conveyor_size_x_2 _conveyor_size_y_2 0.1))
  (`SceneComponent.SetRelativeScale3D` (`self.Box`) (`KismetMathLibrary.MakeVector` _conveyor_size_x _conveyor_size_y 0.3)))