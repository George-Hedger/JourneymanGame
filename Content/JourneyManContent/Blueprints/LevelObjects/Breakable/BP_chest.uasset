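; BP_chest is a breakable chest that bursts into coins when the player character touches it.
; Box overlap applies 1 damage to itself, and any damage not exceeding Health triggers the burst, with Health never decremented.
; A loop spawns BP_Coin1 at random offsets within Range, launches each outward through its ProjectileMovement, and destroys the chest after a short delay.
; A radial impulse branch on the mesh is left unconnected.
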(event `self.Box.OnComponentBeginOverlap`
  (params (OverlappedComponent :type "PrimitiveComponent Object Reference") (OtherActor :type "Actor Object Reference") (OtherComp :type "PrimitiveComponent Object Reference") (OtherBodyIndex :type Integer) (bFromSweep :type Boolean) (SweepResult :type "HitResult Structure (by ref)"))
  (cast `/Game/JourneyManContent/Blueprints/Characters/Player/BP_ThirdPersonCharacter` OtherActor)
  (`GameplayStatics.ApplyDamage` self 1.0))

(event `self.ReceiveAnyDamage`
  (params (Damage :type "Float (single-precision)") (DamageType :type "DamageType Object Reference") (InstigatedBy :type "Controller Object Reference") (DamageCauser :type "Actor Object Reference"))
  (bind (_returnvalue_x _returnvalue_y _returnvalue_z) (`KismetMathLibrary.BreakVector` (+ (`self.K2_GetActorLocation`) (* (`KismetMathLibrary.RandomUnitVector`) (`KismetMathLibrary.RandomFloatInRange` 0.0 (`self.Range`))))))
  (if (<= (- Damage (`self.Health`)) 0.0)
    (for _ (range (+ (`self.Number`) 1))
      (bind _returnvalue (`|SpawnActorFromClass` "/Game/JourneyManContent/Blueprints/LevelObjects/Collectable/BP_Coin1.BP_Coin1_C" (`KismetMathLibrary.MakeTransform` (`KismetMathLibrary.MakeVector` _returnvalue_x _returnvalue_y _returnvalue_z)) "Undefined" "MultiplyWithRoot" null null))
      (set `MovementComponent.Velocity` (* (`KismetMathLibrary.Normal` (- (`SceneComponent.K2_GetComponentLocation` (`/Game/JourneyManContent/Blueprints/LevelObjects/Collectable/BP_Coin1.StaticMesh` _returnvalue)) (`self.K2_GetActorLocation`))) (`self.NewVar`)) (`/Game/JourneyManContent/Blueprints/LevelObjects/Collectable/BP_Coin1.ProjectileMovement` _returnvalue))
      (`KismetSystemLibrary.Delay` 0.2)
      (`self.K2_DestroyActor`))))

(fn `UserConstructionScript`)