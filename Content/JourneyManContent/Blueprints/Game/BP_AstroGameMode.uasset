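; BP_AstroGameMode is a game mode that handles player death and respawning.
; OnPlayerDeath destroys player 0's pawn and triggers RespawnPlayer.
; RespawnPlayer waits for RespawnTimer, then restarts the player at CheckpointPlayerStart, falling back to FindPlayerStart when no valid checkpoint is set.
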(event `RespawnPlayer`
  (bind _returnvalue (`GameplayStatics.GetPlayerController` 0))
  (bind _checkpointplayerstart (`self.CheckpointPlayerStart`))
  (`KismetSystemLibrary.Delay` (`self.RespawnTimer`))
  (`self.RestartPlayerAtPlayerStart` _returnvalue (select `bool` (`KismetSystemLibrary.IsValid` _checkpointplayerstart) :`false` (`self.K2_FindPlayerStart` _returnvalue) :`true` _checkpointplayerstart :!type "Actor Object Reference")))

(fn `OnPlayerDeath`
  (`self.K2_DestroyActor` (`GameplayStatics.GetPlayerPawn` 0))
  (`self.RespawnPlayer`))

(fn `UserConstructionScript`)