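; BP_AstroPlayerController is the player controller that owns the HUD and tracks the player's coins and held pickup.
; On BeginPlay it creates WBP_HUD, stores it as PlayerHUD and adds it to the player screen.
; AddCoin increments the coin count, and SetHeldPickup stores the held item.
; GetHeldPickup is a consuming getter: it returns the held item and clears the reference.
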(event `self.ReceiveBeginPlay`
  (`parent.ReceiveBeginPlay`)
  (bind _returnvalue (`|CreateWidget` "/Game/Blueprints/Widgets/PlayerHUD/WBP_HUD.WBP_HUD_C" self))
  (bind _output_get (set `self.PlayerHUD` _returnvalue))
  (`UserWidget.AddToPlayerScreen` _output_get 0))

(fn `AddCoin`
  (params (NumToAdd :type Integer))
  (set `self.CoinCount` (+ NumToAdd (`self.CoinCount`))))

(fn `GetHeldPickup`
  (returns (HeldPickup :type "/Game/Blueprints/LevelObjects/Pickups/BP_Base_Pickup Object Reference"))
  (locals (HeldObjectTemp :type "/Game/Blueprints/LevelObjects/Pickups/BP_Base_Pickup Object Reference"))
  (set `local.HeldObjectTemp` (`self.HeldPickup`))
  (set `self.HeldPickup` null)
  (return (`local.HeldObjectTemp`)))

(fn `SetHeldPickup`
  (params (HeldPickup :type "/Game/Blueprints/LevelObjects/Pickups/BP_Base_Pickup Object Reference"))
  (set `self.HeldPickup` HeldPickup))

(fn `UserConstructionScript`)