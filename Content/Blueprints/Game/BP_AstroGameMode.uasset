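; Game mode for the Astro level, handling player death and respawn, the run timer, death count and music.
; Death plays sound and Niagara effects, destroys the character, restarts it at the checkpoint or a fallback player start, and resets any boss spawner.
; The first untagged PlayerStart is cached as the default spawn.
; A looping timer event accumulates pausable play time, and music functions swap between main and boss tracks.
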(event `RespawnPlayer`
  (bind _returnvalue (`GameplayStatics.GetPlayerController` 0))
  (bind _checkpointplayerstart (`self.CheckpointPlayerStart`))
  (`GameplayStatics.PlaySound2D` "/Game/Assets/SFX/AstroBotNoises/SQ_AstroBot_FallingToDeath.SQ_AstroBot_FallingToDeath" 1.0 1.0 0.0 null null)
  (`KismetSystemLibrary.Delay` (`self.RespawnAnimTimer`))
  (bind _asbp_third_person_character (cast `/Game/Blueprints/Characters/Player/BP_ThirdPersonCharacter` (`GameplayStatics.GetPlayerPawn` 0)))
  (`SceneComponent.SetVisibility` (`Character.Mesh` _asbp_third_person_character) false true)
  (`NiagaraFunctionLibrary.SpawnSystemAtLocation` "/Game/Assets/Effects/NP_Clockwork_Death.NP_Clockwork_Death" (`self.K2_GetActorLocation` (`GameplayStatics.GetPlayerPawn` 0)))
  (`KismetSystemLibrary.Delay` 0.5)
  (`self.K2_DestroyActor` _asbp_third_person_character)
  (`self.RestartPlayerAtPlayerStart` _returnvalue (select `bool` (`KismetSystemLibrary.IsValid` _checkpointplayerstart) :`false` (`self.K2_FindPlayerStart` _returnvalue) :`true` _checkpointplayerstart :!type "Actor Object Reference"))
  (bind _returnvalue_2 (`GameplayStatics.GetActorOfClass` "/Game/Blueprints/Characters/Enemies/Boss/BP_BossObstacleSpawner.BP_BossObstacleSpawner_C"))
  (`/Engine/EditorBlueprintResources/StandardMacros.IsValid` _returnvalue_2
    (:`Is Valid`
      (`/Game/Blueprints/Characters/Enemies/Boss/BP_BossObstacleSpawner.Reset boss` _returnvalue_2))))

(event `self.ReceiveBeginPlay`
  (bind _returnvalue (`KismetSystemLibrary.K2_SetTimerDelegate` (delegate `Custom Tick`) 0.01 true))
  (set `self.Timer Handle` _returnvalue)
  (`self.PlayMainMusic`))

(event `Pause Timer`
  (`KismetSystemLibrary.K2_PauseTimerHandle` (`self.Timer Handle`)))

(event `Custom Tick`
  (set `self.Timer` (+ 0.01 (`self.Timer`))))

(event `Resume`
  (`KismetSystemLibrary.K2_UnPauseTimerHandle` (`self.Timer Handle`)))

(fn `ChoosePlayerStart`
  (params (Player :type "Controller Object Reference"))
  (returns (ReturnValue :type "Actor Object Reference"))
  (`|ExecutionSequence`
    (:`then_0`
      (`/Engine/EditorBlueprintResources/StandardMacros.DoOnce` false
        (:`Completed`
          (bind _outactors (`GameplayStatics.GetAllActorsOfClass` "/Script/Engine.PlayerStart"))
          (for _array_element _outactors
            (if (== (`PlayerStart.PlayerStartTag` _array_element) "None")
              (set `self.DefaultPlayerStart` _array_element)
              (break))))))
    (:`then_1`
      (return (`self.DefaultPlayerStart`)))))

(fn `OnPlayerDeath`
  (`self.RespawnPlayer`)
  (`/Engine/EditorBlueprintResources/StandardMacros.IncrementInt` (`self.Deaths`)))

(fn `PlayBossMusic`
  (bind _mainmusic (`self.MainMusic`))
  (`/Engine/EditorBlueprintResources/StandardMacros.IsValid` _mainmusic
    (:`Is Valid`
      (`AudioComponent.Stop` _mainmusic))
    (:`Is Not Valid`
      _))
  (bind _returnvalue (`GameplayStatics.CreateSound2D` "/Game/Assets/SFX/Music/SQ_Music_Boss_Cue.SQ_Music_Boss_Cue" 1.0 1.0 0.0 null))
  (bind _output_get (set `self.MainMusic` _returnvalue))
  (`AudioComponent.Play` _output_get 0.0))

(fn `PlayMainMusic`
  (bind _mainmusic (`self.MainMusic`))
  (`/Engine/EditorBlueprintResources/StandardMacros.IsValid` _mainmusic
    (:`Is Valid`
      (`AudioComponent.Stop` _mainmusic))
    (:`Is Not Valid`
      _))
  (bind _returnvalue (`GameplayStatics.CreateSound2D` "/Game/Assets/SFX/Music/SQ_Music_MainLevel_Cue.SQ_Music_MainLevel_Cue" 0.75 1.0 0.0 null))
  (bind _output_get (set `self.MainMusic` _returnvalue))
  (`AudioComponent.Play` _output_get 0.0))

(fn `UserConstructionScript`)