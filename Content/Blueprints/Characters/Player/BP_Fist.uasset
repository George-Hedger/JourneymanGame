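; Extendable punching fist actor that fires from its parent component on the player, damaging what it hits and grabbing grabbable objects.
; A Tick-driven state machine handles idle, extending, pausing and retracting, with collision enabled only while extending.
; Launch direction and retraction account for owner velocity, and AddOffset clamps at the target length to signal state changes.
; A spline mesh stretches back to the idle position, and the fist destroys itself when its parent becomes invalid.
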(event `self.Sphere1.OnComponentHit`
  (params (HitComponent :type "PrimitiveComponent Object Reference") (OtherActor :type "Actor Object Reference") (OtherComp :type "PrimitiveComponent Object Reference") (NormalImpulse :type "Vector Structure") (Hit :type "HitResult Structure (by ref)"))
  (bind _returnvalue (`ActorComponent.GetOwner` (`self.ParentSC`)))
  ; On Hit
  (if (and (!= OtherActor _returnvalue) (`|EnumEquality` (`self.State`) "NewEnumerator1"))
    (`GameplayStatics.ApplyDamage` OtherActor (`self.Damage`) null _returnvalue)
    (`self.OnHitEffect`
      (:`end`
        (bind _asbp_base_grabbable_object (cast `/Game/Blueprints/LevelObjects/Grabbable/BP_Base_GrabbableObject` OtherActor)
          (:`then`
            (`/Game/Blueprints/LevelObjects/Grabbable/BP_Base_GrabbableObject.OnGrab` _asbp_base_grabbable_object self)
            (set `self.State` "NewEnumerator3"))
          (:`CastFailed`
            (`self.BeginPause`)))))))

(event `self.ReceiveTick`
  (params (DeltaSeconds :type "Float (single-precision)"))
  (bind _sphere1 (`self.Sphere1`))
  (bind _returnvalue (- (`self.GetIdlePosition`) (`self.K2_GetActorLocation`)))
  (`|ExecutionSequence`
    (:`then_0`
      ; Destroy alongside player
      (`/Engine/EditorBlueprintResources/StandardMacros.IsValid` (`self.ParentSC`)
        (:`Is Not Valid`
          (`self.K2_DestroyActor`))))
    (:`then_1`
      ; Update Rotation
      (`SceneComponent.K2_SetRelativeRotation` (`self.StaticMesh`) (`self.GetOwnerRotation`) false false)
      (if (`|EnumEquality` (`self.State`) "NewEnumerator1")
        (`PrimitiveComponent.SetCollisionEnabled` _sphere1 "QueryAndPhysics")
        (else
          (`PrimitiveComponent.SetCollisionEnabled` _sphere1 "NoCollision"))))
    (:`then_2`
      ; Update position based on State
      (switch `/Game/Blueprints/Characters/Player/E_FistState` (`self.State`)
        (:`NewEnumerator0`
          (`self.K2_SetActorLocation` (`self.GetIdlePosition`) false true))
        (:`NewEnumerator1`
          (bind _hasreachedlimit (`self.AddOffset` (* (* DeltaSeconds (`self.Speed`)) (`self.ShotNormal`)) (`self.MaxLength`)))
          (if _hasreachedlimit
            (`self.BeginPause`)))
        (:`NewEnumerator2`
          (if (> (`KismetMathLibrary.Dot_VectorVector` _returnvalue (`self.GetOwnerVelocity`)) 0.0)
            (`self.AddOffset` (* (`self.GetOwnerVelocity`) DeltaSeconds)))
          (bind _hasreachedlimit_2 (`self.AddOffset` (* (* DeltaSeconds (`self.Speed`)) (`KismetMathLibrary.Normal` _returnvalue))))
          (if _hasreachedlimit_2
            (set `self.State` "NewEnumerator0")))
        (:`NewEnumerator4`
          (if (>= (`self.Timer`) (`self.PauseTime`))
            (set `self.Timer` 0.0)
            (`self.BeginRetract`)
            (else
              (set `self.Timer` (+ (`self.Timer`) DeltaSeconds))
              (if (and (> (`self.GetExtentionSquared` (`self.K2_GetActorLocation`)) (`self.MaxLength`)) (> (`KismetMathLibrary.Dot_VectorVector` (- (`self.GetIdlePosition`) (`self.K2_GetActorLocation`)) (`self.GetOwnerVelocity`)) 0.0))
                (`self.AddOffset` (* DeltaSeconds (`self.GetOwnerVelocity`)) (`self.MaxLength`))))))))
    (:`then_3`
      ; Update Spline
      (`SplineMeshComponent.SetEndPosition` (`self.SplineMesh`) (- (`self.GetIdlePosition`) (`self.K2_GetActorLocation`)) true))))

(fn `AddOffset`
  (params (Offset :type "Vector Structure (by ref)") (TargetLength :type "Float (double-precision)"))
  (returns (HasReachedLimit :type Boolean))
  (bind _returnvalue (`self.K2_GetActorLocation`))
  (bind _returnvalue_2 (`KismetMathLibrary.Square` TargetLength))
  (bind _returnvalue_3 (>= (`KismetMathLibrary.Abs` (- (`self.GetExtentionSquared` (+ Offset _returnvalue)) _returnvalue_2)) (`KismetMathLibrary.Abs` (- (`self.GetExtentionSquared` _returnvalue) _returnvalue_2))))
  (if _returnvalue_3
    (`self.K2_SetActorLocation` (+ (* TargetLength (`KismetMathLibrary.Normal` (- (`self.K2_GetActorLocation`) (`self.GetIdlePosition`)))) (`self.GetIdlePosition`)) true)
    (else
      (`self.K2_AddActorWorldOffset` Offset true)))
  (return _returnvalue_3))

(fn `BeginExtend`
  (params (MaxLength :type "Float (double-precision)") (ShotDirection :type "Vector Structure") (Speed :type "Float (double-precision)") (Damage :type "Float (double-precision)"))
  (returns (HasFired :type Boolean))
  (if (`|EnumEquality` (`self.State`) "NewEnumerator0")
    (`|ExecutionSequence`
      (:`then_0`
        (set `self.State` "NewEnumerator1"))
      (:`then_1`
        (set `self.MaxLength` MaxLength))
      (:`then_2`
        (set `self.Speed` Speed))
      (:`then_3`
        (set `self.Damage` Damage))
      (:`then_4`
        (set `self.ShotNormal` (`KismetMathLibrary.Normal` (+ (`self.GetOwnerVelocity`) (* Speed (`KismetMathLibrary.Normal` ShotDirection)))))
        (return true)))
    (else
      (return false))))

(fn `BeginPause`
  (set `self.Timer` 0.0)
  (set `self.State` "NewEnumerator4"))

(fn `BeginRetract`
  (if (`|EnumInequality` (`self.State`) "NewEnumerator0")
    (set `self.State` "NewEnumerator2")))

(fn `GetExtentionSquared`
  (params (Position :type "Vector Structure"))
  (returns (ExtentionSquared :type "Float (double-precision)"))
  (return (`KismetMathLibrary.VSizeSquared` (- Position (`self.GetIdlePosition`)))))

(fn `GetIdlePosition`
  (returns (Pos :type "Vector Structure"))
  (return (`KismetMathLibrary.SelectVector` (`/Game/Blueprints/Characters/Player/SC_FistComponent.GetIdleWorldPos` (`self.ParentSC`)) (0.0 0.0 0.0) (`KismetSystemLibrary.IsValid` (`self.ParentSC`)))))

(fn `GetOwnerRotation`
  (returns (Rotation :type "Rotator Structure"))
  (return (select `bool` (`KismetSystemLibrary.IsValid` (`self.ParentSC`)) :`true` (`SceneComponent.K2_GetComponentRotation` (`self.ParentSC`)))))

(fn `GetOwnerVelocity`
  (returns (Vel :type "Vector Structure"))
  (return (`KismetMathLibrary.SelectVector` (`self.GetVelocity` (`ActorComponent.GetOwner` (`self.ParentSC`))) (0.0 0.0 0.0) (`KismetSystemLibrary.IsValid` (`self.ParentSC`)))))

(fn `GetPlayer`
  (returns (Player :type "/Game/Blueprints/Characters/Player/BP_ThirdPersonCharacter Object Reference"))
  (bind _asbp_third_person_character (cast `/Game/Blueprints/Characters/Player/BP_ThirdPersonCharacter` (`ActorComponent.GetOwner` (`self.ParentSC`))))
  (return _asbp_third_person_character))

(fn `UserConstructionScript`)