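; Player camera component that anchors the third-person camera boom to the ground beneath the character, keeping it steady through jumps.
; After Initialise, each tick sphere-traces downward and smoothly interpolates the boom to that point plus a height offset.
; A jump, detected by upward velocity, locks boom height while X and Y follow directly, until the player drops below takeoff or lands.
; Very fast upward motion counts as a launch and releases the lock.
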(event `Initialise`
  (bind (_sensedlocation_x _sensedlocation_y) (`KismetMathLibrary.BreakVector` (`self.SensedLocation`)))
  (bind (_sensedlocation_x_2 _sensedlocation_y_2 _sensedlocation_z) (`KismetMathLibrary.BreakVector` (`self.SensedLocation`)))
  (bind (_returnvalue_x _returnvalue_y _returnvalue_z) (`KismetMathLibrary.BreakVector` (`Actor.K2_GetActorLocation` (`self.As BP Third Person Character`))))
  (bind (_returnvalue_x_2 _returnvalue_y_2 _returnvalue_z_2) (`KismetMathLibrary.BreakVector` (`Actor.K2_GetActorLocation` (`self.As BP Third Person Character`))))
  (`|ExecutionSequence`
    (:`then_0`
      (bind _asbp_third_person_character (cast `/Game/Blueprints/Characters/Player/BP_ThirdPersonCharacter` (`self.GetOwner`)))
      (set `self.As BP Third Person Character` _asbp_third_person_character)
      (set `self.Character Movement` (`Character.CharacterMovement` _asbp_third_person_character))
      (set `self.Camera Boom` (`/Game/Blueprints/Characters/Player/BP_ThirdPersonCharacter.CameraBoom` _asbp_third_person_character))
      (set `self.Follow Camera` (`/Game/Blueprints/Characters/Player/BP_ThirdPersonCharacter.FollowCamera` _asbp_third_person_character))
      (set `SpringArmComponent.TargetArmLength` (`self.BoomLength`) (`self.Camera Boom`)))
    (:`then_1`
      (goto _label :!via `Open`))))

(event `self.ReceiveTick`
  (params (DeltaSeconds :type "Float (single-precision)"))
  (bind (_sensedlocation_x _sensedlocation_y) (`KismetMathLibrary.BreakVector` (`self.SensedLocation`)))
  (bind (_sensedlocation_x_2 _sensedlocation_y_2 _sensedlocation_z) (`KismetMathLibrary.BreakVector` (`self.SensedLocation`)))
  (bind (_returnvalue_x _returnvalue_y _returnvalue_z) (`KismetMathLibrary.BreakVector` (`Actor.K2_GetActorLocation` (`self.As BP Third Person Character`))))
  (bind (_returnvalue_x_2 _returnvalue_y_2 _returnvalue_z_2) (`KismetMathLibrary.BreakVector` (`Actor.K2_GetActorLocation` (`self.As BP Third Person Character`))))
  (`/Engine/EditorBlueprintResources/StandardMacros.Gate` true :!label _label
    (:`Exit`
      (`self.GroundSensor`)
      (`self.JumpingTester`)
      (`|ExecutionSequence`
        (:`then_0`
          (if (and (`self.IsJumping`) (not (`self.IsLaunched`)))
            (`|ExecutionSequence`
              (:`then_0`
                (`/Engine/EditorBlueprintResources/StandardMacros.DoOnce` false :!label _label_2
                  (:`Completed`
                    (set `self.HeightToCompare` (- _returnvalue_z_2 50.0))
                    (set `self.FixBoomHeight` true)
                    (set `self.FixHeight` (+ _sensedlocation_z (`self.BoomHeight`)))
                    (set `self.Islanded` false))))
              (:`then_1`
                (if (< _returnvalue_z (`self.HeightToCompare`))
                  (set `self.FixBoomHeight` false)))
              (:`then_2`
                (goto _label_3 :!via `Reset`)))))
        (:`then_1`
          (if (`self.IsLaunched`)
            (set `self.FixBoomHeight` false)
            (goto _label_3 :!via `Reset`)))
        (:`then_2`
          (`/Engine/EditorBlueprintResources/StandardMacros.DoOnce` false :!label _label_3
            (:`Completed`
              (if (not (`NavMovementInterface.IsFalling` (`self.Character Movement`)))
                (set `self.IsJumping` false)
                (set `self.IsLaunched` false)
                (set `self.FixBoomHeight` false)
                (set `self.Islanded` true)
                (goto _label_2 :!via `Reset`)))))
        (:`then_3`
          (if (`self.FixBoomHeight`)
            (`SceneComponent.K2_SetWorldLocation` (`self.Camera Boom`) (`KismetMathLibrary.MakeVector` _sensedlocation_x _sensedlocation_y (`self.FixHeight`)) false false)
            (else
              (`self.MoveCameraBoom` (`self.SensedLocation`) (`self.SmoothFactor`)))))))))

(fn `GroundSensor`
  (bind _returnvalue (`Actor.K2_GetActorLocation` (`self.As BP Third Person Character`)))
  ; find the ground directly below player character
  (bind (_outhit _returnvalue_2) (`KismetSystemLibrary.SphereTraceSingleByProfile` _returnvalue (- _returnvalue (`KismetMathLibrary.MakeVector` 0.0 0.0 (`self.GroundSensingDistance`))) 35.0 "BlockAllDynamic"))
  (if _returnvalue_2
    (bind (_bblockinghit _binitialoverlap _time _distance _location _impactpoint _normal _impactnormal _physmat _hitactor _hitcomponent _hitbonename _bonename _hititem _elementindex _faceindex _tracestart _traceend) (`GameplayStatics.BreakHitResult` _outhit))
    (set `self.SensedLocation` _location)
    (else
      (set `self.SensedLocation` _traceend))))

(fn `JumpingTester`
  (bind (_returnvalue_x _returnvalue_y _returnvalue_z) (`KismetMathLibrary.BreakVector` (`Actor.GetVelocity` (`self.As BP Third Person Character`))))
  (if (> _returnvalue_z 0.0)
    (if (< _returnvalue_z 1200.0)
      (set `self.IsJumping` true)
      (else
        (set `self.IsLaunched` true)))))

(fn `MoveCameraBoom`
  (params (A :type "Vector Structure") (InterpSpeed :type "Float (single-precision)"))
  (bind _camera_boom (`self.Camera Boom`))
  ; move camera boom smoothly
  (`SceneComponent.K2_SetWorldLocation` _camera_boom (`KismetMathLibrary.VInterpTo` (`SceneComponent.K2_GetComponentLocation` _camera_boom) (+ A (`KismetMathLibrary.MakeVector` 0.0 0.0 (`self.BoomHeight`))) (`GameplayStatics.GetWorldDeltaSeconds`) InterpSpeed) false false))