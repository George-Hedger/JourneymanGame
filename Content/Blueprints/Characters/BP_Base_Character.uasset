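; Base character Blueprint that manages health and destroys the actor on death.
; Health starts at MaxHealth on BeginPlay, and AnyDamage subtracts incoming damage through SetHealth.
; SetHealth either sets or subtracts, clamps the result between zero and MaxHealth, and calls OnDeath when health runs out.
; InstantKillCharacter forces death by setting health to zero through the same path.
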(event `self.ReceiveBeginPlay`
  (`self.SetHealth` (`self.MaxHealth`)))

(event `self.ReceiveAnyDamage`
  (params (Damage :type "Float (single-precision)") (DamageType :type "DamageType Object Reference") (InstigatedBy :type "Controller Object Reference") (DamageCauser :type "Actor Object Reference"))
  (`self.SetHealth` Damage true))

(fn `InstantKillCharacter`
  (`self.SetHealth` 0.0))

(fn `OnDeath`
  (`self.K2_DestroyActor`))

(fn `SetHealth`
  (params (NewHealth :type "Float (double-precision)") (SubtractFromHealth :type Boolean))
  (returns (Health :type "Float (double-precision)"))
  (bind _output_get (set `self.Health` (`KismetMathLibrary.FClamp` (select `bool` SubtractFromHealth :`false` NewHealth :`true` (- (`self.Health`) NewHealth)) 0.0 (`self.MaxHealth`))))
  (if (<= _output_get 0.0)
    (`self.OnDeath`))
  (return _output_get))

(fn `UserConstructionScript`)