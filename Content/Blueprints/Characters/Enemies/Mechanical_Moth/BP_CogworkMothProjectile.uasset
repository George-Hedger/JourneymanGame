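; Projectile actor for the Cogwork Moth enemy that damages the player on contact; no movement logic appears in its graphs.
; Tick spins the cube around its pitch axis at RotationSpeed.
; When its box overlaps the player character, it spawns a short-lived BP_Hitbox there to apply damage with a team filter, then destroys itself.
; The Construction Script calls OnCreation, which destroys the projectile after a timed delay.
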(event `On Creation`
  (`KismetSystemLibrary.Delay` 5.0)
  (`/Engine/EditorBlueprintResources/StandardMacros.IsValid` self
    (:`Is Valid`
      (`self.K2_DestroyActor`))))

(event `self.ReceiveTick`
  (params (DeltaSeconds :type "Float (single-precision)"))
  (`SceneComponent.K2_AddLocalRotation` (`self.Cube`) (`KismetMathLibrary.MakeRotator` 0.0 (* DeltaSeconds (`self.Rotation Speed`))) false false))

(event `self.Box.OnComponentBeginOverlap`
  (params (OverlappedComponent :type "PrimitiveComponent Object Reference") (OtherActor :type "Actor Object Reference") (OtherComp :type "PrimitiveComponent Object Reference") (OtherBodyIndex :type Integer) (bFromSweep :type Boolean) (SweepResult :type "HitResult Structure (by ref)"))
  (bind _box (`self.Box`))
  (bind (_returnvalue_location _returnvalue_rotation) (`KismetMathLibrary.BreakTransform` (`SceneComponent.K2_GetComponentToWorld` _box)))
  (if (== OtherActor (`GameplayStatics.GetPlayerCharacter` 0))
    (bind _returnvalue (`|SpawnActorFromClass` "/Game/Blueprints/Characters/BP_Hitbox.BP_Hitbox_C" (`KismetMathLibrary.MakeTransform` _returnvalue_location _returnvalue_rotation (`BoxComponent.GetScaledBoxExtent` _box)) "AlwaysSpawn" "MultiplyWithRoot" null 10.0 false self "NewEnumerator1" 1.0 null))
    (`/Engine/EditorBlueprintResources/StandardMacros.IsValid` _returnvalue
      (:`Is Valid`
        (`self.K2_DestroyActor`)))))

(fn `UserConstructionScript`
  (`self.On Creation`))