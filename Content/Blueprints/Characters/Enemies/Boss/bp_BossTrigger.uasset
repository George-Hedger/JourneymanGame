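; Boss arena trigger that starts the boss fight when the player enters its overlap cylinder.
; A DoOnce gate starts every boss hand and the obstacle spawner, enables collision on a cylinder mesh, and tells the Astro game mode to play boss music.
; A reset event disables that collision again and rearms the trigger.
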(event `self.Cylinder1.OnComponentBeginOverlap`
  (params (OverlappedComponent :type "PrimitiveComponent Object Reference") (OtherActor :type "Actor Object Reference") (OtherComp :type "PrimitiveComponent Object Reference") (OtherBodyIndex :type Integer) (bFromSweep :type Boolean) (SweepResult :type "HitResult Structure (by ref)"))
  (if (== OtherActor (`GameplayStatics.GetPlayerCharacter` 0))
    (`/Engine/EditorBlueprintResources/StandardMacros.DoOnce` false :!label _label
      (:`Completed`
        (for _array_element (`self.Boss hands`)
          (`/Game/Blueprints/Characters/Enemies/Boss/BP_BossHand.Start` _array_element))
        (`/Game/Blueprints/Characters/Enemies/Boss/BP_BossObstacleSpawner.Start` (`self.Obstaxle spawner`))
        (`PrimitiveComponent.SetCollisionEnabled` (`StaticMeshActor.StaticMeshComponent` (`self.cylinder`)) "QueryAndPhysics")
        (bind _asbp_astro_game_mode (cast `/Game/Blueprints/Game/BP_AstroGameMode` (`GameplayStatics.GetGameMode`)))
        (`/Game/Blueprints/Game/BP_AstroGameMode.PlayBossMusic` _asbp_astro_game_mode)))))

(event `reset trigger`
  (`PrimitiveComponent.SetCollisionEnabled` (`StaticMeshActor.StaticMeshComponent` (`self.cylinder`)) "NoCollision")
  (goto _label :!via `Reset`))

(fn `UserConstructionScript`)