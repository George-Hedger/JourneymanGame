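; BP_BossHand is a clockwork boss hand that sweeps in timed steps, damaging the player and dealing massive damage to anything else its box overlaps.
; A looping timer triggers each timeline-driven yaw step with sound, and cog activation changes short of the goal rescale the interval via SpeedUpVariable.
; Reaching the required activations resets the obstacle spawner, plays a camera cutscene, and spins the hand before death effects, results widget and self-destruction.
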(event `Reset Timer`
  (bind _returnvalue (`KismetSystemLibrary.K2_SetTimerDelegate` (delegate `Movehands`) (`self.Speed`) true :!label _label))
  (set `self.Timer` _returnvalue))

(event `Start`
  (set `self.Starting rotation` (`SceneComponent.K2_GetComponentRotation` (`self.Hand`)))
  (set `self.Speed` 1.0)
  (goto _label))

(event `Movehands`
  (bind (_returnvalue_roll _returnvalue_pitch _returnvalue_yaw) (`KismetMathLibrary.BreakRotator` (`SceneComponent.K2_GetComponentRotation` (`self.Hand`))))
  (bind _returnvalue (`SceneComponent.K2_GetComponentLocation` (`self.Box`)))
  (set `self.Return Value Z (Yaw)` _returnvalue_yaw)
  (`GameplayStatics.PlaySoundAtLocation` "/Game/Assets/SFX/BossSound/SQ_BossSound_Handmoving1.SQ_BossSound_Handmoving1" _returnvalue (struct) 1.0 1.0 0.0 "/Game/Assets/SFX/SoundAttenuation/SA_General.SA_General" null null null)
  (`GameplayStatics.PlaySoundAtLocation` null _returnvalue (struct) 1.0 1.0 0.0 null null null null)
  (bind (_direction _newtrack_0) (`Timeline|Timeline` :!via `PlayFromStart` :!label _label_2)
    (:`Update`
      (`SceneComponent.K2_SetWorldRotation` (`self.Hand`) (`KismetMathLibrary.MakeRotator` 0.0 0.0 (+ (* _newtrack_0 (`self.Movement`)) (`self.Return Value Z (Yaw)`))) false false))))

(event `Stop timeline`
  (goto _label_2 :!via `Stop`))

(event `Reset boss`
  (`SceneComponent.K2_SetWorldRotation` (`self.Hand`) (`self.Starting rotation`) false false)
  (`self.Stop timeline`)
  (`self.stop boss`))

(event `Speed up`
  (set `self.Speed` (/ (`self.Speed`) (`self.Speed up variable`)))
  (`self.Reset Timer`))

(event `stop boss`
  (set `self.Speed` 0.0)
  (`self.Reset Timer`))

(event `/Game/Blueprints/Interfaces/BPI_Activate.OnActivationChanged`
  (params (IsActive :type Boolean))
  (bind _output_get (set `self.NumberActivations` (`KismetMathLibrary.Max` (+ (`self.NumberActivations`) (`KismetMathLibrary.SelectInt` 1 -1 IsActive)))))
  (if (>= _output_get (`self.NumberOfCogActivationsForActive`))
    (`self.Victory`)
    (elif (not (== (`self.NumberActivations`) 0))
      (`self.Speed up`))))

(event `self.Box.OnComponentBeginOverlap`
  (params (OverlappedComponent :type "PrimitiveComponent Object Reference") (OtherActor :type "Actor Object Reference") (OtherComp :type "PrimitiveComponent Object Reference") (OtherBodyIndex :type Integer) (bFromSweep :type Boolean) (SweepResult :type "HitResult Structure (by ref)"))
  (bind _asbp_third_person_character (cast `/Game/Blueprints/Characters/Player/BP_ThirdPersonCharacter` OtherActor)
    (:`then`
      (`GameplayStatics.ApplyDamage` _asbp_third_person_character 20.0 null self))
    (:`CastFailed`
      (`GameplayStatics.ApplyDamage` OtherActor 10000.0 null self))))

(event `Victory`
  (`ActorComponent.K2_DestroyComponent` (`self.Box`))
  (`self.ending cutscene`)
  (bind _obstacle_spawner (`self.obstacle spawner`)
    (:`then`
      (`/Game/Blueprints/Characters/Enemies/Boss/BP_BossObstacleSpawner.Reset boss` _obstacle_spawner)
      (bind _custcene_camera (`self.Custcene camera`)
        (:`then`
          (`/Game/Blueprints/LevelObjects/CoreMechanics/BP_CutsceneCamera.Play Cutscene` _custcene_camera))
        (:`else`)))
    (:`else`)))

(event `ending cutscene`
  (bind _hand (`self.Hand`))
  (bind (_relativerotation_roll _relativerotation_pitch _relativerotation_yaw) (`KismetMathLibrary.BreakRotator` (`SceneComponent.RelativeRotation` _hand)))
  (bind (_direction _newtrack_0) (`Timeline|Timeline_0`)
    (:`Update`
      (`SceneComponent.K2_SetRelativeRotation` _hand (`KismetMathLibrary.MakeRotator` 0.0 0.0 (+ _relativerotation_yaw (* (* _newtrack_0 8.0) (`self.amount of spins end`)))) false false))
    (:`Finished`
      (`GameplayStatics.PlaySoundAtLocation` "/Game/Assets/SFX/BossSound/SQ_BossSound_DefeatNoise3.SQ_BossSound_DefeatNoise3" (`SceneComponent.K2_GetComponentLocation` (`self.DefaultSceneRoot`)) (struct) 1.0 1.0 0.0 null null null null)
      (`NiagaraFunctionLibrary.SpawnSystemAttached` "/Game/Assets/Effects/NP_Clockwork_Death.NP_Clockwork_Death" (`self.Hand`) "None" (0.0 0.0 0.0) (struct) "KeepRelativeOffset" false true "None" false)
      (bind _returnvalue (`|CreateWidget` "/Game/Blueprints/Widgets/Results/WBP_Results.WBP_Results_C" null "Visible"))
      (`UserWidget.AddToViewport` _returnvalue 0)
      (`self.K2_DestroyActor`))))

(fn `UserConstructionScript`)