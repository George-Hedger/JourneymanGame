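; Boss reset volume whose cylinder catches overlapping actors, recycling the example pickup and dealing lethal-scale damage to anything else.
; The pickup moves to a random XY offset within the BP_BossObstacleSpawner's radius, found by class lookup, or an error prints if none exists.
; The offset's Z is the spawner's own height, added on top of its location, so that height counts twice.
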(event `self.Cylinder.OnComponentBeginOverlap`
  (params (OverlappedComponent :type "PrimitiveComponent Object Reference") (OtherActor :type "Actor Object Reference") (OtherComp :type "PrimitiveComponent Object Reference") (OtherBodyIndex :type Integer) (bFromSweep :type Boolean) (SweepResult :type "HitResult Structure (by ref)"))
  (if (== OtherActor "/Game/Blueprints/LevelObjects/Pickups/BP_ExamplePickup.BP_ExamplePickup")
    (bind _returnvalue (`GameplayStatics.GetActorOfClass` "/Game/Blueprints/Characters/Enemies/Boss/BP_BossObstacleSpawner.BP_BossObstacleSpawner_C"))
    (`/Engine/EditorBlueprintResources/StandardMacros.IsValid` _returnvalue
      (:`Is Valid`
        (bind _returnvalue_2 (`SceneComponent.K2_GetComponentLocation` (`/Game/Blueprints/Characters/Enemies/Boss/BP_BossObstacleSpawner.DefaultSceneRoot` _returnvalue)))
        (bind (_returnvalue_x _returnvalue_y) (`KismetMathLibrary.BreakVector` (* (`KismetMathLibrary.RandomUnitVector`) (* (`KismetMathLibrary.RandomFloat`) (`/Game/Blueprints/Characters/Enemies/Boss/BP_BossObstacleSpawner.Radius` _returnvalue)))))
        (`SceneComponent.K2_SetWorldLocation` (`Actor.RootComponent` OtherActor) (+ _returnvalue_2 (`KismetMathLibrary.MakeVector` _returnvalue_x _returnvalue_y (.z _returnvalue_2))) false false))
      (:`Is Not Valid`
        (`KismetSystemLibrary.PrintString` "BOSS RESET VOLUME ERROR" true true (struct :`R` 1.0 :`G` 0.034441 :`A` 1.0))))
    (else
      (`GameplayStatics.ApplyDamage` OtherActor 10000.0 null self))))

(fn `UserConstructionScript`)