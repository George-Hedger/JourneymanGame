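; BP_SmallerSpider is a spider enemy whose AI state is driven through Blackboard flags for seen player, waiting and dead.
; PawnSensing flags the player after navigation path checks, with sight requiring a complete path ending near the player.
; Damage reduces health with a sound and brief material flash, while activation changes toggle waiting.
; Death stops movement, notifies its activation area, plays a montage and destroys the actor on blend out.
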(event `self.PawnSensing.OnHearNoise`
  (params (Instigator :type "Pawn Object Reference") (Location :type "Vector Structure (by ref)") (Volume :type "Float (single-precision)"))
  (bind _returnvalue (`GameplayStatics.GetPlayerCharacter` 0))
  (`/Engine/EditorBlueprintResources/StandardMacros.IsValid` Instigator
    (:`Is Valid`
      (if (== Instigator _returnvalue)
        (bind _returnvalue_2 (`NavigationSystemV1.FindPathToLocationSynchronously` (`self.K2_GetActorLocation` self) (`self.K2_GetActorLocation` _returnvalue) null null))
        (`/Engine/EditorBlueprintResources/StandardMacros.IsValid` _returnvalue_2
          (:`Is Valid`
            (cast `/Game/Blueprints/Characters/Player/BP_ThirdPersonCharacter` Instigator)
            (`BlackboardComponent.SetValueAsBool` (`AIBlueprintHelperLibrary.GetBlackboard` self) "hasSeenPlayer?" true)))))))

(event `self.PawnSensing.OnSeePawn`
  (params (Pawn :type "Pawn Object Reference"))
  (bind _returnvalue (`NavigationSystemV1.FindPathToLocationSynchronously` (`self.K2_GetActorLocation` self) (`self.K2_GetActorLocation` Pawn) Pawn null))
  (`/Engine/EditorBlueprintResources/StandardMacros.IsValid` _returnvalue
    (:`Is Valid`
      (if (not (`NavigationPath.IsPartial` _returnvalue))
        (bind _pathpoints (`NavigationPath.PathPoints` _returnvalue))
        (if (< (`KismetMathLibrary.Vector_Distance` (`|GetArrayItem` _pathpoints (`KismetArrayLibrary.Array_LastIndex` _pathpoints)) (`self.K2_GetActorLocation` (`GameplayStatics.GetPlayerCharacter` 0))) 100.0)
          (cast `/Game/Blueprints/Characters/Player/BP_ThirdPersonCharacter` Pawn)
          (`BlackboardComponent.SetValueAsBool` (`AIBlueprintHelperLibrary.GetBlackboard` (`AIBlueprintHelperLibrary.GetAIController` self)) "hasSeenPlayer?" true))))))

(event `/Game/Blueprints/Interfaces/BPI_Activate.OnActivationChanged`
  (params (IsActive :type Boolean))
  (`BlackboardComponent.SetValueAsBool` (`AIBlueprintHelperLibrary.GetBlackboard` (`AIBlueprintHelperLibrary.GetAIController` self)) "Waiting" IsActive))

(event `self.Get Active Area`
  (params (`Activation Area` :type "/Game/Blueprints/Characters/Enemies/BP_EnemyStart Object Reference"))
  (set `self.Active Area` `Activation Area`))

(event `self.OnDeath`
  (bind _active_area (`self.Active Area`))
  (`BlackboardComponent.SetValueAsBool` (`AIBlueprintHelperLibrary.GetBlackboard` (`AIBlueprintHelperLibrary.GetAIController` self)) "IsDead?" true)
  (`MovementComponent.StopMovementImmediately` (`self.CharacterMovement`))
  (`GameplayStatics.PlaySoundAtLocation` "/Game/Assets/SFX/SpiderSound/S_Spider_Death2.S_Spider_Death2" (`self.K2_GetActorLocation`) (struct) 1.0 1.0 0.0 "/Game/Assets/SFX/SoundAttenuation/SA_General.SA_General" null null null)
  (`/Engine/EditorBlueprintResources/StandardMacros.IsValid` _active_area
    (:`Is Valid`
      (`/Game/Blueprints/Characters/Enemies/BP_EnemyStart.EnemyDeath` _active_area))
    (:`Is Not Valid`
      _))
  (`|PlayMontage` (`self.Mesh`) "/Game/Assets/Animations/Enemies/Bjorn/Animation_Sequences/AM_GiantSpider_Death_Montage.AM_GiantSpider_Death_Montage"
    (:`OnBlendOut`
      (`self.K2_DestroyActor`))))

(event `self.ReceiveAnyDamage`
  (params (Damage :type "Float (single-precision)") (DamageType :type "DamageType Object Reference") (InstigatedBy :type "Controller Object Reference") (DamageCauser :type "Actor Object Reference"))
  (bind _mesh (`self.Mesh`))
  (if (not (`BlackboardComponent.GetValueAsBool` (`AIBlueprintHelperLibrary.GetBlackboard` (`AIBlueprintHelperLibrary.GetAIController` self)) "IsDead?"))
    (`self.SetHealth` Damage true)
    (`GameplayStatics.PlaySoundAtLocation` "/Game/Assets/SFX/SpiderSound/S_Spider_Injured2.S_Spider_Injured2" (`self.K2_GetActorLocation`) (struct) 1.0 1.0 0.0 "/Game/Assets/SFX/SoundAttenuation/SA_General.SA_General" null null null)
    (`/Engine/EditorBlueprintResources/StandardMacros.IsValid` _mesh
      (:`Is Valid`
        (`PrimitiveComponent.SetMaterial` _mesh 0 "/Game/Assets/Materials/Characters/Enemies/M_DamageFlash.M_DamageFlash")
        (`KismetSystemLibrary.Delay` 0.2)
        (`PrimitiveComponent.SetMaterial` _mesh 0 (`self.Material`))))))

(fn `UserConstructionScript`
  (`parent.UserConstructionScript`))