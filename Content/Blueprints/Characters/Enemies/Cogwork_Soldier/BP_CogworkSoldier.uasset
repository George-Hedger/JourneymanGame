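; Cogwork Soldier enemy that, while activated, patrols a looping list of waypoints and chases the player on entering its ChaseBox.
; Activation changes adjust a counter that scales walk speed, so repeated activations stack.
; Patrol and Chase are self-re-calling AI MoveTo loops, switched by ChaseBox overlaps.
; Player overlap with AttackRange spawns a short-lived damage hitbox in front of it, regardless of activation.
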(event `self.ReceiveBeginPlay`
  ;[0.003416 0.15 0.00705 0.5] Begin play
  (`parent.ReceiveBeginPlay`)
  (set `self.IsActivated?` false)
  (set `self.IsChasing?` false)
  (set `self.TimesActivated` 0))

(event `self.OnDeath`
  ;[0.15 0 0.01339 0.5] Death
  (`self.K2_DestroyActor`))

(event `/Game/Blueprints/Interfaces/BPI_Activate.OnActivationChanged`
  (params (IsActive :type Boolean))
  (bind _timesactivated (`self.TimesActivated`))
  (bind _timesactivated_2 (`self.TimesActivated`))
  ;[0.02593 0.15 0.02818 0.5] activate event
  (set `self.IsActivated?` IsActive)
  (`self.patrol`)
  (if (`self.IsActivated?`)
    ;; Enemy Speed
    (bind _result (`/Engine/EditorBlueprintResources/StandardMacros.IncrementInt` _timesactivated_2)
      (:`  `
        (set `self.TimesActivated` _result)
        (set `CharacterMovementComponent.MaxWalkSpeed` (`KismetMathLibrary.Conv_IntToDouble` (* _timesactivated_2 250)) (`self.CharacterMovement`))))
    (else
      (bind _result_2 (`/Engine/EditorBlueprintResources/StandardMacros.DecrementInt` _timesactivated)
        (:`  `
          (set `self.TimesActivated` _result_2)
          (set `CharacterMovementComponent.MaxWalkSpeed` (`KismetMathLibrary.Conv_IntToDouble` (* _timesactivated 250)) (`self.CharacterMovement`)))))))

(event `Chase`
  ; Chase
  (if (`self.IsActivated?`)
    (if (`self.IsChasing?`)
      (`|AIMoveTo` self (0.0 0.0 0.0) (`self.Player Ref`)
        (:`OnSuccess`
          (`KismetSystemLibrary.Delay` 0.2)
          (`self.Chase`))))))

(event `patrol`
  (bind _current_waypoint (`self.Current Waypoint`))
  ; Patrol
  (if (`self.IsActivated?`)
    (if (not (`self.IsChasing?`))
      (`|AIMoveTo` self (0.0 0.0 0.0) (`|GetArrayItem` (`self.Waypoint`) (`self.Current Waypoint`))
        (:`OnSuccess`
          (`KismetSystemLibrary.Delay` 0.5)
          (`/Engine/EditorBlueprintResources/StandardMacros.IncrementInt` _current_waypoint
            (:`  `
              (if (>= _current_waypoint (`KismetArrayLibrary.Array_Length` (`self.Waypoint`)))
                (set `self.Current Waypoint` 0))
              (`self.patrol`))))))))

(event `self.Chase Box.OnComponentBeginOverlap`
  (params (OverlappedComponent :type "PrimitiveComponent Object Reference") (OtherActor :type "Actor Object Reference") (OtherComp :type "PrimitiveComponent Object Reference") (OtherBodyIndex :type Integer) (bFromSweep :type Boolean) (SweepResult :type "HitResult Structure (by ref)"))
  ; Chase start / Chase end
  (bind _asbp_third_person_character (cast `/Game/Blueprints/Characters/Player/BP_ThirdPersonCharacter` OtherActor))
  (set `self.Player Ref` _asbp_third_person_character)
  (if (`self.IsActivated?`)
    (`MovementComponent.StopMovementImmediately` (`self.CharacterMovement`))
    (set `self.IsChasing?` true)
    (`self.Chase`)))

(event `self.Chase Box.OnComponentEndOverlap`
  (params (OverlappedComponent :type "PrimitiveComponent Object Reference") (OtherActor :type "Actor Object Reference") (OtherComp :type "PrimitiveComponent Object Reference") (OtherBodyIndex :type Integer))
  ; Chase start / Chase end
  (cast `/Game/Blueprints/Characters/Player/BP_ThirdPersonCharacter` OtherActor)
  (if (`self.IsActivated?`)
    (`MovementComponent.StopMovementImmediately` (`self.CharacterMovement`))
    (set `self.IsChasing?` false)
    (`self.patrol`)))

(event `Attack`
  (bind _returnvalue (`self.GetTransform` self))
  ; Attack
  (bind _returnvalue_2 (`|SpawnActorFromClass` "/Game/Blueprints/Characters/BP_Hitbox.BP_Hitbox_C" (`KismetMathLibrary.MakeTransform` (`KismetMathLibrary.TransformLocation` _returnvalue (100.0 0.0 0.0)) (.rotation _returnvalue) (100.0 100.0 100.0)) "AlwaysSpawn" "MultiplyWithRoot" null 35.0 false null "NewEnumerator1" 1.0 null)))

(event `self.Attack Range.OnComponentBeginOverlap`
  (params (OverlappedComponent :type "PrimitiveComponent Object Reference") (OtherActor :type "Actor Object Reference") (OtherComp :type "PrimitiveComponent Object Reference") (OtherBodyIndex :type Integer) (bFromSweep :type Boolean) (SweepResult :type "HitResult Structure (by ref)"))
  ; Attack
  (cast `/Game/Blueprints/Characters/Player/BP_ThirdPersonCharacter` OtherActor)
  (`self.Attack`)
  (`KismetSystemLibrary.Delay` 0.2))

(fn `UserConstructionScript`
  (`parent.UserConstructionScript`))