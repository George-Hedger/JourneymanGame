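; Windup Warrior enemy character whose AI is driven through blackboard flags for active, player seen and dead.
; Construction script places two checkpoint arrows ahead of and behind the direction arrow, and BeginPlay caches their locations.
; While active, it flags the player as seen only if a complete nav path reaches them, and takes damage with a sound and material flash.
; Death halts movement and plays a montage, destroying the actor on blend out.
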(event `self.ReceiveBeginPlay`
  (`parent.ReceiveBeginPlay`)
  (set `self.Material` (`PrimitiveComponent.GetMaterial` (`self.Mesh`) 0))
  (set `self.Checkpoint 1 Location` (`SceneComponent.K2_GetComponentLocation` (`self.Checkpoint Arrow 1`)))
  (set `self.Checkpoint 2 Location` (`SceneComponent.K2_GetComponentLocation` (`self.Checkpoint Arrow 2`)))
  (if (`self.Start Active?`)
    (`KismetSystemLibrary.DelayUntilNextTick`)
    (`KismetSystemLibrary.DelayUntilNextTick`)
    (`BlackboardComponent.SetValueAsBool` (`AIBlueprintHelperLibrary.GetBlackboard` (`AIBlueprintHelperLibrary.GetAIController` self)) "Active?" true)
    (set `CharacterMovementComponent.MaxWalkSpeed` (`self.Max Speed`) (`self.CharacterMovement`))))

(event `self.PawnSensing.OnSeePawn`
  (params (Pawn :type "Pawn Object Reference"))
  (bind _returnvalue (`AIBlueprintHelperLibrary.GetBlackboard` (`AIBlueprintHelperLibrary.GetAIController` self)))
  (if (`BlackboardComponent.GetValueAsBool` _returnvalue "Active?")
    (bind _returnvalue_2 (`NavigationSystemV1.FindPathToLocationSynchronously` (`self.K2_GetActorLocation` self) (`self.K2_GetActorLocation` Pawn) Pawn null))
    (`/Engine/EditorBlueprintResources/StandardMacros.IsValid` _returnvalue_2
      (:`Is Valid`
        (if (not (`NavigationPath.IsPartial` _returnvalue_2))
          (bind _pathpoints (`NavigationPath.PathPoints` _returnvalue_2))
          (if (< (`KismetMathLibrary.Vector_Distance` (`|GetArrayItem` _pathpoints (`KismetArrayLibrary.Array_LastIndex` _pathpoints)) (`self.K2_GetActorLocation` (`GameplayStatics.GetPlayerCharacter` 0))) 100.0)
            (cast `/Game/Blueprints/Characters/Player/BP_ThirdPersonCharacter` Pawn)
            (`BlackboardComponent.SetValueAsBool` _returnvalue "hasSeenPlayer?" true)))))))

(event `self.ReceiveAnyDamage`
  (params (Damage :type "Float (single-precision)") (DamageType :type "DamageType Object Reference") (InstigatedBy :type "Controller Object Reference") (DamageCauser :type "Actor Object Reference"))
  (bind _mesh (`self.Mesh`))
  (bind _returnvalue (`AIBlueprintHelperLibrary.GetBlackboard` (`AIBlueprintHelperLibrary.GetAIController` self)))
  (if (`BlackboardComponent.GetValueAsBool` _returnvalue "IsDead?")
    _
    (elif (`BlackboardComponent.GetValueAsBool` _returnvalue "Active?")
      (`self.SetHealth` Damage true)
      (`GameplayStatics.PlaySoundAtLocation` "/Game/Assets/SFX/ClockworkMothSounds/SW_ClockworkMoth_Gettinghit1.SW_ClockworkMoth_Gettinghit1" (`self.K2_GetActorLocation`) (struct) 1.0 1.0 0.0 "/Game/Assets/SFX/SoundAttenuation/SA_General.SA_General" null null null)
      (`/Engine/EditorBlueprintResources/StandardMacros.IsValid` _mesh
        (:`Is Valid`
          (`PrimitiveComponent.SetMaterial` _mesh 0 "/Game/Assets/Materials/Characters/Enemies/M_DamageFlash.M_DamageFlash")
          (`KismetSystemLibrary.Delay` 0.2)
          (`PrimitiveComponent.SetMaterial` _mesh 0 null))))))

(event `/Game/Blueprints/Interfaces/BPI_Activate.OnActivationChanged`
  (params (IsActive :type Boolean))
  (bind _returnvalue (`AIBlueprintHelperLibrary.GetBlackboard` (`AIBlueprintHelperLibrary.GetAIController` self)))
  (if IsActive
    (`BlackboardComponent.SetValueAsBool` _returnvalue "Active?" true)
    (else
      (`KismetSystemLibrary.DelayUntilNextTick`)
      (`BlackboardComponent.SetValueAsBool` _returnvalue "Active?" false))))

(event `self.OnDeath`
  (`BlackboardComponent.SetValueAsBool` (`AIBlueprintHelperLibrary.GetBlackboard` (`AIBlueprintHelperLibrary.GetAIController` self)) "IsDead?" true)
  (`MovementComponent.StopMovementImmediately` (`self.CharacterMovement`))
  (`|PlayMontage` (`self.Mesh`) "/Game/Assets/Animations/Enemies/WindUpWarrior/AM_WindUpWarrior_Death_Montage.AM_WindUpWarrior_Death_Montage"
    (:`then`
      (`GameplayStatics.PlaySoundAtLocation` "/Game/Assets/SFX/ClockworkMothSounds/SW_ClockworkMoth_Death.SW_ClockworkMoth_Death" (`self.K2_GetActorLocation`) (struct) 1.0 1.0 0.0 "/Game/Assets/SFX/SoundAttenuation/SA_General.SA_General" null null null))
    (:`OnBlendOut`
      (`self.K2_DestroyActor`))))

(fn `UserConstructionScript`
  (bind _direction_arrow (`self.Direction Arrow`))
  (bind _returnvalue (`SceneComponent.GetForwardVector` _direction_arrow))
  (bind _returnvalue_2 (`SceneComponent.K2_GetComponentLocation` _direction_arrow))
  (`parent.UserConstructionScript`)
  (`SceneComponent.K2_SetWorldLocation` (`self.Checkpoint Arrow 1`) (+ _returnvalue_2 (* _returnvalue (`self.Distance Forward`))) false false)
  (`SceneComponent.K2_SetWorldLocation` (`self.Checkpoint Arrow 2`) (- _returnvalue_2 (* _returnvalue (`self.Distance Backward`))) false false))