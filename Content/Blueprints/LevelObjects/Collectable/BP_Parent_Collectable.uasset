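; Parent collectable actor that calls an empty OnPickup hook when a BP_ThirdPersonCharacter overlaps it, then plays a sound and destroys itself.
; Tick spins the static mesh and bobs it on a sine wave around its starting offset, with a randomized initial yaw.
; Optional spawn physics simulates the sphere and can set its starting velocity through RandomVel.
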(event `self.ReceiveTick`
  (params (DeltaSeconds :type "Float (single-precision)"))
  (`SceneComponent.K2_AddRelativeRotation` (`self.StaticMesh`) (`KismetMathLibrary.MakeRotator` 0.0 0.0 (* DeltaSeconds (`self.Rotation Speed`))) false true)
  (bind _output_get (set `self.TimerInRadians` (`KismetMathLibrary.FWrap` (+ (* (`self.RadiansPerSec`) DeltaSeconds) (`self.TimerInRadians`)) 0.0 2.0)))
  (`SceneComponent.K2_SetRelativeLocation` (`self.StaticMesh`) (+ (`self.StartingOffset`) (`KismetMathLibrary.MakeVector` 0.0 0.0 (* (`KismetMathLibrary.Sin` (* _output_get (`KismetMathLibrary.GetPI`))) (`self.Bounce Height`)))) false true))

(event `self.ReceiveBeginPlay`
  (bind _returnvalue_location (`KismetMathLibrary.BreakTransform` (`SceneComponent.GetRelativeTransform` (`self.StaticMesh`))))
  (bind (_returnvalue_x _returnvalue_y) (`KismetMathLibrary.BreakVector2D` (* (`KismetMathLibrary.GetRotated2D` (1.0 0.0) (`KismetMathLibrary.RandomFloatInRange` 0.0 360.0)) (`KismetMathLibrary.RandomFloatInRange` 0.0 100.0))))
  (set `self.RadiansPerSec` (* (/ 1.0 (`self.TimeTakenToBounce`)) 2.0))
  (set `self.StartingOffset` _returnvalue_location)
  (`SceneComponent.K2_SetRelativeRotation` (`self.StaticMesh`) (`KismetMathLibrary.MakeRotator` 0.0 0.0 (`KismetMathLibrary.RandomFloatInRange` 0.0 360.0)) false false)
  (if (`self.Spawn with physics?`)
    (`PrimitiveComponent.SetSimulatePhysics` (`self.Sphere`) true)
    (if (`self.RandomStartingVelocity?`)
      (`PrimitiveComponent.SetPhysicsLinearVelocity` (`self.Sphere`) (* (`KismetMathLibrary.Normal` (`KismetMathLibrary.MakeVector` _returnvalue_x _returnvalue_y (`KismetMathLibrary.RandomFloatInRange` 50.0 90.0))) (`KismetMathLibrary.RandomFloatInRange` 350.0 550.0)) false "None"))))

(event `self.ReceiveActorBeginOverlap`
  (params (OtherActor :type "Actor Object Reference"))
  (bind _asbp_third_person_character (cast `/Game/Blueprints/Characters/Player/BP_ThirdPersonCharacter` OtherActor))
  (`self.OnPickup` _asbp_third_person_character)
  (`GameplayStatics.PlaySound2D` (`self.Pickup Sound`) 1.0 1.0 0.0 null null)
  (`self.K2_DestroyActor`))

(fn `OnPickup`
  (params (Player :type "/Game/Blueprints/Characters/Player/BP_ThirdPersonCharacter Object Reference")))

(fn `UserConstructionScript`)