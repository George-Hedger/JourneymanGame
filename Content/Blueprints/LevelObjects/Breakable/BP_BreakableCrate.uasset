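; Breakable Chaos geometry collection crate that crumbles once its health runs out or it fractures, triggering a short-lived master field.
; When the player pawn is the damage causer, it spawns a random number of physics coins with slight delays, subject to a chance roll for spawned boxes.
; A gate in TryDestroy removes the actor on the second call, so both the coin step and Chaos fragment removal can finish first.
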(event `self.ReceiveAnyDamage`
  (params (Damage :type "Float (single-precision)") (DamageType :type "DamageType Object Reference") (InstigatedBy :type "Controller Object Reference") (DamageCauser :type "Actor Object Reference"))
  (bind _returnvalue (`self.K2_GetActorLocation`))
  (bind _chance_to_spawn_coin (`self.Chance to spawn coin`))
  (`GameplayStatics.PlaySoundAtLocation` "/Game/Assets/SFX/Level/CrateSounds/SQ_WoodHit.SQ_WoodHit" _returnvalue (struct) 1.0 1.0 0.0 "/Game/Assets/SFX/SoundAttenuation/SA_General.SA_General" null null null)
  (bind _output_get (set `self.ObjectHealth` (- (`self.ObjectHealth`) Damage)))
  (if (<= _output_get 0.0)
    (`/Engine/EditorBlueprintResources/StandardMacros.DoOnce` false :!label _label
      (:`Completed`
        (`GameplayStatics.PlaySoundAtLocation` "/Game/Assets/SFX/Level/SW_WallDestroyed.SW_WallDestroyed" _returnvalue (struct) 1.0 1.0 0.0 "/Game/Assets/SFX/SoundAttenuation/SA_General.SA_General" null null null)
        (`self.CrumblePhysics`)
        (set `self.CoinCoint` (+ (`self.CoinNumMin`) (`KismetMathLibrary.RandomInteger` (- (`self.CoinNumMax`) (`self.CoinNumMin`) -1))))
        (if (== DamageCauser (`GameplayStatics.GetPlayerPawn` 0))
          (if (`self.Spawned box?`)
            (if (== (`KismetMathLibrary.RandomIntegerInRange` 0 _chance_to_spawn_coin) _chance_to_spawn_coin)
              (if (> (`self.CoinCoint`) 0) :!label _label_2
                (`/Engine/EditorBlueprintResources/StandardMacros.DecrementInt` (`self.CoinCoint`)
                  (:`  `
                    (`KismetSystemLibrary.Delay` (`KismetMathLibrary.RandomFloatInRange` 0.0 0.1))
                    (`|SpawnActorFromClass` "/Game/Blueprints/LevelObjects/Collectable/BP_Coin.BP_Coin_C" (`KismetMathLibrary.MakeTransform` (+ (`KismetSystemLibrary.GetComponentBounds` (`self.GC_BP_BreakableCrate`)) (`KismetMathLibrary.MakeVector` (`KismetMathLibrary.RandomFloatInRange` -25.0 25.0) (`KismetMathLibrary.RandomFloatInRange` -25.0 25.0) (`KismetMathLibrary.RandomFloatInRange` -25.0 25.0)))) "Undefined" "MultiplyWithRoot" null true true null)
                    (goto _label_2)))
                (else
                  (`self.TryDestroy`)))
              (else
                (`self.TryDestroy`)))
            (else
              (goto _label_2)))
          (else
            (`self.TryDestroy`)))))))

(event `self.GC_BP_BreakableCrate.OnChaosBreakEvent`
  (params (BreakEvent :type "ChaosBreakEvent Structure (by ref)"))
  (`/Engine/EditorBlueprintResources/StandardMacros.IncrementInt` (`self.FragmentsToRemove`)
    (:`  `
      (goto _label))))

(event `TryDestroy`
  (`|ExecutionSequence`
    (:`then_0`
      (`/Engine/EditorBlueprintResources/StandardMacros.Gate` true :!label _label_3
        (:`Exit`
          (`self.K2_DestroyActor`))))
    (:`then_1`
      (goto _label_3 :!via `Open`))))

(event `self.GC_BP_BreakableCrate.OnChaosRemovalEvent`
  (params (RemovalEvent :type "ChaosRemovalEvent Structure (by ref)"))
  (bind _result (`/Engine/EditorBlueprintResources/StandardMacros.DecrementInt` (`self.FragmentsToRemove`))
    (:`  `
      (if (== _result 0)
        (`self.TryDestroy`)))))

(fn `CrumblePhysics`
  (bind _returnvalue (`|SpawnActorFromClass` "/Engine/EditorResources/FieldNodes/FS_MasterField.FS_MasterField_C" (`KismetMathLibrary.MakeTransform` (`KismetSystemLibrary.GetComponentBounds` (`self.GC_BP_BreakableCrate`))) "Undefined" "MultiplyWithRoot" null null))
  (set `/Engine/EditorResources/FieldNodes/FS_MasterField.ActivationType` "NewEnumerator4" _returnvalue)
  (`/Engine/EditorResources/FieldNodes/FS_MasterField.CE_Trigger` _returnvalue)
  (`self.SetLifeSpan` _returnvalue 0.2))

(fn `UserConstructionScript`)