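; BP_Checkpoint is a level checkpoint that sets the game mode's active respawn PlayerStart when the player character overlaps its box.
; It stores its assigned PlayerStart in BP_AstroGameMode and plays a sound only when that value changes.
; The PlayerStart is tagged in the construction script and retagged differently on BeginPlay, which prints a warning if none is assigned.
; WhenCheckpointed is an empty stub.
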(event `self.ReceiveBeginPlay`
  (`/Engine/EditorBlueprintResources/StandardMacros.IsValid` (`self.Player Start`)
    (:`Is Valid`
      (set `PlayerStart.PlayerStartTag` "TiedToCheckpoint" (`self.Player Start`)))
    (:`Is Not Valid`
      (`KismetSystemLibrary.PrintString` "CHECKPOINT HAS NO PLAYERSTART SELECTED" true true (struct :`R` 1.0 :`G` 0.001409 :`A` 1.0) 1000000.0))))

(event `self.Box.OnComponentBeginOverlap`
  (params (OverlappedComponent :type "PrimitiveComponent Object Reference") (OtherActor :type "Actor Object Reference") (OtherComp :type "PrimitiveComponent Object Reference") (OtherBodyIndex :type Integer) (bFromSweep :type Boolean) (SweepResult :type "HitResult Structure (by ref)"))
  (bind _player_start (`self.Player Start`))
  (cast `/Game/Blueprints/Characters/Player/BP_ThirdPersonCharacter` OtherActor)
  (`KismetSystemLibrary.PrintString` "checkpoint overlap")
  (bind _asbp_astro_game_mode (cast `/Game/Blueprints/Game/BP_AstroGameMode` (`GameplayStatics.GetGameMode`)))
  (if (not (== (`/Game/Blueprints/Game/BP_AstroGameMode.CheckpointPlayerStart` _asbp_astro_game_mode) _player_start))
    (set `/Game/Blueprints/Game/BP_AstroGameMode.CheckpointPlayerStart` _player_start _asbp_astro_game_mode)
    (`GameplayStatics.PlaySound2D` "/Game/Assets/SFX/Level/SQ_Checkpoint.SQ_Checkpoint" 1.0 1.0 0.0 null null)))

(fn `UserConstructionScript`
  (bind _player_start (`self.Player Start`))
  (`/Engine/EditorBlueprintResources/StandardMacros.IsValid` _player_start
    (:`Is Valid`
      (set `PlayerStart.PlayerStartTag` "CheckpointStart" _player_start))))

(fn `WhenCheckpointed`)