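; BP_CutsceneCamera is a placeable camera that plays a cutscene shot when PlayCutscene is called.
; It blends the player view to itself in cinematic mode, holds, then triggers the next linked CameraChain camera.
; The last camera in the chain blends back to the player pawn at half blend time, exits cinematic mode and calls EndCutscene on the third-person character.
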(event `Play Cutscene`
  (`PlayerController.SetViewTargetWithBlend` (`GameplayStatics.GetPlayerController` 0) self (`self.Camera Blend Time`) "VTBlend_EaseInOut" 2.0 false)
  (`PlayerController.SetCinematicMode` (`GameplayStatics.GetPlayerController` 0) true false true true true)
  (`KismetSystemLibrary.Delay` (+ (`self.Pause At Target Time`) (`self.Camera Blend Time`)))
  (`/Engine/EditorBlueprintResources/StandardMacros.IsValid` (`self.Camera Chain`)
    (:`Is Valid`
      (`self.Play Cutscene` (`self.Camera Chain`)))
    (:`Is Not Valid`
      (`PlayerController.SetViewTargetWithBlend` (`GameplayStatics.GetPlayerController` 0) (`GameplayStatics.GetPlayerPawn` 0) (/ (`self.Camera Blend Time`) 2.0) "VTBlend_EaseInOut" 2.0 false)
      (`PlayerController.SetCinematicMode` (`GameplayStatics.GetPlayerController` 0) false false true true true)
      (bind _asbp_third_person_character (cast `/Game/Blueprints/Characters/Player/BP_ThirdPersonCharacter` (`GameplayStatics.GetPlayerPawn` 0)))
      (`/Game/Blueprints/Characters/Player/BP_ThirdPersonCharacter.EndCutscene` _asbp_third_person_character))))

(fn `UserConstructionScript`)