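; Level-placed trigger volume that shows a pop-up widget with a configurable title and description while the player is inside it.
; Begin overlap by BP_ThirdPersonCharacter creates a WBP_Pop_Up from TitleText and DescriptionText and adds it to the viewport; end overlap removes it.
; BeginPlay waits one tick, then checks whether the player already overlaps the volume and shows the pop-up if so.
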(event `self.ReceiveBeginPlay`
  (`KismetSystemLibrary.DelayUntilNextTick`)
  (if (`PrimitiveComponent.IsOverlappingActor` (`self.Volume`) (`GameplayStatics.GetPlayerCharacter` 0))
    (bind _returnvalue (`|CreateWidget` "/Game/Blueprints/Widgets/PlayerHUD/WBP_Pop_Up.WBP_Pop_Up_C" (`GameplayStatics.GetPlayerController` 0) (`self.Title Text`) (`self.Description Text`) :!label _label))
    (`UserWidget.AddToViewport` _returnvalue 0)))

(event `self.Volume.OnComponentBeginOverlap`
  (params (OverlappedComponent :type "PrimitiveComponent Object Reference") (OtherActor :type "Actor Object Reference") (OtherComp :type "PrimitiveComponent Object Reference") (OtherBodyIndex :type Integer) (bFromSweep :type Boolean) (SweepResult :type "HitResult Structure (by ref)"))
  (cast `/Game/Blueprints/Characters/Player/BP_ThirdPersonCharacter` OtherActor)
  (goto _label))

(event `self.Volume.OnComponentEndOverlap`
  (params (OverlappedComponent :type "PrimitiveComponent Object Reference") (OtherActor :type "Actor Object Reference") (OtherComp :type "PrimitiveComponent Object Reference") (OtherBodyIndex :type Integer))
  (cast `/Game/Blueprints/Characters/Player/BP_ThirdPersonCharacter` OtherActor)
  (`Widget.RemoveFromParent` (stale `self.ReceiveBeginPlay` _returnvalue)))

(fn `UserConstructionScript`)