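; Base interactable slot where the player installs or removes a carried cog pickup to switch linked objects on or off.
; Changes propagate to ObjectsToActivate through BPI_Activate, on either the actor or its components.
; The first insertion can play a camera cutscene, delaying activation and marking every BP_ActiveCamera as played.
; While filled, Tick spins the cog and two counter-rotating component groups; hovering with a held item shows an outline.
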(event `self.ReceiveBeginPlay`
  (`self.UpdateAllObjects` false))

(event `Remove cog`
  (bind _pickupinslot (`self.PickupInSlot`)
    (:`then`
      (`self.K2_DestroyActor` _pickupinslot)
      (set `self.PickupInSlot` null :!label _label)
      (`self.UpdateAllObjects` false))
    (:`else`)))

(event `/Game/Blueprints/Interfaces/BPI_Interactable.OnInteract`
  (bind (_returnvalue_location _returnvalue_rotation _returnvalue_scale) (`KismetMathLibrary.BreakTransform` (`self.GetTransform`)))
  (bind _asbp_third_person_character (cast `/Game/Blueprints/Characters/Player/BP_ThirdPersonCharacter` (`GameplayStatics.GetPlayerPawn` 0)))
  (`/Engine/EditorBlueprintResources/StandardMacros.IsValid` (`self.PickupInSlot`)
    (:`Is Valid`
      (if (`self.Can cog be taken out?`)
        (`/Game/Blueprints/Characters/Player/BP_ThirdPersonCharacter.PickupItem` _asbp_third_person_character (`self.PickupInSlot`))
        (`GameplayStatics.PlaySound2D` "/Game/Assets/SFX/Level/SQ_CogRemoval.SQ_CogRemoval" 1.0 1.0 0.0 null null)
        (goto _label)))
    (:`Is Not Valid`
      (bind _helditemref (`/Game/Blueprints/Characters/Player/BP_ThirdPersonCharacter.DropPickup` _asbp_third_person_character))
      (`/Engine/EditorBlueprintResources/StandardMacros.IsValid` _helditemref
        (:`Is Valid`
          (`/Game/Blueprints/LevelObjects/Pickups/BP_Base_Pickup.DisableCollision` _helditemref)
          (bind _output_get (set `self.PickupInSlot` _helditemref))
          (`self.K2_SetActorTransform` _output_get (`KismetMathLibrary.MakeTransform` (+ _returnvalue_location (`self.PickupTransform`)) _returnvalue_rotation _returnvalue_scale) false true)
          (`GameplayStatics.PlaySound2D` "/Game/Assets/SFX/Level/SQ_CogInstallation1.SQ_CogInstallation1" 1.0 1.0 0.0 null null)
          (if (`self.HasPlayedCutscene`)
            (`self.UpdateAllObjects` true :!label _label_2)
            (else
              (bind _targetcutscenecamera (`self.TargetCutsceneCamera`)
                (:`then`
                  (`/Game/Blueprints/LevelObjects/CoreMechanics/BP_CutsceneCamera.Play Cutscene` _targetcutscenecamera)
                  (bind _asbp_third_person_character_2 (cast `/Game/Blueprints/Characters/Player/BP_ThirdPersonCharacter` (`GameplayStatics.GetPlayerPawn` 0))
                    (:`then`
                      (`/Game/Blueprints/Characters/Player/BP_ThirdPersonCharacter.StartCutscene` _asbp_third_person_character_2))
                    (:`CastFailed`
                      _))
                  (`KismetSystemLibrary.Delay` (+ (`/Game/Blueprints/LevelObjects/CoreMechanics/BP_CutsceneCamera.Camera Blend Time` _targetcutscenecamera) (* (`/Game/Blueprints/LevelObjects/CoreMechanics/BP_CutsceneCamera.Pause At Target Time` _targetcutscenecamera) 0.3)))
                  (`self.UpdateAllObjects` true)
                  (`|ExecutionSequence`
                    (:`then_0`
                      (set `self.HasPlayedCutscene` true))
                    (:`then_1`
                      (bind _outactors (`GameplayStatics.GetAllActorsOfClass` "/Game/Blueprints/Characters/Enemies/Cogwork_Soldier/BP_ActiveCamera.BP_ActiveCamera_C"))
                      (for _array_element _outactors
                        (set `/Game/Blueprints/Characters/Enemies/Cogwork_Soldier/BP_ActiveCamera.Has played` true _array_element)))))
                (:`else`
                  (set `self.HasPlayedCutscene` true)
                  (goto _label_2))))))))))

(event `self.ReceiveTick`
  (params (DeltaSeconds :type "Float (single-precision)"))
  (bind _returnvalue (* (`KismetMathLibrary.MakeRotator` 0.0 (`self.SlotActorRotationSpeed`)) DeltaSeconds))
  (if (`self.HasPlayedCutscene`)
    (`/Engine/EditorBlueprintResources/StandardMacros.IsValid` (`self.PickupInSlot`)
      (:`Is Valid`
        (`self.K2_AddActorLocalRotation` (`self.PickupInSlot`) _returnvalue false false)
        (`|ExecutionSequence`
          (:`then_0`
            (`self.RotateChildren` _returnvalue (`self.Rotate`)))
          (:`then_1`
            (`self.RotateChildren` (`KismetMathLibrary.NegateRotator` _returnvalue) (`self.RotateOpposite`))))))))

(event `/Game/Blueprints/Interfaces/BPI_Interactable.OnPlayerHoverBegin`
  (bind _asbp_third_person_character (cast `/Game/Blueprints/Characters/Player/BP_ThirdPersonCharacter` (`GameplayStatics.GetPlayerPawn` 0)))
  (`/Game/Blueprints/Characters/Player/BP_ThirdPersonCharacter.HeldPickupableActor` _asbp_third_person_character
    (:`then`
      (`MeshComponent.SetOverlayMaterial` (`self.Mesh`) "/Game/Assets/Materials/Effects/Outline/MI_InteractOutline.MI_InteractOutline"))
    (:`else`)))

(event `/Game/Blueprints/Interfaces/BPI_Interactable.OnPlayerHoverEnd`
  (`MeshComponent.SetOverlayMaterial` (`self.Mesh`) null))

(fn `UpdateAllObjects`
  (params (IsActive :type Boolean))
  (for (_array_element _array_index) (`self.ObjectsToActivate`)
    (if (`KismetSystemLibrary.DoesImplementInterface` _array_element "/Game/Blueprints/Interfaces/BPI_Activate.BPI_Activate_C")
      (message `/Game/Blueprints/Interfaces/BPI_Activate.OnActivationChanged` _array_element IsActive)
      (else
        (bind _returnvalue (`self.GetComponentsByInterface` _array_element "/Game/Blueprints/Interfaces/BPI_Activate.BPI_Activate_C"))
        (if (> (`KismetArrayLibrary.Array_Length` _returnvalue) 0)
          (for _array_element_2 _returnvalue
            (message `/Game/Blueprints/Interfaces/BPI_Activate.OnActivationChanged` _array_element_2 IsActive))
          (else
            (`KismetSystemLibrary.PrintString` (`KismetStringLibrary.Concat_StrStr` "Object at index: " (`KismetStringLibrary.Conv_IntToString` _array_index) " does not implement BPI_Activate and cannot be activated") true true (struct :`R` 1.0 :`A` 1.0) 100.0)))))))

(fn `UserConstructionScript`)