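; BP_Pendulum is a decorative level object that swings a static mesh in pitch using a timeline scaled by DegreeOfSwing.
; It plays on BeginPlay if active, or when its activation count reaches NumberOfCogActivationsForActive, then jumping to position 0.5.
; Activation changes raise or lower that count, but nothing stops the timeline.
; ACTimeslow's multiplier changes set the timeline's play rate, so the swing follows time slow.
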(event `/Game/Blueprints/Interfaces/BPI_Activate.OnActivationChanged`
  (params (IsActive :type Boolean))
  (bind _pendulum (`self.Pendulum`))
  (bind _output_get (set `self.NumberActivations` (`KismetMathLibrary.Max` (+ (`self.NumberActivations`) (`KismetMathLibrary.SelectInt` 1 -1 IsActive)))))
  (if (>= _output_get (`self.NumberOfCogActivationsForActive`))
    (`TimelineComponent.Play` _pendulum)
    (`TimelineComponent.SetPlaybackPosition` _pendulum 0.5 false true)))

(event `self.ReceiveBeginPlay`
  (add `/Game/Blueprints/Components/AC_Timeslow.OnMultiplierChanged` (`self.AC_Timeslow`) (delegate `MultChanged`))
  (if (`self.Is Active?`)
    (bind (_direction _newtrack_0) (`Timeline|Pendulum` :`NewTime` 0.5)
      (:`Update`
        (`SceneComponent.K2_SetRelativeRotation` (`self.StaticMesh`) (`KismetMathLibrary.MakeRotator` 0.0 (* _newtrack_0 (`self.Degree of swing`))) false false)))))

(event `MultChanged`
  (`TimelineComponent.SetPlayRate` (`self.Pendulum`) (`/Game/Blueprints/Components/AC_Timeslow.Timeslow Multiplier` (`self.AC_Timeslow`))))

(fn `UserConstructionScript`)