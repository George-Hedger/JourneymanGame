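; Destructible cobweb hazard that hampers the player character while overlapped.
; Overlapping Cylinder1 divides the character's walk speed, jump velocity and dive speed by tunable factors, and leaving restores the web's stored max values.
; Damage plays a hit sound and drains health; at zero it restores player 0's movement, plays a destroy sound and destroys itself.
; Wall physics starts via Simulate, or on BeginPlay when SpawnWithPhysics is set.
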(event `Simulate`
  (`PrimitiveComponent.SetSimulatePhysics` (`self.Wall`) true :!label _label))

(event `self.ReceiveBeginPlay`
  (if (`self.Spawn with physics?`)
    (goto _label)))

(event `self.Cylinder1.OnComponentBeginOverlap`
  (params (OverlappedComponent :type "PrimitiveComponent Object Reference") (OtherActor :type "Actor Object Reference") (OtherComp :type "PrimitiveComponent Object Reference") (OtherBodyIndex :type Integer) (bFromSweep :type Boolean) (SweepResult :type "HitResult Structure (by ref)"))
  (bind _asbp_third_person_character (cast `/Game/Blueprints/Characters/Player/BP_ThirdPersonCharacter` OtherActor))
  (bind _charactermovement (`Character.CharacterMovement` _asbp_third_person_character))
  (set `CharacterMovementComponent.MaxWalkSpeed` (/ (`self.Max speed`) (`self.Slowdown amount`)) _charactermovement)
  (set `CharacterMovementComponent.JumpZVelocity` (/ (`self.Max jump`) (`self.Jump dampen`)) _charactermovement)
  (set `/Game/Blueprints/Characters/Player/BP_ThirdPersonCharacter.DiveHorizontalSpeed` (/ (`self.Max dive speed`) (`self.Dive dampen`)) _asbp_third_person_character))

(event `self.Cylinder1.OnComponentEndOverlap`
  (params (OverlappedComponent :type "PrimitiveComponent Object Reference") (OtherActor :type "Actor Object Reference") (OtherComp :type "PrimitiveComponent Object Reference") (OtherBodyIndex :type Integer))
  (bind _asbp_third_person_character (cast `/Game/Blueprints/Characters/Player/BP_ThirdPersonCharacter` OtherActor))
  (bind _charactermovement (`Character.CharacterMovement` _asbp_third_person_character))
  (set `CharacterMovementComponent.MaxWalkSpeed` (`self.Max speed`) _charactermovement)
  (set `CharacterMovementComponent.JumpZVelocity` (`self.Max jump`) _charactermovement)
  (set `/Game/Blueprints/Characters/Player/BP_ThirdPersonCharacter.DiveHorizontalSpeed` (`self.Max dive speed`) _asbp_third_person_character))

(event `self.ReceiveAnyDamage`
  (params (Damage :type "Float (single-precision)") (DamageType :type "DamageType Object Reference") (InstigatedBy :type "Controller Object Reference") (DamageCauser :type "Actor Object Reference"))
  (`GameplayStatics.PlaySoundAtLocation` "/Game/Assets/SFX/Level/CobwebSounds/SQ_Cobweb_Hit.SQ_Cobweb_Hit" (`self.K2_GetActorLocation`) (struct) 1.0 1.0 0.0 "/Game/Assets/SFX/SoundAttenuation/SA_General.SA_General" null null null)
  (bind _output_get (set `self.ObjectHealth` (- (`self.ObjectHealth`) Damage)))
  (if (<= _output_get 0.0)
    (bind _asbp_third_person_character (cast `/Game/Blueprints/Characters/Player/BP_ThirdPersonCharacter` (`GameplayStatics.GetPlayerCharacter` 0)))
    (bind _charactermovement (`Character.CharacterMovement` _asbp_third_person_character))
    (set `CharacterMovementComponent.MaxWalkSpeed` (`self.Max speed`) _charactermovement)
    (set `CharacterMovementComponent.JumpZVelocity` (`self.Max jump`) _charactermovement)
    (set `/Game/Blueprints/Characters/Player/BP_ThirdPersonCharacter.DiveHorizontalSpeed` (`self.Max dive speed`) _asbp_third_person_character)
    (`GameplayStatics.PlaySoundAtLocation` "/Game/Assets/SFX/Level/CobwebSounds/SQ_CobwebDestroyed.SQ_CobwebDestroyed" (`self.K2_GetActorLocation`) (struct) 1.0 1.0 0.0 "/Game/Assets/SFX/SoundAttenuation/SA_General.SA_General" null null null)
    (`self.K2_DestroyActor`)))

(fn `UserConstructionScript`)