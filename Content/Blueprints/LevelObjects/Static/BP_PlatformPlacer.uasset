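; Level-building tool that lays copies of a Platform static mesh along a spline to form static platform runs.
; The construction script derives the count from spline length and mesh X extent plus XOffset, then adds evenly spaced mesh components ignoring the Camera collision channel.
; Pieces follow spline yaw but never roll; ZHeightOverride drops the spline's height, while PitchOverride makes them follow its pitch.
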(fn `UserConstructionScript`
  (bind _pitchoverride (`self.PitchOverride`))
  (set `self.MeshLength` (* (.x (`.BoxExtent` (`KismetMathLibrary.BreakBoxSphereBounds` (`StaticMesh.GetBounds` (`self.Platform`))))) 2.0))
  (set `self.MeshNumber` (`KismetMathLibrary.FTrunc` (/ (`SplineComponent.GetSplineLength` (`self.Spline`)) (+ (`self.MeshLength`) (`self.XOffset`)))))
  (for _index (range (`self.MeshNumber`))
    (if (`self.ZHeightOverride`)
      (if _pitchoverride
        (bind _returnvalue (`SplineComponent.GetTransformAtDistanceAlongSpline` (`self.Spline`) (* (`KismetMathLibrary.Conv_IntToDouble` _index) (+ (`self.MeshLength`) (`self.XOffset`))) "Local" false))
        (bind _x (.x (.location _returnvalue)))
        (bind _y (.y (.location _returnvalue)))
        (bind _returnvalue_2 (`AddComponent|NODE_AddStaticMeshComponent-4` :`RelativeTransform` (`KismetMathLibrary.MakeTransform` (`KismetMathLibrary.MakeVector` _x _y) (`KismetMathLibrary.MakeRotator` 0.0 (.pitch (.rotation _returnvalue)) (.yaw (.rotation _returnvalue))))))
        (`StaticMeshComponent.SetStaticMesh` _returnvalue_2 (`self.Platform`))
        (`PrimitiveComponent.SetCollisionResponseToChannel` _returnvalue_2 "ECC_Camera" "ECR_Ignore")
        (else
          (bind _returnvalue_3 (`AddComponent|NODE_AddStaticMeshComponent-2` :`RelativeTransform` (`KismetMathLibrary.MakeTransform` (`KismetMathLibrary.MakeVector` _x _y) (`KismetMathLibrary.MakeRotator` 0.0 0.0 (.yaw (.rotation _returnvalue))))))
          (`StaticMeshComponent.SetStaticMesh` _returnvalue_3 (`self.Platform`))
          (`PrimitiveComponent.SetCollisionResponseToChannel` _returnvalue_3 "ECC_Camera" "ECR_Ignore")))
      (elif _pitchoverride
        (bind _returnvalue_4 (`AddComponent|NODE_AddStaticMeshComponent-1` :`RelativeTransform` (`KismetMathLibrary.MakeTransform` (.location _returnvalue) (`KismetMathLibrary.MakeRotator` 0.0 (.pitch (.rotation _returnvalue)) (.yaw (.rotation _returnvalue))))))
        (`StaticMeshComponent.SetStaticMesh` _returnvalue_4 (`self.Platform`))
        (`PrimitiveComponent.SetCollisionResponseToChannel` _returnvalue_4 "ECC_Camera" "ECR_Ignore")
        (else
          (bind _returnvalue_5 (`AddComponent|NODE_AddStaticMeshComponent-0` :`RelativeTransform` (`KismetMathLibrary.MakeTransform` (.location _returnvalue) (`KismetMathLibrary.MakeRotator` 0.0 0.0 (.yaw (.rotation _returnvalue))))))
          (`StaticMeshComponent.SetStaticMesh` _returnvalue_5 (`self.Platform`))
          (`PrimitiveComponent.SetCollisionResponseToChannel` _returnvalue_5 "ECC_Camera" "ECR_Ignore"))))))