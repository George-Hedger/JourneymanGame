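; BP_NailTrail is a static level object that scatters nail meshes in a band along a spline.
; Its construction script turns Density into a spacing, then steps along the spline length and across Width to build a grid centered on the curve.
; Each point gets a new static mesh component with random sideways jitter within RandomOffset and random yaw.
; A looping random MultiGate picks one of three nail meshes for each component.
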(fn `UserConstructionScript`
  (bind _spline (`self.Spline`))
  (bind _randomoffset (`self.RandomOffset`))
  (`|ExecutionSequence`
    (:`then_0`
      (bind _output_get (set `self.IntervalLength` (/ 100.0 (`self.Density`))))
      (set `self.IntervalAmount` (`KismetMathLibrary.FTrunc` (/ (`SplineComponent.GetSplineLength` (`self.Spline`)) _output_get)))
      (set `self.SpawnAmount` (`KismetMathLibrary.FTrunc` (/ (`self.Width`) (`self.IntervalLength`)))))
    (:`then_1`
      (for _index (range (`self.IntervalAmount`))
        (for _index_2 (range (`self.SpawnAmount`))
          (bind _returnvalue (* _index (`self.IntervalLength`)))
          (bind _returnvalue_2 (`KismetMathLibrary.Normal` (`KismetMathLibrary.GetRightVector` (`SplineComponent.GetRotationAtDistanceAlongSpline` _spline _returnvalue "Local"))))
          (bind _returnvalue_3 (`AddComponent|NODE_AddStaticMeshComponent-1` :`RelativeTransform` (`KismetMathLibrary.MakeTransform` (+ (* _index_2 (`self.IntervalLength`) _returnvalue_2) (`SplineComponent.GetLocationAtDistanceAlongSpline` _spline _returnvalue "Local") (* _returnvalue_2 (* (`self.IntervalLength`) -0.5 (`self.SpawnAmount`))) (* (`KismetMathLibrary.RandomFloatInRange` (* _randomoffset -1.0) _randomoffset) _returnvalue_2)) (`KismetMathLibrary.MakeRotator` 0.0 0.0 (`KismetMathLibrary.RandomFloatInRange` -180.0 180.0)))))
          ; randomly select a mesh to apply
          (`|MultiGate` true true
            (:`Out 0`
              (`StaticMeshComponent.SetStaticMesh` _returnvalue_3 "/Game/Assets/StaticMeshes/Hazards/Nails/SM_Nail_2.SM_Nail_2"))
            (:`Out 1`
              (`StaticMeshComponent.SetStaticMesh` _returnvalue_3 "/Game/Assets/StaticMeshes/Hazards/Nails/SM_Nail_1.SM_Nail_1"))
            (:`Out 2`
              (`StaticMeshComponent.SetStaticMesh` _returnvalue_3 "/Game/Assets/StaticMeshes/Hazards/Nails/SM_Nail_0.SM_Nail_0"))))))))