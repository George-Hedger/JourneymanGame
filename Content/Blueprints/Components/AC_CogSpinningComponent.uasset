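; Actor component that spins its owning cog actor by rotating the root component each tick while enabled.
; The rotation speed scales with the owner's AC_Timeslow multiplier when present, and the owner's Niagara effects are hidden while time is slowed.
; Activation changes toggle spinning and timeslow highlighting, and a rotating cog sound plays once, either on activation or at start if already enabled.
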(event `self.ReceiveTick`
  (params (DeltaSeconds :type "Float (single-precision)"))
  (bind _returnvalue (`Actor.K2_GetComponentsByClass` (`self.GetOwner`) "/Script/Niagara.NiagaraComponent"))
  (bind _returnvalue_2 (`Actor.K2_GetComponentsByClass` (`self.GetOwner`) "/Script/Niagara.NiagaraComponent"))
  (`|ExecutionSequence`
    (:`then_0`
      (if (`self.Enabled`)
        (`SceneComponent.K2_AddLocalRotation` (`Actor.RootComponent` (`self.GetOwner`)) (* (`self.RotationAmount`) (* DeltaSeconds (`self.GetMultiplier`))) false false)))
    (:`then_1`
      (if (< (`self.GetMultiplier`) 1.0)
        (for _ _returnvalue_2
          (`SceneComponent.SetVisibility` _returnvalue_2 false true))
        (else
          (for _ _returnvalue
            (`SceneComponent.SetVisibility` _returnvalue true true)))))))

(event `/Game/Blueprints/Interfaces/BPI_Activate.OnActivationChanged`
  (params (IsActive :type Boolean))
  (bind _output_get (set `self.Enabled` IsActive))
  (bind _output_get_2 (set `/Game/Blueprints/Components/AC_Timeslow.ShouldHighlight` _output_get (`Actor.GetComponentByClass` (`self.GetOwner`) "/Game/Blueprints/Components/AC_Timeslow.AC_Timeslow_C")))
  (if _output_get_2
    (`self.PlaySound`)))

(event `self.ReceiveBeginPlay`
  (bind _returnvalue (`Actor.GetComponentByClass` (`self.GetOwner`) "/Game/Blueprints/Components/AC_Timeslow.AC_Timeslow_C"))
  (`|ExecutionSequence`
    (:`then_0`
      (`KismetSystemLibrary.DelayUntilNextTick`)
      (if (`self.Enabled`)
        (`self.PlaySound`)))
    (:`then_1`
      (`/Engine/EditorBlueprintResources/StandardMacros.IsValid` _returnvalue
        (:`Is Valid`
          (set `self.Timeslow exists?` true)
          (set `self.Timeslow` _returnvalue)
          (set `/Game/Blueprints/Components/AC_Timeslow.ShouldHighlight` (`self.Enabled`) _returnvalue))
        (:`Is Not Valid`
          (set `self.Timeslow exists?` false))))))

(event `PlaySound`
  (`/Engine/EditorBlueprintResources/StandardMacros.DoOnce` false
    (:`Completed`
      (`GameplayStatics.PlaySoundAtLocation` "/Game/Assets/SFX/Level/Cog/SQ_Cog_Rotating3.SQ_Cog_Rotating3" (`SceneComponent.K2_GetComponentLocation` (`Actor.RootComponent` (`self.GetOwner`))) (struct) 1.0 1.0 0.0 "/Game/Assets/SFX/SoundAttenuation/SA_Cog.SA_Cog" null null null))))

(fn `GetMultiplier`
  (returns (`TimeSlow Mult` :type "Float (double-precision)"))
  (if (`self.Timeslow exists?`)
    (return (`/Game/Blueprints/Components/AC_Timeslow.Timeslow Multiplier` (`self.Timeslow`)))
    (else
      (return 1.0))))