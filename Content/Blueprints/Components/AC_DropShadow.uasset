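; Actor component that gives its owner a fake drop shadow using a projected decal.
; On BeginPlay it adds a scaled-down M_DropShadow decal to the owner and stops the owner's primitive component from receiving decals.
; Each Tick it traces on Visibility along that primitive's negative up vector and, on a hit, moves the decal just above the impact point in world Z.
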(event `self.ReceiveBeginPlay`
  (bind _returnvalue (`self.GetOwner`))
  (bind _returnvalue_2 (`|AddComponentByClass` _returnvalue "/Script/Engine.DecalComponent" false (`KismetMathLibrary.MakeTransform` (0.0 0.0 0.0) (struct :`Pitch` 90.0) (0.25 0.25 0.25))))
  (bind _output_get (set `self.Decal` _returnvalue_2))
  (`PrimitiveComponent.SetReceivesDecals` (`Actor.GetComponentByClass` _returnvalue "/Script/Engine.PrimitiveComponent") false)
  (`DecalComponent.SetDecalMaterial` _output_get "/Game/Assets/Materials/Characters/Player/M_DropShadow.M_DropShadow"))

(event `self.ReceiveTick`
  (params (DeltaSeconds :type "Float (single-precision)"))
  (bind _returnvalue (`Actor.GetComponentByClass` (`self.GetOwner`) "/Script/Engine.PrimitiveComponent"))
  (bind _returnvalue_2 (`SceneComponent.K2_GetComponentLocation` _returnvalue))
  (bind (_outhit _returnvalue_3) (`KismetSystemLibrary.LineTraceSingle` _returnvalue_2 (- _returnvalue_2 (* (`SceneComponent.GetUpVector` _returnvalue) 5000)) "TraceTypeQuery1"))
  (if _returnvalue_3
    (bind (_bblockinghit _binitialoverlap _time _distance _location _impactpoint) (`GameplayStatics.BreakHitResult` _outhit))
    (`SceneComponent.K2_SetWorldLocation` (`self.Decal`) (`KismetMathLibrary.MakeVector` (.x _impactpoint) (.y _impactpoint) (+ (.z _impactpoint) 16.0)) false false)))