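; Actor component that makes its owner a time-slow target, with hover outline, start sound and Niagara effects.
; BeginPlay caches the owner's static meshes and disables Nanite on them; hover events toggle their overlay material.
; Start attaches effects to each mesh and lowers the target multiplier; stop destroys them and restores it.
; A Tick-driven gate interpolates the multiplier at constant speed, broadcasting changes until it reaches the target.
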(event `self.ReceiveBeginPlay`
  (bind _output_get (set `self.StaticMesh` (`Actor.K2_GetComponentsByClass` (`self.GetOwner`) "/Script/Engine.StaticMeshComponent")))
  (for _array_element _output_get
    (set `StaticMeshComponent.bDisallowNanite` true _array_element)
    (`MeshComponent.SetOverlayMaterialMaxDrawDistance` _array_element 999999.0)))

(event `Timeslow Player Hover Begin`
  (if (`self.ShouldHighlight`)
    (for _array_element (`self.StaticMesh`)
      (`MeshComponent.SetOverlayMaterial` _array_element "/Game/Assets/Materials/Effects/Outline/MI_TimeSlowOutline.MI_TimeSlowOutline"))))

(event `Timeslow Player Hover End`
  (for _array_element (`self.StaticMesh`)
    (`MeshComponent.SetOverlayMaterial` _array_element null)))

(event `Timeslow Start`
  (`GameplayStatics.PlaySound2D` "/Game/Assets/SFX/PlayerSound/SQ_TimeSlow_Begain.SQ_TimeSlow_Begain" 1.0 1.0 0.0 null null)
  (for _array_element (`self.StaticMesh`)
    (bind _returnvalue (`NiagaraFunctionLibrary.SpawnSystemAttached` "/Game/Assets/Effects/NP__Time_Slow_Object.NP__Time_Slow_Object" _array_element "None" (0.0 0.0 0.0) (struct) "SnapToTargetIncludingScale" false true "None" false))
    (`KismetArrayLibrary.Array_Add` (`self.NP_TimeSlow_Object`) _returnvalue))
  (set `self.NP_TImeSlow_Player` null)
  (set `self.Timeslow Target` 0.15)
  (goto _label :!via `Open`))

(event `self.ReceiveTick`
  (params (DeltaSeconds :type "Float (single-precision)"))
  (`/Engine/EditorBlueprintResources/StandardMacros.Gate` true :!label _label
    (:`Exit`
      (`self.OnMultiplierChanged`)
      (bind _output_get (set `self.Timeslow Multiplier` (`KismetMathLibrary.FInterpTo_Constant` (`self.Timeslow Multiplier`) (`self.Timeslow Target`) DeltaSeconds (`self.Interp Speed`))))
      (if (== _output_get (`self.Timeslow Target`))
        (`|ExecutionSequence`
          (:`then_0`
            (`MeshComponent.SetOverlayMaterial` (`Actor.GetComponentByClass` (`self.GetOwner`) "/Script/Engine.StaticMeshComponent") null))
          (:`then_1`
            (goto _label :!via `Close`)))))))

(event `Timeslow Stop`
  (for _array_element (`self.NP_TimeSlow_Object`)
    (`self.K2_DestroyComponent` _array_element)
    (`KismetArrayLibrary.Array_Clear` (`self.NP_TimeSlow_Object`))
    (`self.Deactivate` (`self.NP_TImeSlow_Player`))
    (set `self.Timeslow Target` 1.0)
    (goto _label :!via `Open`)))